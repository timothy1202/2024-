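; BP_BossPortal is a portal that takes the player to the Boss_Lizard level.
; It starts hidden with collision off until ShowPortal reveals the plane and enables the trigger box.
; When a Player-tagged component overlaps, a timeline drives noise intensity in the DistortionMPC parameter collection while the camera fades out.
; After a short delay it saves game data, sets the loading screen and opens the level.
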(event `self.ReceiveBeginPlay`
  (`PrimitiveComponent.SetCollisionEnabled` (`self.Box`) "NoCollision")
  (`SceneComponent.SetVisibility` (`self.Plane`) false false))

(event `self.Box.OnComponentBeginOverlap`
  (params (OverlappedComponent :type "PrimitiveComponent Object Reference") (OtherActor :type "Actor Object Reference") (OtherComp :type "PrimitiveComponent Object Reference") (OtherBodyIndex :type Integer) (bFromSweep :type Boolean) (SweepResult :type "HitResult Structure (by ref)"))
  (if (`ActorComponent.ComponentHasTag` OtherComp "Player")
    (bind _asbp_player (cast `/Game/TopDown/Blueprints/BP_Player` OtherActor))
    (set `self.As BP Player` _asbp_player)
    (`|ExecutionSequence`
      (:`then_0`
        (bind (_direction _noise_intencity_value) (`Timeline|Noise Intencity Value`)
          (:`Update`
            (`KismetMaterialLibrary.SetScalarParameterValue` (`self.DistortionMPC`) (`self.Nosie Value Name`) _noise_intencity_value))))
      (:`then_1`
        (`PlayerCameraManager.StartCameraFade` :`self` (`GameplayStatics.GetPlayerCameraManager` 0) :`ToAlpha` 1.0 :`Duration` 1.0 :`bHoldWhenFinished` true)
        (`KismetSystemLibrary.Delay` 1.3)
        (`/Game/TopDown/Blueprints/BP_Player.SaveGameData` (`self.As BP Player`))
        (`/Game/TopDown/Blueprints/TeamProjectLibrary.SetLoadingScreen`)
        (`GameplayStatics.OpenLevel` "Boss_Lizard")))))

(event `ShowPortal`
  (`SceneComponent.SetVisibility` (`self.Plane`) true false)
  (`PrimitiveComponent.SetCollisionEnabled` (`self.Box`) "QueryOnly"))

(fn `UserConstructionScript`)