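; Player pawn component that fades meshes blocking the view between the player camera and the pawn.
; On a configurable tick interval it sphere-traces from the camera to a height-adjusted point offset from the player toward the camera.
; Hits resolve to BC_FadeThisMesh components by actor, or by matching static mesh for tagged Blueprint components.
; Comparing those against the current list drives FadeStart and FadeEnd calls, with optional debug drawing.
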(event `self.ReceiveBeginPlay`
  (`KismetSystemLibrary.Delay` 0.03)
  (`self.SetComponentTickInterval` (`self.Tick Interval`))
  (bind `_as폰` (cast `Pawn` (`self.GetOwner`)))
  (bind _output_get (set `self.Player` `_as폰`))
  (bind `_as플레이어_컨트롤러` (cast `PlayerController` (`Pawn.GetController` _output_get)))
  (bind _playercameramanager (`PlayerController.PlayerCameraManager` `_as플레이어_컨트롤러`)
    (:`then`
      (set `self.Camera` _playercameramanager)
      (if (`self.DebugFadeTrace`)
        (set `self.DebugTrace` "ForDuration")
        (else
          (set `self.DebugTrace` "None"))))
    (:`else`)))

(event `self.ReceiveTick`
  (params (DeltaSeconds :type "Float (single-precision)"))
  (`self.Check"FadeThisMesh"ComponentActivity`))

(fn `Check"FadeThisMesh"ComponentActivity`
  (locals (FTM_ToUpdate :type "Array of /Game/FadeAnything/Blueprints/BC_FadeThisMesh Object Reference") (`"FadeThisMesh"Mesh's` :type "/Game/FadeAnything/Blueprints/BC_FadeThisMesh Object Reference") (PlayerLocation :type "Vector Structure") (CameraLocation :type "Vector Structure"))
  (bind __fadethismesh_mesh_s (`local."FadeThisMesh"Mesh's`))
  (bind __fadethismesh_mesh_s_2 (`local."FadeThisMesh"Mesh's`))
  (bind _staticmesh_array (`self.StaticMesh Array`))
  (bind _staticmesh_array_2 (`self.StaticMesh Array`))
  (bind _faderadius (`self.FadeRadius`))
  (bind (_returnvalue_x _returnvalue_y _returnvalue_z) (`KismetMathLibrary.BreakVector` (`self.LocationPointBetweenA_AndB` (`local.PlayerLocation`) (`local.CameraLocation`) (`self.TraceDistanceFromPlayer`) _faderadius)))
  (bind _player (`self.Player`)
    (:`then`
      (set `local.PlayerLocation` (`Actor.K2_GetActorLocation` _player))
      (bind _camera (`self.Camera`)
        (:`then`
          (set `local.CameraLocation` (`PlayerCameraManager.GetCameraLocation` _camera))
          (bind _outhits (`KismetSystemLibrary.SphereTraceMulti` (`local.CameraLocation`) (`KismetMathLibrary.MakeVector` _returnvalue_x _returnvalue_y (+ _returnvalue_z (`self.TraceOffsetHeight`))) _faderadius (`self.Trace Channel`) true (`|MakeArray` (`self.Player`) :!type "Actor Object Reference") (`self.DebugTrace`) true (struct :`R` 1.0 :`A` 1.0) (struct :`G` 1.0 :`A` 1.0) 0.09))
          (if (== (`KismetArrayLibrary.Array_Length` _outhits) 0)
            (if (not (`KismetArrayLibrary.Array_Identical` (`self.FTM_CurrentList`) (`local.FTM_ToUpdate`))) :!label _label
              (for _array_element (`local.FTM_ToUpdate`)
                (bind _output_get (set `local."FadeThisMesh"Mesh's` _array_element))
                (if (not (`KismetArrayLibrary.Array_Contains` (`self.FTM_CurrentList`) _output_get))
                  (`/Game/FadeAnything/Blueprints/BC_FadeThisMesh.FadeStart` __fadethismesh_mesh_s_2)
                  (`KismetArrayLibrary.Array_Add` (`self.FTM_CurrentList`) __fadethismesh_mesh_s_2)
                  (`KismetArrayLibrary.Array_Remove` _staticmesh_array_2 (`self.Array Index`))
                  (`KismetArrayLibrary.Array_Clear` _staticmesh_array_2)))
              (for _array_element_2 (`self.FTM_CurrentList`) :!label _label_2
                (bind _output_get_2 (set `local."FadeThisMesh"Mesh's` _array_element_2))
                (if (not (`KismetArrayLibrary.Array_Contains` (`local.FTM_ToUpdate`) _output_get_2))
                  (`/Game/FadeAnything/Blueprints/BC_FadeThisMesh.FadeEnd` __fadethismesh_mesh_s)
                  (`KismetArrayLibrary.Array_RemoveItem` (`self.FTM_CurrentList`) __fadethismesh_mesh_s))))
            (else
              (for (_array_element_3 _array_index) _outhits
                (if (not (`self.ComponentHasTag` (`.HitComponent` (`GameplayStatics.BreakHitResult` _array_element_3)) (`self.Fade Blueprint Tag`)))
                  (`/Engine/EditorBlueprintResources/StandardMacros.IsValid` (`.HitActor` (`GameplayStatics.BreakHitResult` _array_element_3))
                    (:`Is Valid`
                      (bind _returnvalue (`Actor.GetComponentByClass` (`.HitActor` (`GameplayStatics.BreakHitResult` _array_element_3)) "/Game/FadeAnything/Blueprints/BC_FadeThisMesh.BC_FadeThisMesh_C"))
                      (`/Engine/EditorBlueprintResources/StandardMacros.IsValid` _returnvalue
                        (:`Is Valid`
                          (`KismetArrayLibrary.Array_Add` (`local.FTM_ToUpdate`) _returnvalue) ; Static Mesh\nComponents
                          (goto _label))
                        (:`Is Not Valid`
                          (goto _label_2)))))
                  (else
                    (`KismetArrayLibrary.Array_Set` _staticmesh_array _array_index (`.HitComponent` (`GameplayStatics.BreakHitResult` _array_element_3)) true)
                    (for (_array_element_4 _array_index_2) _staticmesh_array
                      (set `self.Array Index` _array_index_2)
                      (for _array_element_5 (`Actor.K2_GetComponentsByClass` (`.HitActor` (`GameplayStatics.BreakHitResult` _array_element_3)) "/Game/FadeAnything/Blueprints/BC_FadeThisMesh.BC_FadeThisMesh_C")
                        (if (== _array_element_4 (`/Game/FadeAnything/Blueprints/BC_FadeThisMesh.StaticMesh` _array_element_5))
                          (`/Engine/EditorBlueprintResources/StandardMacros.IsValid` _array_element_4
                            (:`Is Valid`
                              (`/Engine/EditorBlueprintResources/StandardMacros.IsValid` _array_element_5
                                (:`Is Valid`
                                  (`KismetArrayLibrary.Array_Add` (`local.FTM_ToUpdate`) _array_element_5) ; Blueprint Static Mesh\nComponents
                                  (goto _label)))))
                          (else
                            (goto _label_2)))))))))))
        (:`else`)))
    (:`else`)))

(fn `LocationPointBetweenA_AndB`
  (params (LocationA :type "Vector Structure") (LocationB :type "Vector Structure") (OffsetFromA :type "Float (double-precision)") (FadeRadius :type "Float (double-precision)"))
  (returns (ReturnValue :type "Vector Structure"))
  (return (+ LocationA (* (`KismetMathLibrary.GetDirectionUnitVector` LocationA LocationB) (+ OffsetFromA FadeRadius)))))