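; Sword skeleton NPC Blueprint that plays a sword attack and turns into an archer skeleton on death.
; Attack plays the sword montage only while the NPC is alive.
; Tick watches IsNPCDead and, through a DoOnce, disables movement and plays the death montage.
; After a short delay it destroys itself and spawns BP_Skeleton_Archer with its behavior tree at the same transform.
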(event `self.ReceiveTick`
  (params (DeltaSeconds :type "Float (single-precision)"))
  ;[1 1 1] 플레이어 사망 체크 & 부활
  (if (`self.IsNPCDead?`)
    (`/Engine/EditorBlueprintResources/StandardMacros.DoOnce` false
      (:`Completed`
        (`CharacterMovementComponent.DisableMovement` (`self.CharacterMovement`))
        (`self.PlayAnimMontage` "/Game/Assets/SkeletonEnemy/Animations/Anim_Death_Montage.Anim_Death_Montage")
        (`KismetSystemLibrary.Delay` 0.8)
        (`self.K2_DestroyActor`)
        (`AIBlueprintHelperLibrary.SpawnAIFromClass` "/Game/NPC/BP/BP_Skeleton_Archer.BP_Skeleton_Archer_C" "/Game/NPC/AI/BT/BT_Skeleton_Archer.BT_Skeleton_Archer" (`self.K2_GetActorLocation`) (`self.K2_GetActorRotation`) false null)
        (set `self.IsNPCDead?` false)))))

(fn `Attack`
  (returns (`Animation Duration` :type "Float (double-precision)"))
  (if (not (`self.IsNPCDead?`))
    (bind _returnvalue (`self.PlayAnimMontage` "/Game/Assets/SkeletonEnemy/Animations/Anim_Attack_Sword_1_Montage.Anim_Attack_Sword_1_Montage"))
    (return _returnvalue)))

(fn `UserConstructionScript`
  (`parent.UserConstructionScript`))