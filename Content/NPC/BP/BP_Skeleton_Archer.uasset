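; Skeleton archer NPC that fires arrows and respawns after death.
; Attack plays the bow montage while alive, and a separate ShootArrow event spawns BP_Arrow at the Arrow1 transform.
; Tick polls IsNPCDead and, through a DoOnce, disables movement, plays the death montage, waits briefly, destroys the actor and spawns a replacement with BT_Skeleton_Archer at its location and rotation.
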(event `ShootArrow`
  (bind (_returnvalue_location _returnvalue_rotation) (`KismetMathLibrary.BreakTransform` (`SceneComponent.K2_GetComponentToWorld` (`self.Arrow1`))))
  ;[1 1 1] 활 공격
  (`|SpawnActorFromClass` "/Game/NPC/BP/Weapon_BP/BP_Arrow.BP_Arrow_C" (`KismetMathLibrary.MakeTransform` _returnvalue_location _returnvalue_rotation) "AlwaysSpawn" "MultiplyWithRoot" null null))

(event `self.ReceiveTick`
  (params (DeltaSeconds :type "Float (single-precision)"))
  ;[1 1 1] 플레이어 사망 체크 & 부활
  (if (`self.IsNPCDead?`)
    (`/Engine/EditorBlueprintResources/StandardMacros.DoOnce` false
      (:`Completed`
        (`CharacterMovementComponent.DisableMovement` (`self.CharacterMovement`))
        (`self.PlayAnimMontage` "/Game/Assets/SkeletonEnemy/Animations/Anim_Death_Montage.Anim_Death_Montage")
        (`KismetSystemLibrary.Delay` 0.8)
        (`self.K2_DestroyActor`)
        (`AIBlueprintHelperLibrary.SpawnAIFromClass` "BP_Skeleton_Archer_C" "/Game/NPC/AI/BT/BT_Skeleton_Archer.BT_Skeleton_Archer" (`self.K2_GetActorLocation`) (`self.K2_GetActorRotation`) false null)
        (set `self.IsNPCDead?` false)))))

(fn `Attack`
  (returns (`Animation Duration` :type "Float (double-precision)"))
  (if (not (`self.IsNPCDead?`))
    (bind _returnvalue (`self.PlayAnimMontage` "/Game/Assets/SkeletonEnemy/Animations/Anim_AttackBow_Montage.Anim_AttackBow_Montage"))
    (return _returnvalue)))

(fn `UserConstructionScript`
  (`parent.UserConstructionScript`))