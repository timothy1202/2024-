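; BP_Skeleton_Wizard is a skeleton caster NPC that attacks with fireballs and periodically summons skeleton minions.
; Attack plays a cast montage unless dead or summoning; SpawnSkeletonFireBall launches the projectile from a hand socket, restoring walking after a delay.
; A looping timer from BeginPlay plays a summon montage, then spawns BP_Skeleton_Hand with its behavior tree nearby at random.
; Both actions disable movement, but only the fireball event re-enables it.
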(event `SpawnSkeletonFireBall`
  ;[1 1 1] 파이어볼 공격
  (`|SpawnActorFromClass` "/Game/NPC/BP/Weapon_BP/BP_Skeleton_Fireball.BP_Skeleton_Fireball_C" (`KismetMathLibrary.MakeTransform` (`SceneComponent.GetSocketLocation` (`self.Mesh`) "ring_03_r_Socket_Fir") (`self.K2_GetActorRotation` self)) "Undefined" "MultiplyWithRoot" null null)
  (`KismetSystemLibrary.Delay` 3.0)
  (`CharacterMovementComponent.SetMovementMode` (`self.CharacterMovement`) "MOVE_Walking" 0))

(event `self.ReceiveBeginPlay`
  ;[1 1 1] 근접 스켈레톤 소환
  (`parent.ReceiveBeginPlay`)
  (`KismetSystemLibrary.K2_SetTimerDelegate` (delegate `SpawnActorAtRandomLocation`) 7.0 true))

(event `SpawnActorAtRandomLocation`
  (bind (_returnvalue_x _returnvalue_y _returnvalue_z) (`KismetMathLibrary.BreakVector` (`self.K2_GetActorLocation`)))
  ;[1 1 1] 근접 스켈레톤 소환
  (set `self.isSummoning` true)
  (`CharacterMovementComponent.DisableMovement` (`self.CharacterMovement`))
  (`self.PlayAnimMontage` "/Game/Animations/Magic_Skeleton_animation/magic_Skeleton_skill_areaStanding_2H_Magic_Area_Attack_01_Montage.magic_Skeleton_skill_areaStanding_2H_Magic_Area_Attack_01_Montage")
  (`KismetSystemLibrary.Delay` 1.5)
  (bind _output_get (set `self.EnemySpawnLocation` (`KismetMathLibrary.MakeVector` (+ _returnvalue_x (`KismetMathLibrary.RandomFloatInRange` -400.0 400.0)) (+ _returnvalue_y (`KismetMathLibrary.RandomFloatInRange` -400.0 400.0)) _returnvalue_z)))
  (`AIBlueprintHelperLibrary.SpawnAIFromClass` "/Game/NPC/BP/BP_Skeleton_Hand.BP_Skeleton_Hand_C" "/Game/NPC/AI/BT/BT_Skeleton_Hand.BT_Skeleton_Hand" _output_get (struct) false null)
  (set `self.isSummoning` false))

(fn `Attack`
  (returns (`Animation Duration` :type "Float (double-precision)"))
  (if (`self.IsNPCDead?`)
    _
    (elif (not (`self.isSummoning`))
      (`CharacterMovementComponent.DisableMovement` (`self.CharacterMovement`))
      (bind _returnvalue (`self.PlayAnimMontage` "/Game/Animations/Magic_Skeleton_animation/Magic_SkeletonStanding_1H_Magic_Attack_01__1__Montage.Magic_SkeletonStanding_1H_Magic_Attack_01__1__Montage"))
      (return _returnvalue))))

(fn `UserConstructionScript`
  (`parent.UserConstructionScript`))