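; BP_Skeleton_Hand is a skeleton NPC character with attack, hit reaction and death behavior.
; Tick watches IsNPCDead and, once set, disables movement, plays the death montage, then destroys the actor.
; While alive, a BP_Player overlapping HealthSphere briefly halts movement with a hit montage, and Attack plays a double-attack montage.
; The resurrection event contains only a delay.
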(event `self.ReceiveTick`
  (params (DeltaSeconds :type "Float (single-precision)"))
  ;[1 1 1] 플레이어 사망 체크
  (if (`self.IsNPCDead?`)
    (`/Engine/EditorBlueprintResources/StandardMacros.DoOnce` false
      (:`Completed`
        (`CharacterMovementComponent.DisableMovement` (`self.CharacterMovement`))
        (`self.PlayAnimMontage` "/Game/Assets/SkeletonEnemy/Animations/Anim_Death_Montage.Anim_Death_Montage")
        (`KismetSystemLibrary.Delay` 0.8)
        (`self.K2_DestroyActor`)))))

(event `self.HealthSphere.OnComponentBeginOverlap`
  (params (OverlappedComponent :type "PrimitiveComponent Object Reference") (OtherActor :type "Actor Object Reference") (OtherComp :type "PrimitiveComponent Object Reference") (OtherBodyIndex :type Integer) (bFromSweep :type Boolean) (SweepResult :type "HitResult Structure (by ref)"))
  (bind _charactermovement (`self.CharacterMovement`))
  ;[1 1 1] 피격
  (cast `/Game/TopDown/Blueprints/BP_Player` OtherActor)
  (if (not (`self.IsNPCDead?`))
    (`CharacterMovementComponent.DisableMovement` _charactermovement)
    (`self.PlayAnimMontage` "/Game/Assets/SkeletonEnemy/Animations/Anim_Hit_Montage.Anim_Hit_Montage")
    (`KismetSystemLibrary.Delay` 1.5)
    (`CharacterMovementComponent.SetMovementMode` _charactermovement "MOVE_Walking" 0)))

(event `resurrection`
  (`KismetSystemLibrary.Delay` 1.0))

(fn `Attack`
  (returns (`Animation Duration` :type "Float (double-precision)"))
  (if (not (`self.IsNPCDead?`))
    (bind _returnvalue (`self.PlayAnimMontage` "/Game/Assets/SkeletonEnemy/Animations/SK_Skeleton_AttackDouble_Montage.SK_Skeleton_AttackDouble_Montage"))
    (return _returnvalue)))

(fn `UserConstructionScript`
  (`parent.UserConstructionScript`))