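; Orc NPC character with a two-handed melee attack, hit reaction and death sequence.
; Tick polls IsNPCDead and once true halts movement, plays the death montage, then destroys the actor after a delay.
; While alive, a BP_Player overlap on HealthSphere briefly stops movement with a hit montage, and Attack plays the swing montage.
; The HitGround event temporarily switches the attack collision to the HitGround profile, then back to NoCollision.
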(event `self.ReceiveTick`
  (params (DeltaSeconds :type "Float (single-precision)"))
  ;[1 1 1] 플레이어 사망 체크
  (if (`self.IsNPCDead?`)
    (`/Engine/EditorBlueprintResources/StandardMacros.DoOnce` false
      (:`Completed`
        (`CharacterMovementComponent.DisableMovement` (`self.CharacterMovement`))
        (`self.PlayAnimMontage` "/Game/Assets/Orcs_Bundle/Orc_Hunter/Animations/Combat/Anim_Orc_Death_Orc_Death_Montage.Anim_Orc_Death_Orc_Death_Montage")
        (`KismetSystemLibrary.Delay` 2.0)
        (`self.K2_DestroyActor`)))))

(event `self.HealthSphere.OnComponentBeginOverlap`
  (params (OverlappedComponent :type "PrimitiveComponent Object Reference") (OtherActor :type "Actor Object Reference") (OtherComp :type "PrimitiveComponent Object Reference") (OtherBodyIndex :type Integer) (bFromSweep :type Boolean) (SweepResult :type "HitResult Structure (by ref)"))
  (bind _charactermovement (`self.CharacterMovement`))
  ;[1 1 1] 피격
  (cast `/Game/TopDown/Blueprints/BP_Player` OtherActor)
  (if (not (`self.IsNPCDead?`))
    (`CharacterMovementComponent.DisableMovement` _charactermovement)
    (`self.PlayAnimMontage` "/Game/Assets/Orcs_Bundle/Orc_Hunter/Animations/Combat/Anim_Orc_GetHit_Orc_GetHit_Montage.Anim_Orc_GetHit_Orc_GetHit_Montage")
    (`KismetSystemLibrary.Delay` 1.5)
    (`CharacterMovementComponent.SetMovementMode` _charactermovement "MOVE_Walking" 0)))

(event `HitGround`
  ;[1 1 1] 땅 타격
  (`PrimitiveComponent.SetCollisionProfileName` (`self.TwoHandAttackCollision`) "HitGround" true)
  (`KismetSystemLibrary.Delay` 3.0)
  (`PrimitiveComponent.SetCollisionProfileName` (`self.TwoHandAttackCollision`) "NoCollision" true))

(fn `Attack`
  (returns (`Animation Duration` :type "Float (double-precision)"))
  (if (not (`self.IsNPCDead?`))
    (bind _returnvalue (`self.PlayAnimMontage` "/Game/Assets/Orcs_Bundle/Orc_Hunter/Animations/Combat/Anim_Orc_MeleeAttack_TwoHanded_Orc_MeleeAttack_TwoHanded_Montage.Anim_Orc_MeleeAttack_TwoHanded_Orc_MeleeAttack_TwoHanded_Montage"))
    (return _returnvalue)))

(fn `UserConstructionScript`
  (`parent.UserConstructionScript`))