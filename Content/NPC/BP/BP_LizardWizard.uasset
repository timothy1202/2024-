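; Lizard wizard NPC Blueprint that casts fireballs and handles its own death.
; Attack plays a spell montage while the NPC is alive and returns the montage result.
; A separate SpawnFireBall event spawns BP_Lizard_Fireball at the right thumb socket, facing the actor's rotation.
; Tick polls IsNPCDead and, through a DoOnce, disables movement, plays the death montage and destroys the actor after a short delay.
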(event `self.ReceiveTick`
  (params (DeltaSeconds :type "Float (single-precision)"))
  ;[1 1 1] 플레이어 사망 체크
  (if (`self.IsNPCDead?`)
    (`/Engine/EditorBlueprintResources/StandardMacros.DoOnce` false
      (:`Completed`
        (`CharacterMovementComponent.DisableMovement` (`self.CharacterMovement`))
        (`self.PlayAnimMontage` "/Game/Assets/DrakeAssassin/Animations/Anim_DrakeAssassin_death_Montage.Anim_DrakeAssassin_death_Montage")
        (`KismetSystemLibrary.Delay` 2.5)
        (`self.K2_DestroyActor`)))))

(event `SpawnFireBall`
  ;[1 1 1] 파이어 볼 생성
  (`|SpawnActorFromClass` "/Game/NPC/BP/Weapon_BP/BP_Lizard_Fireball.BP_Lizard_Fireball_C" (`KismetMathLibrary.MakeTransform` (`SceneComponent.GetSocketLocation` (`self.Mesh`) "thumb_03_r_Socket") (`self.K2_GetActorRotation` self)) "Undefined" "MultiplyWithRoot" null null))

(fn `Attack`
  (returns (`Animation Duration` :type "Float (double-precision)"))
  (if (not (`self.IsNPCDead?`))
    (bind _returnvalue (`self.PlayAnimMontage` "/Game/Assets/DrakeAssassin/Animations/Anim_DrakeAssassin_spell02_Montage.Anim_DrakeAssassin_spell02_Montage"))
    (return _returnvalue)))

(fn `UserConstructionScript`
  (`parent.UserConstructionScript`))