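; BP_LizardWarrior_Hand is a lizard warrior enemy NPC with attack, hit and death montages and self-healing.
; The player entering its HealthSphere blocks recovery and, while alive, triggers a hit reaction that briefly halts movement.
; After the player leaves, a delay re-enables recovery and a looping timer restores health until full or blocked.
; Tick watches IsNPCDead to play death once and destroy the actor; damage handling defers to the parent.
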(event `self.ReceiveTick`
  (params (DeltaSeconds :type "Float (single-precision)"))
  ;[1 1 1] 플레이어 사망 체크
  (if (`self.IsNPCDead?`)
    (`/Engine/EditorBlueprintResources/StandardMacros.DoOnce` false
      (:`Completed`
        (`CharacterMovementComponent.DisableMovement` (`self.CharacterMovement`))
        (`self.PlayAnimMontage` "/Game/Assets/DrakeAssassin/Animations/Anim_DrakeAssassin_death_Montage.Anim_DrakeAssassin_death_Montage")
        (`KismetSystemLibrary.Delay` 2.0)
        (`self.K2_DestroyActor`)))))

(event `self.HealthSphere.OnComponentBeginOverlap`
  (params (OverlappedComponent :type "PrimitiveComponent Object Reference") (OtherActor :type "Actor Object Reference") (OtherComp :type "PrimitiveComponent Object Reference") (OtherBodyIndex :type Integer) (bFromSweep :type Boolean) (SweepResult :type "HitResult Structure (by ref)"))
  (bind _charactermovement (`self.CharacterMovement`))
  ;[1 1 1] 자힐 불가 설정 & 피격
  (cast `/Game/TopDown/Blueprints/BP_Player` OtherActor)
  (set `self.CanRecover` false)
  (if (not (`self.IsNPCDead?`))
    (`CharacterMovementComponent.DisableMovement` _charactermovement)
    (`self.PlayAnimMontage` "/Game/Assets/DrakeWarrior/Animation/Anim_DrakeWarrior_hit_Montage.Anim_DrakeWarrior_hit_Montage")
    (`KismetSystemLibrary.Delay` 1.5)
    (`CharacterMovementComponent.SetMovementMode` _charactermovement "MOVE_Walking" 0)))

(event `self.HealthSphere.OnComponentEndOverlap`
  (params (OverlappedComponent :type "PrimitiveComponent Object Reference") (OtherActor :type "Actor Object Reference") (OtherComp :type "PrimitiveComponent Object Reference") (OtherBodyIndex :type Integer))
  ;[1 1 1] 자힐 가능 설정 및 자힐
  (cast `/Game/TopDown/Blueprints/BP_Player` OtherActor)
  (`KismetSystemLibrary.Delay` 2.0)
  (set `self.CanRecover` true)
  (bind _returnvalue (`KismetSystemLibrary.K2_SetTimerDelegate` (delegate `GetHealed`) 1.0 true))
  (bind _asbp_player (cast `/Game/TopDown/Blueprints/BP_Player` OtherActor))
  (`/Engine/EditorBlueprintResources/StandardMacros.IsValid` _asbp_player
    (:`Is Valid`
      (`self.Update Healed Health Bar` (`self.HealHealth`)))))

(event `GetHealed`
  (bind _returnvalue (* (`self.maxHealth`) (mod (`self.healthRegenTime`) 1.0)))
  ;[1 1 1] 자힐
  (if (`self.CanRecover`)
    (if (< (`self.curHealth`) (`self.maxHealth`))
      (set `self.HealHealth` _returnvalue)
      (set `self.curHealth` (+ (`self.curHealth`) _returnvalue))
      (else
        (`KismetSystemLibrary.K2_ClearAndInvalidateTimerHandle` (stale `self.HealthSphere.OnComponentEndOverlap` _returnvalue))))
    (else
      (`KismetSystemLibrary.K2_ClearAndInvalidateTimerHandle` (stale `self.HealthSphere.OnComponentEndOverlap` _returnvalue)))))

(event `self.EnemyTakeDamage`
  (`parent.EnemyTakeDamage`))

(fn `Attack`
  (returns (`Animation Duration` :type "Float (double-precision)"))
  (if (not (`self.IsNPCDead?`))
    (bind _returnvalue (`self.PlayAnimMontage` "/Game/Assets/DrakeWarrior/Animation/LizardWarriorAttack_Montage.LizardWarriorAttack_Montage"))
    (return _returnvalue)))

(fn `Update Healed Health Bar`
  (params (`Heal Amount` :type "Float (double-precision)"))
  (set `self.curHealth` (+ (`self.curHealth`) `Heal Amount`))
  (return))

(fn `UserConstructionScript`
  (`parent.UserConstructionScript`))