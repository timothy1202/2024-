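; Orc NPC variant with a mace that adds a periodic skill attack to the normal melee attack.
; A looping timer from BeginPlay fires the skill every few seconds, playing a 360 swing montage with movement disabled until a short delay restores walking.
; The Attack function plays a downward swing montage only while the orc is alive and not mid-skill; the timed skill itself has no death check.
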(event `self.ReceiveBeginPlay`
  (`parent.ReceiveBeginPlay`)
  (`KismetSystemLibrary.K2_SetTimerDelegate` (delegate `Mace Skill`) 7.0 true))

(event `Mace Skill`
  ;[1 1 1] 철퇴 스킬
  (set `self.isMaceSkilling` true)
  (`CharacterMovementComponent.DisableMovement` (`self.CharacterMovement`))
  (`self.PlayAnimMontage` "/Game/Animations/ORC_IRON_MACE_Animation/ORC_IRON_Mace_SKillStanding_Melee_Attack_360_High_Montage.ORC_IRON_Mace_SKillStanding_Melee_Attack_360_High_Montage")
  (`KismetSystemLibrary.Delay` 1.5)
  (`CharacterMovementComponent.SetMovementMode` (`self.CharacterMovement`) "MOVE_Walking" 0)
  (set `self.isMaceSkilling` false))

(event `self.ReceiveTick`
  (params (DeltaSeconds :type "Float (single-precision)"))
  (`parent.ReceiveTick` DeltaSeconds))

(fn `Attack`
  (returns (`Animation Duration` :type "Float (double-precision)"))
  (if (`self.IsNPCDead?`)
    _
    (elif (not (`self.isMaceSkilling`))
      (bind _returnvalue (`self.PlayAnimMontage` "/Game/Animations/ORC_IRON_MACE_Animation/ORC_IRON_MACE_ATTACKStanding_Melee_Attack_Downward_Montage.ORC_IRON_MACE_ATTACKStanding_Melee_Attack_Downward_Montage"))
      (return _returnvalue))))

(fn `UserConstructionScript`
  (`parent.UserConstructionScript`))