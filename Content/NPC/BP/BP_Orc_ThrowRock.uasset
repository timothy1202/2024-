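; Orc NPC Blueprint variant that attacks by throwing rocks.
; Attack plays a standing stone-throw montage unless the NPC is dead.
; The ThrowRock event spawns a BP_Rock actor at the location and rotation of the Arrow1 component, always spawning regardless of collision.
; BeginPlay and overlap events are disabled stubs, and Tick only calls the parent.
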(event `ThrowRock`
  (bind (_returnvalue_location _returnvalue_rotation) (`KismetMathLibrary.BreakTransform` (`SceneComponent.K2_GetComponentToWorld` (`self.Arrow1`))))
  ;[1 1 1] 돌 투척
  (`|SpawnActorFromClass` "/Game/NPC/BP/Weapon_BP/BP_Rock.BP_Rock_C" (`KismetMathLibrary.MakeTransform` _returnvalue_location _returnvalue_rotation) "AlwaysSpawn" "MultiplyWithRoot" null null))

(event `self.ReceiveTick`
  (params (DeltaSeconds :type "Float (single-precision)"))
  (`parent.ReceiveTick` DeltaSeconds))

(fn `Attack`
  (returns (`Animation Duration` :type "Float (double-precision)"))
  (if (not (`self.IsNPCDead?`))
    (bind _returnvalue (`self.PlayAnimMontage` "/Game/Animations/ORC_STONE_animation/ORC_Stone_AttackStanding_1H_Magic_Attack_03_Montage.ORC_Stone_AttackStanding_1H_Magic_Attack_03_Montage"))
    (return _returnvalue)))

(fn `UserConstructionScript`
  (`parent.UserConstructionScript`))