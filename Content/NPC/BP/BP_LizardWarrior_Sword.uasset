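; BP_LizardWarrior_Sword is a sword-wielding lizard warrior NPC Blueprint that handles its attack and death.
; Attack plays the DrakeWarrior attack montage only while IsNPCDead is false.
; A custom event checks IsNPCDead and, through a DoOnce, disables movement, plays a DrakeAssassin death montage, then destroys the actor after a short delay.
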(event `CustomEvent`
  (params (DeltaSeconds :type "Float (single-precision)"))
  ;[1 1 1] 플레이어 사망 체크
  (if (`self.IsNPCDead?`)
    (`/Engine/EditorBlueprintResources/StandardMacros.DoOnce` false
      (:`Completed`
        (`CharacterMovementComponent.DisableMovement` (`self.CharacterMovement`))
        (`self.PlayAnimMontage` "/Game/Assets/DrakeAssassin/Animations/Anim_DrakeAssassin_death_Montage.Anim_DrakeAssassin_death_Montage")
        (`KismetSystemLibrary.Delay` 1.5)
        (`self.K2_DestroyActor`)))))

(fn `Attack`
  (returns (`Animation Duration` :type "Float (double-precision)"))
  (if (not (`self.IsNPCDead?`))
    (bind _returnvalue (`self.PlayAnimMontage` "/Game/Assets/DrakeWarrior/Animation/Anim_DrakeWarrior_attack02_Montage.Anim_DrakeWarrior_attack02_Montage"))
    (return _returnvalue)))

(fn `UserConstructionScript`
  (`parent.UserConstructionScript`))