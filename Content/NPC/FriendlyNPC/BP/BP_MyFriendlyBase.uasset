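; Base Blueprint for friendly NPC units, handling stat setup, player-follow state and damage response.
; On BeginPlay it copies the unit's DT_Friendly row, including health, speed, attack and skill stats, into variables, then calls Init.
; Overlapping a "muster"-tagged component sets the IsChasingPlayer blackboard key, which Dontfollowplayer clears.
; TakeDamage drives hit effects and the health bar, calling NpcDead at zero health; Attack is a stub returning zero.
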(event `self.ReceiveBeginPlay`
  ;[1 1 1] 코멘트
  (`self.Get Data Table1`)
  (`self.Init`))

(event `self.CapsuleComponent.OnComponentBeginOverlap`
  (params (OverlappedComponent :type "PrimitiveComponent Object Reference") (OtherActor :type "Actor Object Reference") (OtherComp :type "PrimitiveComponent Object Reference") (OtherBodyIndex :type Integer) (bFromSweep :type Boolean) (SweepResult :type "HitResult Structure (by ref)"))
  ;[1 1 1] 소집 관련 콜리전
  (if (`ActorComponent.ComponentHasTag` OtherComp "muster")
    (`BlackboardComponent.SetValueAsBool` (`AIBlueprintHelperLibrary.GetBlackboard` (`AIBlueprintHelperLibrary.GetAIController` self)) (`self.isChasingPlayer`) true)))

(event `Dont follow player`
  ;[1 1 1] 소집 따라가는 것
  (`BlackboardComponent.SetValueAsBool` (`AIBlueprintHelperLibrary.GetBlackboard` (`AIBlueprintHelperLibrary.GetAIController` self)) (`self.isChasingPlayer`) false))

(event `/Game/TopDown/Blueprints/Interface/BPI_Hitable.Take Damage`
  (params (IsPlayer :type Boolean) (damageValue :type "Float (double-precision)"))
  ;[1 1 1] 피격
  (`/Game/TopDown/Blueprints/Components/AC_HitEffectComponent.HitEffect` (`self.AC_HitEffectComponent`) "NewEnumerator1" damageValue)
  (`self.UpdateDamagedHealthBar` damageValue)
  (bind _output_get (set `self.IsNpcDead` (<= (`self.cur_health`) 0.0)))
  (if _output_get
    (`self.NpcDead`)))

(event `self.PlayDieEffectFun`
  ;[1 1 1] die effect function 실행 순서를 위한 노드
  (`/Game/TopDown/Blueprints/Components/AC_HitEffectComponent.PlayDieEffect` (`self.AC_HitEffectComponent`)))

(fn `Attack`
  (returns (`Animation Duration` :type "Float (double-precision)"))
  (return 0.0))

(fn `Get Data Table1`
  (bind _returnvalue (`|GetDataTableRow` "/Game/NPC/FriendlyNPC/DT_Friendly.DT_Friendly" (`self.Row Name`))
    (:`then`
      (set `self.Unit_Type` (break `/Game/NPC/FriendlyNPC/ST_Friendly` _returnvalue))
      (set `self.Unit_Tier` (`.Unit_Tier_37_C55BD44C4876EF3F1C4716B946AA4908` (break `/Game/NPC/FriendlyNPC/ST_Friendly` _returnvalue)))
      (set `self.Unit_Name` (`.Unit_Name_55_063B2AFD40F4E42988C1F1ADEC7396F2` (break `/Game/NPC/FriendlyNPC/ST_Friendly` _returnvalue)))
      (set `self.Unit_Max_Health` (`.Unit_Max_Health_38_3A27D94344BC0C7ABC5BC0AF97B6EEEB` (break `/Game/NPC/FriendlyNPC/ST_Friendly` _returnvalue)))
      (set `self.Unit_Walk_Spd` (`.Unit_Walk_Spd_39_2938A4D04C8B1E203F7D72B8435E8E2B` (break `/Game/NPC/FriendlyNPC/ST_Friendly` _returnvalue)))
      (set `self.Unit_ATK_Dmg` (`.Unit_ATK_Dmg_40_09D9AF1D4CB50A42618557BCCA41D67E` (break `/Game/NPC/FriendlyNPC/ST_Friendly` _returnvalue)))
      (set `self.Unit_Atk_Spd` (`.Unit_Atk_Spd_41_0E28E77546D3342499D34C9C6B400610` (break `/Game/NPC/FriendlyNPC/ST_Friendly` _returnvalue)))
      (set `self.Unit_ATK_Rng` (`.Unit_ATK_Rng_42_7F32DF70465275B506AFF98C6E40D4D5` (break `/Game/NPC/FriendlyNPC/ST_Friendly` _returnvalue)))
      (set `self.Unit_PT_Dmg` (`.Unit_PT_Dmg_43_FF03BC414F717CF25A6AEB93E52CB15D` (break `/Game/NPC/FriendlyNPC/ST_Friendly` _returnvalue)))
      (set `self.Unit_PT_Speed` (`.Unit_PT_Speed_44_DEF66AC44DB19F0808E43EB4A8919FC9` (break `/Game/NPC/FriendlyNPC/ST_Friendly` _returnvalue)))
      (set `self.Skill_CoolTime` (`.Skill_CoolTime_45_AAF31B9A45F9F33BFFF123A896D16CF8` (break `/Game/NPC/FriendlyNPC/ST_Friendly` _returnvalue)))
      (set `self.Skill_ATK_Dmg` (`.Skill_ATK_Dmg_46_00B482C34BB990DFF7A6829C1896A8BB` (break `/Game/NPC/FriendlyNPC/ST_Friendly` _returnvalue)))
      (set `self.Hunter_Fire_Dmg` (`.Hunter_Fire_Dmg_47_9AC618B74BC4176FF3C340A4CA517207` (break `/Game/NPC/FriendlyNPC/ST_Friendly` _returnvalue)))
      (set `self.Hunter_Fire_Rng` (`.Hunter_Fire_Rng_48_411FC0AA4F9E1DC2708182A5FEA2CC6B` (break `/Game/NPC/FriendlyNPC/ST_Friendly` _returnvalue))))))

(fn `UserConstructionScript`)