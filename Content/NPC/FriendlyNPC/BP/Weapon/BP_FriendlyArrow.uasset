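; Arrow projectile for the friendly archer NPC that damages enemies it hits.
; ShootArrow starts the trail effect, sets gravity scale from Speed and computes an arcing launch velocity to the target's current location via SuggestProjectileVelocityCustomArc.
; Overlapping a BP_MyEnemyBase applies UnitPTDmg from the first BP_FriendlyArcher found in the world, not necessarily the shooter, then destroys the arrow.
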(event `ShootArrow`
  (params (Target :type "Actor Object Reference"))
  (bind _projectilemovement (`self.ProjectileMovement`))
  ;[1 1 1] 포물선
  (`ActorComponent.Activate` (`self.FX_Weapon_trail`) false)
  (set `ProjectileMovementComponent.ProjectileGravityScale` (`self.Speed`) _projectilemovement)
  (bind _outlaunchvelocity (`GameplayStatics.SuggestProjectileVelocity_CustomArc` (`self.K2_GetActorLocation`) (`self.K2_GetActorLocation` Target) (`MovementComponent.GetGravityZ` _projectilemovement)))
  (set `MovementComponent.Velocity` _outlaunchvelocity (`self.ProjectileMovement`)))

(event `self.AttackCollision.OnComponentBeginOverlap`
  (params (OverlappedComponent :type "PrimitiveComponent Object Reference") (OtherActor :type "Actor Object Reference") (OtherComp :type "PrimitiveComponent Object Reference") (OtherBodyIndex :type Integer) (bFromSweep :type Boolean) (SweepResult :type "HitResult Structure (by ref)"))
  ;[1 1 1] 총알 플레이어 닿았는지
  (bind _asbp_my_enemy_base (cast `/Game/NPC/EnemeyNPC/BP/BP_MyEnemyBase` OtherActor))
  (bind _returnvalue (`GameplayStatics.GetActorOfClass` "/Game/NPC/FriendlyNPC/BP/BP_FriendlyArcher.BP_FriendlyArcher_C"))
  (`/Game/NPC/EnemeyNPC/BP/BP_MyEnemyBase.Take Damage` _asbp_my_enemy_base false (`FriendlyBase.Unit_PT_Dmg` _returnvalue))
  (`/Engine/EditorBlueprintResources/StandardMacros.IsValid` self
    (:`Is Valid`
      (`ActorComponent.Deactivate` (`self.FX_Weapon_trail`))
      (`self.K2_DestroyActor`))))

(fn `UserConstructionScript`)