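; Base Blueprint for friendly NPCs, handling health, a proximity-shown health bar and a sword-slash montage attack.
; BeginPlay binds the health widget to the NPC and fills health to max.
; Player overlap with HealthSphere subtracts Damage, plays a hit effect and updates the death flag, showing the bar if still alive; leaving hides it.
; EnemyTakeDamage is an empty stub, and death only prints a message.
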(event `self.ReceiveBeginPlay`
  ;[1 1 1] HP바
  (`self.Update Damaged Health Bar` 0.0)
  (bind _asfriendly_ai_health_widget_1 (cast `/Game/NPC/FriendlyNPC/Widgets/FriendlyAI_HealthWidget1` (`WidgetComponent.GetWidget` (`self.HealthWidget`))))
  (`/Game/NPC/FriendlyNPC/Widgets/FriendlyAI_HealthWidget1.Init` _asfriendly_ai_health_widget_1 self)
  (set `self.curHealth` (`self.maxHealth`)))

(event `self.HealthSphere.OnComponentBeginOverlap`
  (params (OverlappedComponent :type "PrimitiveComponent Object Reference") (OtherActor :type "Actor Object Reference") (OtherComp :type "PrimitiveComponent Object Reference") (OtherBodyIndex :type Integer) (bFromSweep :type Boolean) (SweepResult :type "HitResult Structure (by ref)"))
  ;[1 1 1] 플레이어가 가까이가면 HP바 보임
  (bind _asbp_player (cast `/Game/TopDown/Blueprints/BP_Player` OtherActor))
  (`/Engine/EditorBlueprintResources/StandardMacros.IsValid` _asbp_player
    (:`Is Valid`
      (if (not (`self.IsNPCDead?`))
        (`self.Update Damaged Health Bar` (`self.Damage`))
        (`/Game/TopDown/Blueprints/AC_CharacterEffectComponent.HitEffect` (`self.AC_CharacterEffectComponent`) "NewEnumerator0" (`self.Damage`))
        (set `self.IsNPCDead?` (<= (`self.curHealth`) 0.0))
        (cast `/Game/TopDown/Blueprints/BP_Player` OtherActor)
        (if (`self.IsNPCDead?`)
          (`KismetSystemLibrary.PrintString` "NPCDead")
          (else
            (`SceneComponent.SetVisibility` (`self.HealthWidget`) true false)))))))

(event `self.HealthSphere.OnComponentEndOverlap`
  (params (OverlappedComponent :type "PrimitiveComponent Object Reference") (OtherActor :type "Actor Object Reference") (OtherComp :type "PrimitiveComponent Object Reference") (OtherBodyIndex :type Integer))
  ;[1 1 1] 플레이어가 가까이가면 HP바 보임
  (cast `/Game/TopDown/Blueprints/BP_Player` OtherActor)
  (`SceneComponent.SetVisibility` (`self.HealthWidget`) false false)
  (`self.Update Damaged Health Bar` 0.0))

(event `EnemyTakeDamage`)

(fn `Attack`
  (returns (`Animation Duration` :type "Float (double-precision)"))
  (bind _returnvalue (`self.PlayAnimMontage` "/Game/Animations/Melee/Montage_Sword_Slash.Montage_Sword_Slash"))
  (return _returnvalue))

(fn `Update Damaged Health Bar`
  (params (damage :type "Float (double-precision)"))
  (set `self.curHealth` (- (`self.curHealth`) damage))
  (return))

(fn `UserConstructionScript`)