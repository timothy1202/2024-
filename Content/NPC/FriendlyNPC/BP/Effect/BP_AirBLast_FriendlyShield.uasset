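; BP_AirBLast_FriendlyShield is a short-lived air blast effect, apparently for a friendly NPC shield, that knocks enemies away.
; One tick after spawning it sets a three-second lifespan and scans its Sphere once for components tagged Enemy.
; Each is recorded, and those with collision get a velocity-change impulse directed away from the blast center, based on their owner's location.
; The damage logic is disconnected and the overlap event is empty.
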(event `self.ReceiveBeginPlay`
  (`KismetSystemLibrary.DelayUntilNextTick`)
  (`self.SetLifeSpan` 3.0)
  (`self.ExecuteLogic`))

(event `ExecuteLogic`
  (for _array_element (`PrimitiveComponent.GetOverlappingComponents` (`self.Sphere`))
    (if (`ActorComponent.ComponentHasTag` _array_element "Enemy")
      (`KismetArrayLibrary.Array_AddUnique` (`self.EnemyComps`) _array_element)
      (if (`PrimitiveComponent.K2_IsCollisionEnabled` _array_element)
        (`PrimitiveComponent.AddImpulse` _array_element (* (`KismetMathLibrary.GetForwardVector` (`KismetMathLibrary.FindLookAtRotation` (`self.K2_GetActorLocation` (`ActorComponent.GetOwner` _array_element)) (`self.K2_GetActorLocation`))) -500.0) "None" true)))))

(event `self.Sphere.OnComponentBeginOverlap`
  (params (OverlappedComponent :type "PrimitiveComponent Object Reference") (OtherActor :type "Actor Object Reference") (OtherComp :type "PrimitiveComponent Object Reference") (OtherBodyIndex :type Integer) (bFromSweep :type Boolean) (SweepResult :type "HitResult Structure (by ref)")))

(fn `UserConstructionScript`)