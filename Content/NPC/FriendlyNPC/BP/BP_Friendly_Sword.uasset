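; Friendly sword-wielding NPC that fights enemies with montage-driven melee attacks.
; Attack plays the sword montage at the unit's attack speed while the NPC is alive and returns the montage duration.
; Overlaps on the sword collision apply the unit's attack damage to enemies derived from BP_MyEnemyBase, flagged as non-player damage.
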(event `self.Sword Collision.OnComponentBeginOverlap`
  (params (OverlappedComponent :type "PrimitiveComponent Object Reference") (OtherActor :type "Actor Object Reference") (OtherComp :type "PrimitiveComponent Object Reference") (OtherBodyIndex :type Integer) (bFromSweep :type Boolean) (SweepResult :type "HitResult Structure (by ref)"))
  (bind _asbp_my_enemy_base (cast `/Game/NPC/EnemeyNPC/BP/BP_MyEnemyBase` OtherActor))
  (`/Game/NPC/EnemeyNPC/BP/BP_MyEnemyBase.Take Damage` _asbp_my_enemy_base false (`self.Unit_ATK_Dmg`)))

(fn `Attack`
  (returns (`Animation Duration` :type "Float (double-precision)"))
  (if (not (`self.IsNpcDead`))
    (bind _returnvalue (`AnimInstance.Montage_Play` (`SkeletalMeshComponent.GetAnimInstance` (`self.Mesh`)) "/Game/NPC/FriendlyNPC/New_NPC_Sword_1_tier/01_Sword_Animation/Sword_Attack_Montage.Sword_Attack_Montage" (`self.Unit_Atk_Spd`) "Duration" 0.0 true))
    (return _returnvalue)))

(fn `UserConstructionScript`
  (`parent.UserConstructionScript`))