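; Friendly sword-and-shield NPC Blueprint that extends a parent NPC with a shield block skill.
; A one-shot timer shortly after BeginPlay sets IsPlayingSkill, and nothing in this Blueprint clears it.
; While alive, Attack plays the block montage if that flag is set, otherwise the sword attack montage, both at unit attack speed.
; SpawnSkill spawns a friendly shield air blast at the shield mesh, passing in skill damage.
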(event `self.ReceiveBeginPlay`
  (`parent.ReceiveBeginPlay`)
  (`KismetSystemLibrary.K2_SetTimerDelegate` (delegate `Block Skill`) 1.0))

(event `Block Skill`
  (set `self.isPlayingSkill` true))

(fn `Attack`
  (returns (`Animation Duration` :type "Float (double-precision)"))
  (if (`self.IsNpcDead`)
    _
    (elif (`self.isPlayingSkill`)
      (bind _returnvalue (`AnimInstance.Montage_Play` (`SkeletalMeshComponent.GetAnimInstance` (`self.Mesh`)) "/Game/Assets/Sword_Friend_NPC/Animation/Shield_Sword_Skill1block_AnimationSword_And_Shield_Block_Idle_Montage.Shield_Sword_Skill1block_AnimationSword_And_Shield_Block_Idle_Montage" (`self.Unit_Atk_Spd`) "Duration" 0.0 true))
      (return _returnvalue)
      (else
        (bind _returnvalue_2 (`AnimInstance.Montage_Play` (`SkeletalMeshComponent.GetAnimInstance` (`self.Mesh`)) "/Game/Assets/Sword_Friend_NPC/Animation/Shield_Sword_Attack_Montage.Shield_Sword_Attack_Montage" (`self.Unit_Atk_Spd`) "Duration" 0.0 true))
        (return _returnvalue_2)))))

(fn `Spawn Skill`
  (bind (_returnvalue_x _returnvalue_y _returnvalue_z) (`KismetMathLibrary.BreakVector` (`SceneComponent.K2_GetComponentLocation` (`self.ShieldMesh`))))
  (`|SpawnActorFromClass` "/Game/NPC/FriendlyNPC/BP/Effect/BP_AirBLast_FriendlyShield.BP_AirBLast_FriendlyShield_C" (`KismetMathLibrary.MakeTransform` (`KismetMathLibrary.MakeVector` _returnvalue_x _returnvalue_y _returnvalue_z)) "AlwaysSpawn" "MultiplyWithRoot" null (`self.Skill_ATK_Dmg`) null))

(fn `UserConstructionScript`
  (`parent.UserConstructionScript`))