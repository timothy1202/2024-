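; Friendly Hunter NPC that adds a periodic kick skill to its normal attack.
; A looping cooldown timer sets IsPlayingSkill and shrinks the AI blackboard StopDistance so the Hunter closes in.
; Attack then plays the kick montage and restores StopDistance, but nothing here clears the flag; otherwise it plays the regular attack montage.
; KickCollision overlaps apply skill damage to BP_MyEnemyBase actors.
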(event `self.ReceiveBeginPlay`
  ;[1 1 1] 코멘트
  (`parent.ReceiveBeginPlay`)
  (`KismetSystemLibrary.K2_SetTimerDelegate` (delegate `Kick Skill`) (`self.Skill_CoolTime`) true))

(event `Kick Skill`
  ;[1 1 1] 코멘트
  ;;[1 1 1] 코멘트
  (`KismetSystemLibrary.PrintString` "Hello")
  (`BlackboardComponent.SetValueAsFloat` (`AIBlueprintHelperLibrary.GetBlackboard` (`AIBlueprintHelperLibrary.GetAIController` self)) (`self.StopDistance`) 10.0)
  (set `self.isPlayingSkill` true))

(event `End Skill`
  ;[1 1 1] 코멘트
  ;;[1 1 1] 코멘트
  (`BlackboardComponent.SetValueAsFloat` (`AIBlueprintHelperLibrary.GetBlackboard` (`AIBlueprintHelperLibrary.GetAIController` self)) (`self.StopDistance`) 600.0))

(event `self.KickCollision.OnComponentBeginOverlap`
  (params (OverlappedComponent :type "PrimitiveComponent Object Reference") (OtherActor :type "Actor Object Reference") (OtherComp :type "PrimitiveComponent Object Reference") (OtherBodyIndex :type Integer) (bFromSweep :type Boolean) (SweepResult :type "HitResult Structure (by ref)"))
  ;[1 1 1] 코멘트
  (bind _asbp_my_enemy_base (cast `/Game/NPC/EnemeyNPC/BP/BP_MyEnemyBase` OtherActor))
  (`/Game/NPC/EnemeyNPC/BP/BP_MyEnemyBase.Take Damage` _asbp_my_enemy_base false (`self.Skill_ATK_Dmg`)))

(fn `Attack`
  (returns (`Animation Duration` :type "Float (double-precision)"))
  (if (`self.IsNpcDead`)
    _
    (elif (`self.isPlayingSkill`)
      (bind _returnvalue (`AnimInstance.Montage_Play` (`SkeletalMeshComponent.GetAnimInstance` (`self.Mesh`)) "/Game/Assets/Archer_NPC/Animation/Kick_Anim_Hunter_Only.Kick_Anim_Hunter_Only" (`self.Unit_Atk_Spd`) "Duration" 0.0 true))
      (`self.End Skill`)
      (return _returnvalue)
      (else
        (bind _returnvalue_2 (`AnimInstance.Montage_Play` (`SkeletalMeshComponent.GetAnimInstance` (`self.Mesh`)) "/Game/Assets/Archer_NPC/Animation/Attack_Anim.Attack_Anim" (`self.Unit_Atk_Spd`) "Duration" 0.0 true))
        (return _returnvalue_2)))))

(fn `UserConstructionScript`
  (`parent.UserConstructionScript`))