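; BP_FriendlyArcher is a friendly NPC archer that attacks its AI target with arrows.
; Attack plays the attack montage at the unit's attack speed unless the NPC is dead, returning the montage duration.
; The separate ShootArrow event spawns a BP_FriendlyArrow at the Arrow1 component, then passes it the Blackboard's AttackTarget actor.
; The arrow spawns before the target cast, so it exists even when that cast fails.
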(event `ShootArrow`
  (bind (_returnvalue_location _returnvalue_rotation) (`KismetMathLibrary.BreakTransform` (`SceneComponent.K2_GetComponentToWorld` (`self.Arrow1`))))
  ;[1 1 1] 활 공격
  (bind _returnvalue (`|SpawnActorFromClass` "/Game/NPC/FriendlyNPC/BP/Weapon/BP_FriendlyArrow.BP_FriendlyArrow_C" (`KismetMathLibrary.MakeTransform` _returnvalue_location _returnvalue_rotation) "AlwaysSpawn" "MultiplyWithRoot" null null))
  (bind `_as액터` (cast `Actor` (`BlackboardComponent.GetValueAsObject` (`AIBlueprintHelperLibrary.GetBlackboard` (`AIBlueprintHelperLibrary.GetAIController` self)) (`self.AttackTarget`))))
  (`/Game/NPC/FriendlyNPC/BP/Weapon/BP_FriendlyArrow.ShootArrow` _returnvalue `_as액터`))

(fn `Attack`
  (returns (`Animation Duration` :type "Float (double-precision)"))
  (if (not (`self.IsNpcDead`))
    (bind _returnvalue (`AnimInstance.Montage_Play` (`SkeletalMeshComponent.GetAnimInstance` (`self.Mesh`)) "/Game/Assets/Archer_NPC/Animation/Attack_Anim.Attack_Anim" (`self.Unit_Atk_Spd`) "Duration" 0.0 true))
    (return _returnvalue)))

(fn `UserConstructionScript`
  (`parent.UserConstructionScript`))