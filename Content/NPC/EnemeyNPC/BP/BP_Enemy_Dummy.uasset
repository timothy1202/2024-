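; Dummy enemy NPC Blueprint that overrides its behavior events with empty bodies, leaving it effectively inert.
; Tick and the construction script only call the parent, while BeginPlay skips it and GetDataTable_1 calls an empty DefaultSetting.
; Data-table loading, walk speed, attack montage and timed death-montage logic remain as disconnected nodes that never run.
; DieLogic destroys the actor, but the timer meant to trigger it is also disconnected.
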(event `self.ReceiveTick`
  (params (DeltaSeconds :type "Float (single-precision)"))
  (`parent.ReceiveTick` DeltaSeconds))

(event `self.ReceiveBeginPlay`
  ;[1 1 1] 코멘트
)

(event `Sk_Dead`
  (params (NewParam :type "AnimMontage Object Reference"))
  ;[1 1 1] 플레이어 사망 체크
)

(event `GetDataTable_1`
  (params (RowName :type Name))
  ;[1 1 1] 데이터 테이블 변수화
  (`self.DefaultSetting`))

(event `DefaultSetting`
  ;[1 1 1] 디폴트 세팅 설정
)

(event `self.NpcDead`)

(fn `Attack`
  (returns (`Animation Duration` :type "Float (double-precision)")))

(fn `DieLogic`
  (`self.K2_DestroyActor`))

(fn `UserConstructionScript`
  (`parent.UserConstructionScript`))