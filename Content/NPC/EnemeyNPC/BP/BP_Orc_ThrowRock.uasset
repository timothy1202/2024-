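; Orc enemy NPC variant that attacks by throwing rocks, built on a parent NPC class.
; On BeginPlay it requests data table row 6008, then applies the enemy walk speed to character movement after the parent loads the row.
; Attack plays a magic-attack montage unless the NPC is dead.
; A separate ThrowRock event spawns BP_Rock at the location and rotation of Arrow1, with no caller in this graph.
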(event `self.ReceiveBeginPlay`
  ;[1 1 1] 코멘트
  (`/Game/NPC/EnemeyNPC/AI/Interface/BPI_AI_BehaviorTrees.GetDataTable` "6008")
  (`parent.ReceiveBeginPlay`))

(event `ThrowRock`
  (bind (_returnvalue_location _returnvalue_rotation) (`KismetMathLibrary.BreakTransform` (`SceneComponent.K2_GetComponentToWorld` (`self.Arrow1`))))
  ;[1 1 1] 돌 투척
  (`|SpawnActorFromClass` "/Game/NPC/EnemeyNPC/BP/Weapon_BP/BP_Rock.BP_Rock_C" (`KismetMathLibrary.MakeTransform` _returnvalue_location _returnvalue_rotation) "AlwaysSpawn" "MultiplyWithRoot" null null))

(event `/Game/NPC/EnemeyNPC/AI/Interface/BPI_AI_BehaviorTrees.GetDataTable`
  (params (RowName :type Name))
  ;[1 1 1] 데이터 테이블 변수화
  (`parent.GetDataTable` RowName)
  (`self.DefaultSetting_OrcThrowRock`))

(event `DefaultSetting_OrcThrowRock`
  ;[1 1 1] 디폴트 세팅 설정
  (set `CharacterMovementComponent.MaxWalkSpeed` (`self.Enemy Npc Walk Speed`) (`self.CharacterMovement`)))

(fn `Attack`
  (returns (`Animation Duration` :type "Float (double-precision)"))
  (if (not (`self.IsNPCDead?`))
    (bind _returnvalue (`self.PlayAnimMontage` "/Game/Animations/ORC_STONE_animation/Orc_Attack_AnimationStanding_1H_Magic_Attack_03_Fixed_Montage.Orc_Attack_AnimationStanding_1H_Magic_Attack_03_Fixed_Montage"))
    (return _returnvalue)))

(fn `UserConstructionScript`
  (`parent.UserConstructionScript`))