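; Skeleton wizard enemy NPC that throws fireballs and periodically summons melee skeletons, with stats from a data table row.
; Attack plays the casting montage, and a separate event spawns the fireball at AttackDirection.
; A looping timer spawns AI-driven BP_Skeleton_Hand minions at random nearby points.
; IsNormalAttacking and IsSummoning keep the actions exclusive: a summon due mid-attack pauses the timer and runs after the fireball spawns.
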(event `SpawnSkeletonFireBall`
  (bind (_returnvalue_x _returnvalue_y _returnvalue_z) (`KismetMathLibrary.BreakVector` (`self.K2_GetActorLocation`)))
  (bind _attackdirection (`self.AttackDirection`))
  ;[1 1 1] 파이어볼 공격
  (`|SpawnActorFromClass` "/Game/NPC/EnemeyNPC/BP/Weapon_BP/BP_Skeleton_Fireball.BP_Skeleton_Fireball_C" (`KismetMathLibrary.MakeTransform` (`SceneComponent.K2_GetComponentLocation` _attackdirection) (`SceneComponent.K2_GetComponentRotation` _attackdirection)) "Undefined" "MultiplyWithRoot" null null)
  (set `self.isNormalAttacking` false)
  (if (`self.isSummoning`)
    ;[1 1 1] 근접 스켈레톤 소환
    (if (`self.isNormalAttacking`) :!label _label
      (`KismetSystemLibrary.K2_PauseTimerHandle` (stale `self.ReceiveBeginPlay` _returnvalue))
      (else
        (`KismetSystemLibrary.K2_UnPauseTimerHandle` (stale `self.ReceiveBeginPlay` _returnvalue))
        (`self.PlayAnimMontage` "/Game/Animations/Magic_Skeleton_animation/Magic_SK_Skill_SpellStanding_2H_Magic_Area_Attack_01_Fixed_Montage.Magic_SK_Skill_SpellStanding_2H_Magic_Area_Attack_01_Fixed_Montage")
        (bind _output_get (set `self.EnemySpawnLocation` (`KismetMathLibrary.MakeVector` (+ _returnvalue_x (`KismetMathLibrary.RandomFloatInRange` -400.0 400.0)) (+ _returnvalue_y (`KismetMathLibrary.RandomFloatInRange` -400.0 400.0)) _returnvalue_z)))
        (`AIBlueprintHelperLibrary.SpawnAIFromClass` "/Game/NPC/EnemeyNPC/BP/BP_Skeleton_Hand.BP_Skeleton_Hand_C" "/Game/NPC/EnemeyNPC/AI/BT/BT_Skeleton_Hand.BT_Skeleton_Hand" _output_get (struct) false null)
        (set `self.isSummoning` false)))))

(event `self.ReceiveBeginPlay`
  ;[1 1 1] 근접 스켈레톤 소환
  (`/Game/NPC/EnemeyNPC/AI/Interface/BPI_AI_BehaviorTrees.GetDataTable` "6003")
  (`parent.ReceiveBeginPlay`)
  (bind _returnvalue (`KismetSystemLibrary.K2_SetTimerDelegate` (delegate `SpawnActorAtRandomLocation`) 7.0 true)))

(event `SpawnActorAtRandomLocation`
  ;[1 1 1] 근접 스켈레톤 소환
  (set `self.isSummoning` true)
  (goto _label))

(event `/Game/NPC/EnemeyNPC/AI/Interface/BPI_AI_BehaviorTrees.GetDataTable`
  (params (RowName :type Name))
  ;[1 1 1] 데이터 테이블 변수화
  (`parent.GetDataTable` RowName)
  (`self.DefaultSetting_SkWizard`))

(event `DefaultSetting_SkWizard`
  ;[1 1 1] 디폴트 세팅 설정
  (set `CharacterMovementComponent.MaxWalkSpeed` (`self.Enemy Npc Walk Speed`) (`self.CharacterMovement`)))

(fn `Attack`
  (returns (`Animation Duration` :type "Float (double-precision)"))
  (if (`self.IsNPCDead?`)
    _
    (elif (not (`self.isSummoning`))
      (set `self.isNormalAttacking` true)
      (bind _returnvalue (`self.PlayAnimMontage` "/Game/Animations/Magic_Skeleton_animation/Magic_SK_Normal_AttackStanding_1H_Magic_Attack_01__1__Fixed_Montage.Magic_SK_Normal_AttackStanding_1H_Magic_Attack_01__1__Fixed_Montage"))
      (return _returnvalue))))

(fn `UserConstructionScript`
  (`parent.UserConstructionScript`))