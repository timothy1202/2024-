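; BP_Skeleton_Hand is a skeleton enemy NPC built on a parent Blueprint that supplies shared behavior.
; BeginPlay loads data table row 6000 through the parent, then sets walk speed from it.
; Attack plays a double-attack montage, and player overlap on HealthSphere plays a hit reaction, both only while alive.
; Tick polls the death check, which once plays the death montage, calls NpcDead and destroys the actor after a delay.
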(event `self.ReceiveTick`
  (params (DeltaSeconds :type "Float (single-precision)"))
  (`parent.ReceiveTick` 0.0)
  (`self.Sk_Dead` (`self.Sk_Montage`)))

(event `self.ReceiveBeginPlay`
  ;[1 1 1] 코멘트
  (`/Game/NPC/EnemeyNPC/AI/Interface/BPI_AI_BehaviorTrees.GetDataTable` "6000")
  (`parent.ReceiveBeginPlay`))

(event `Sk_Dead`
  (params (NewParam :type "AnimMontage Object Reference"))
  ;[1 1 1] 플레이어 사망 체크
  (if (`self.IsNPCDead?`)
    (`/Engine/EditorBlueprintResources/StandardMacros.DoOnce` false
      (:`Completed`
        (`self.PlayAnimMontage` NewParam)
        (`self.NpcDead`)
        (`KismetSystemLibrary.Delay` 2.0)
        (`self.K2_DestroyActor`)))))

(event `self.HealthSphere.OnComponentBeginOverlap`
  (params (OverlappedComponent :type "PrimitiveComponent Object Reference") (OtherActor :type "Actor Object Reference") (OtherComp :type "PrimitiveComponent Object Reference") (OtherBodyIndex :type Integer) (bFromSweep :type Boolean) (SweepResult :type "HitResult Structure (by ref)"))
  ;[1 1 1] 피격
  (cast `/Game/TopDown/Blueprints/BP_Player` OtherActor)
  (if (not (`self.IsNPCDead?`))
    (`self.PlayAnimMontage` "/Game/Assets/SkeletonEnemy/Animations/Anim_Hit_Montage.Anim_Hit_Montage")))

(event `/Game/NPC/EnemeyNPC/AI/Interface/BPI_AI_BehaviorTrees.GetDataTable`
  (params (RowName :type Name))
  ;[1 1 1] 데이터 테이블 변수화
  (`parent.GetDataTable` RowName)
  (`self.DefaultSetting`))

(event `DefaultSetting`
  ;[1 1 1] 디폴트 세팅 설정
  (set `CharacterMovementComponent.MaxWalkSpeed` (`self.Enemy Npc Walk Speed`) (`self.CharacterMovement`)))

(fn `Attack`
  (returns (`Animation Duration` :type "Float (double-precision)"))
  (if (not (`self.IsNPCDead?`))
    (bind _returnvalue (`self.PlayAnimMontage` "/Game/Assets/SkeletonEnemy/Animations/SK_Skeleton_AttackDouble_Montage.SK_Skeleton_AttackDouble_Montage"))
    (return _returnvalue)))

(fn `UserConstructionScript`
  (`parent.UserConstructionScript`))