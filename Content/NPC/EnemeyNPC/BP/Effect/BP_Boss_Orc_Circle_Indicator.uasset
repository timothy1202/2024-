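; Telegraphed circular area attack for the orc boss that warns with a ground indicator, then strikes.
; Dynamic materials draw the rim and fill, with a timeline animating AreaValue, though Tick also writes that parameter.
; When the timeline finishes, it hides the indicator, enables Sphere collision, spawns BP_AirBlast_BossOrc and later destroys itself.
; Sphere overlap passes a DoOnce, damaging a player or base building at most once.
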(event `self.ReceiveBeginPlay`
  (`|ExecutionSequence`
    (:`then_0`
      (bind _returnvalue (`DecalComponent.CreateDynamicMaterialInstance` (`self.Circem`)))
      (bind _output_get (set `self.CircumRef` _returnvalue))
      (`MaterialInstanceDynamic.SetScalarParameterValue` _output_get "Circum1Area0" 1.0))
    (:`then_1`
      (bind _returnvalue_2 (`DecalComponent.CreateDynamicMaterialInstance` (`self.Area`)))
      (bind _output_get_2 (set `self.AreaRef` _returnvalue_2))
      (`MaterialInstanceDynamic.SetScalarParameterValue` _output_get_2 "Circum1Area0" 0.0))
    (:`then_2`
      (`KismetSystemLibrary.Delay` 0.1)
      (bind (_direction _areavaluealpha) (`Timeline|타임라인`)
        (:`Update`
          (`MaterialInstanceDynamic.SetScalarParameterValue` (`self.AreaRef`) "AreaValue" _areavaluealpha))
        (:`Finished`
          (`SceneComponent.SetVisibility` (`self.Area`) false false)
          (`SceneComponent.SetVisibility` (`self.Circem`) false false)
          (`PrimitiveComponent.SetCollisionEnabled` (`self.Sphere`) "QueryAndPhysics")
          (`|SpawnActorFromClass` "/Game/NPC/EnemeyNPC/BP/Effect/BP_AirBlast_BossOrc.BP_AirBlast_BossOrc_C" (`self.GetTransform`) "AlwaysSpawn" "MultiplyWithRoot" null null)
          (`KismetSystemLibrary.Delay` 11.0)
          (`self.K2_DestroyActor`))))))

(event `self.ReceiveTick`
  (params (DeltaSeconds :type "Float (single-precision)"))
  (bind _circumradian (`self.CircumRadian`))
  (if (> (`self.CircumRadian`) 0.0)
    (set `self.CircumRadian` 0.0)
    (else
      (`KismetSystemLibrary.Delay` 0.001)
      (`MaterialInstanceDynamic.SetScalarParameterValue` (`self.AreaRef`) "AreaValue" _circumradian)
      (set `self.CircumRadian` (+ _circumradian 0.4))
      (`KismetSystemLibrary.Delay` 0.01))))

(event `self.Sphere.OnComponentBeginOverlap`
  (params (OverlappedComponent :type "PrimitiveComponent Object Reference") (OtherActor :type "Actor Object Reference") (OtherComp :type "PrimitiveComponent Object Reference") (OtherBodyIndex :type Integer) (bFromSweep :type Boolean) (SweepResult :type "HitResult Structure (by ref)"))
  (`/Engine/EditorBlueprintResources/StandardMacros.DoOnce` false
    (:`Completed`
      (bind _asbp_player (cast `/Game/TopDown/Blueprints/BP_Player` OtherActor)
        (:`then`
          (`/Game/TopDown/Blueprints/BP_Player.DamagePlayer` _asbp_player 40.0))
        (:`CastFailed`
          (bind _asbp_base_building (cast `/Game/Building/BP_BaseBuilding` OtherActor))
          (`/Game/Building/BP_BaseBuilding.Take Damage` _asbp_base_building false 40.0))))))

(fn `UserConstructionScript`)