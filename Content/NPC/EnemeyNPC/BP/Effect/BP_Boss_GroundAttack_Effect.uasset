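; Boss ground attack effect actor that applies area damage through a Sphere collision component.
; When something begins overlapping the sphere, it passes its Damage value to a BP_Player through DamagePlayer, or to a BP_BaseBuilding through TakeDamage flagged as non-player.
; Other actors are ignored.
; Logic to scale the sphere by the owner NPC's attack range exists but is disconnected and never runs.
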(event `self.Sphere.OnComponentBeginOverlap`
  (params (OverlappedComponent :type "PrimitiveComponent Object Reference") (OtherActor :type "Actor Object Reference") (OtherComp :type "PrimitiveComponent Object Reference") (OtherBodyIndex :type Integer) (bFromSweep :type Boolean) (SweepResult :type "HitResult Structure (by ref)"))
  ;[1 1 1] 코멘트
  (bind _asbp_player (cast `/Game/TopDown/Blueprints/BP_Player` OtherActor)
    (:`then`
      (`/Game/TopDown/Blueprints/BP_Player.DamagePlayer` _asbp_player (`self.Damage`)))
    (:`CastFailed`
      (bind _asbp_base_building (cast `/Game/Building/BP_BaseBuilding` OtherActor))
      (`/Game/Building/BP_BaseBuilding.Take Damage` _asbp_base_building false (`self.Damage`)))))

(event `self.ReceiveBeginPlay`
  ;[1 1 1] 코멘트
)

(fn `UserConstructionScript`)