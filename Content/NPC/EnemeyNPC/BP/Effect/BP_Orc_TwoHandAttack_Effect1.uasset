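; Attack effect actor for an orc NPC's two-handed attack that deals area damage through a sphere overlap.
; On BeginPlay it scales the sphere by the owner NPC's attack range divided by 100.
; On overlap it casts the other actor to player, base building or friendly base in turn, then applies the owner's attack damage through that target's damage function.
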(event `self.Sphere.OnComponentBeginOverlap`
  (params (OverlappedComponent :type "PrimitiveComponent Object Reference") (OtherActor :type "Actor Object Reference") (OtherComp :type "PrimitiveComponent Object Reference") (OtherBodyIndex :type Integer) (bFromSweep :type Boolean) (SweepResult :type "HitResult Structure (by ref)"))
  ;[1 1 1] 코멘트
  (bind _asbp_player (cast `/Game/TopDown/Blueprints/BP_Player` OtherActor)
    (:`then`
      (`/Game/TopDown/Blueprints/BP_Player.DamagePlayer` _asbp_player (`EnemyBase.EnemyNpc_AtkDmg` (`self.owner_npc`))))
    (:`CastFailed`
      (bind _asbp_base_building (cast `/Game/Building/BP_BaseBuilding` OtherActor)
        (:`then`
          (`/Game/Building/BP_BaseBuilding.Take Damage` _asbp_base_building false (`EnemyBase.EnemyNpc_AtkDmg` (`self.owner_npc`))))
        (:`CastFailed`
          (bind _asbp_my_friendly_base (cast `/Game/NPC/FriendlyNPC/BP/BP_MyFriendlyBase` OtherActor))
          (`/Game/NPC/FriendlyNPC/BP/BP_MyFriendlyBase.Take Damage` _asbp_my_friendly_base false (`EnemyBase.EnemyNpc_AtkDmg` (`self.owner_npc`))))))))

(event `self.ReceiveBeginPlay`
  (bind _sphere (`self.Sphere`))
  ;[1 1 1] 코멘트
  (`SceneComponent.SetWorldScale3D` _sphere (* (`SceneComponent.K2_GetComponentScale` _sphere) (/ (`EnemyBase.EnemyNpc_AtkRng` (`self.owner_npc`)) 100.0))))

(fn `UserConstructionScript`)