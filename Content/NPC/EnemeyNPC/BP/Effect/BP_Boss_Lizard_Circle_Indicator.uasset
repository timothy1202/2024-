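; Circular ground telegraph for the lizard boss's area debuff, built from outline and fill decals or meshes driven by dynamic materials.
; A timeline animates the fill, then hides the indicator and briefly enables sphere collision; Tick also writes the fill value.
; The first overlap passes a DoOnce, halving attack speed and damage on a player or friendly unit for 10 seconds.
; The actor destroys itself about 11 seconds after the hit window.
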(event `self.ReceiveBeginPlay`
  (`|ExecutionSequence`
    (:`then_0`
      (bind _returnvalue (`DecalComponent.CreateDynamicMaterialInstance` (`self.Circem`)))
      (bind _output_get (set `self.CircumRef` _returnvalue))
      (`MaterialInstanceDynamic.SetScalarParameterValue` _output_get "Circum1Area0" 1.0))
    (:`then_1`
      (bind _returnvalue_2 (`DecalComponent.CreateDynamicMaterialInstance` (`self.Area`)))
      (bind _output_get_2 (set `self.AreaRef` _returnvalue_2))
      (`MaterialInstanceDynamic.SetScalarParameterValue` _output_get_2 "Circum1Area0" 0.0))
    (:`then_2`
      (`KismetSystemLibrary.Delay` 0.1)
      (bind (_direction _areavaluealpha) (`Timeline|타임라인_0`)
        (:`Update`
          (`MaterialInstanceDynamic.SetScalarParameterValue` (`self.AreaRef`) "AreaValue" _areavaluealpha))
        (:`Finished`
          (`SceneComponent.SetVisibility` (`self.Area`) false false)
          (`SceneComponent.SetVisibility` (`self.Circem`) false false)
          (`PrimitiveComponent.SetCollisionEnabled` (`self.Sphere`) "QueryAndPhysics")
          (`KismetSystemLibrary.Delay` 0.1)
          (`PrimitiveComponent.SetCollisionEnabled` (`self.Sphere`) "NoCollision")
          (`KismetSystemLibrary.Delay` 11.0)
          (`self.K2_DestroyActor`))))))

(event `self.ReceiveTick`
  (params (DeltaSeconds :type "Float (single-precision)"))
  (bind _circumradian (`self.CircumRadian`))
  (if (> (`self.CircumRadian`) 0.0)
    (set `self.CircumRadian` 0.0)
    (else
      (`KismetSystemLibrary.Delay` 0.01)
      (`MaterialInstanceDynamic.SetScalarParameterValue` (`self.AreaRef`) "AreaValue" _circumradian)
      (set `self.CircumRadian` (+ _circumradian 0.01))
      (`KismetSystemLibrary.Delay` 0.1))))

(event `self.Sphere.OnComponentBeginOverlap`
  (params (OverlappedComponent :type "PrimitiveComponent Object Reference") (OtherActor :type "Actor Object Reference") (OtherComp :type "PrimitiveComponent Object Reference") (OtherBodyIndex :type Integer) (bFromSweep :type Boolean) (SweepResult :type "HitResult Structure (by ref)"))
  (`/Engine/EditorBlueprintResources/StandardMacros.DoOnce` false
    (:`Completed`
      (bind _asbp_player (cast `/Game/TopDown/Blueprints/BP_Player` OtherActor)
        (:`then`
          (`KismetSystemLibrary.PrintString` "strat")
          (set `/Game/TopDown/Blueprints/BP_Player.공격 속도` (/ (`/Game/TopDown/Blueprints/BP_Player.공격 속도` _asbp_player) 2.0) _asbp_player)
          (set `/Game/TopDown/Blueprints/BP_Player.공격력` (/ (`/Game/TopDown/Blueprints/BP_Player.공격력` _asbp_player) 2.0) _asbp_player)
          (`KismetSystemLibrary.Delay` 10.0)
          (set `/Game/TopDown/Blueprints/BP_Player.공격 속도` (* (`/Game/TopDown/Blueprints/BP_Player.공격 속도` _asbp_player) 2.0) _asbp_player)
          (set `/Game/TopDown/Blueprints/BP_Player.공격력` (* (`/Game/TopDown/Blueprints/BP_Player.공격력` _asbp_player) 2.0) _asbp_player)
          (`KismetSystemLibrary.PrintString` "디버프 끝남"))
        (:`CastFailed`
          (bind _asbp_my_friendly_base (cast `/Game/NPC/FriendlyNPC/BP/BP_MyFriendlyBase` OtherActor))
          (set `FriendlyBase.Unit_Atk_Spd` (/ (`FriendlyBase.Unit_Atk_Spd` _asbp_my_friendly_base) 2.0) _asbp_my_friendly_base)
          (set `FriendlyBase.Unit_ATK_Dmg` (/ (`FriendlyBase.Unit_ATK_Dmg` _asbp_my_friendly_base) 2.0) _asbp_my_friendly_base)
          (`KismetSystemLibrary.Delay` 10.0)
          (set `FriendlyBase.Unit_Atk_Spd` (* (`FriendlyBase.Unit_Atk_Spd` _asbp_my_friendly_base) 2.0) _asbp_my_friendly_base)
          (set `FriendlyBase.Unit_ATK_Dmg` (* (`FriendlyBase.Unit_ATK_Dmg` _asbp_my_friendly_base) 2.0) _asbp_my_friendly_base))))))

(fn `UserConstructionScript`)