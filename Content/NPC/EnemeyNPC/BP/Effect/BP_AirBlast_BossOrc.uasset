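; BP_AirBlast_BossOrc is a short-lived air blast actor, named for the boss orc, that knocks back player components.
; One tick after spawn, it gathers Sphere overlaps tagged Player, enables their physics and pushes collision-enabled ones away with a velocity-change impulse.
; A second later it switches physics off on those stored components, and its lifespan then removes it.
; The randomized damage call is unwired and never runs.
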(event `self.ReceiveBeginPlay`
  (`KismetSystemLibrary.DelayUntilNextTick`)
  (`self.SetLifeSpan` 3.0)
  (`self.ExecuteLogic`)
  (`KismetSystemLibrary.Delay` 1.0)
  (`self.FinishLogic`))

(event `ExecuteLogic`
  (for _array_element (`PrimitiveComponent.GetOverlappingComponents` (`self.Sphere`))
    (`KismetSystemLibrary.PrintString` (`KismetSystemLibrary.GetDisplayName` _array_element))
    (if (`ActorComponent.ComponentHasTag` _array_element "Player")
      (`PrimitiveComponent.SetSimulatePhysics` _array_element true)
      (`KismetArrayLibrary.Array_AddUnique` (`self.EnemyComps`) _array_element)
      (if (`PrimitiveComponent.K2_IsCollisionEnabled` _array_element)
        (`PrimitiveComponent.AddImpulse` _array_element (* (`KismetMathLibrary.GetForwardVector` (`KismetMathLibrary.FindLookAtRotation` (`self.K2_GetActorLocation` (`ActorComponent.GetOwner` _array_element)) (`self.K2_GetActorLocation`))) -900.0) "None" true)))))

(event `FinishLogic`
  (for _array_element (`self.EnemyComps`)
    (`PrimitiveComponent.SetSimulatePhysics` _array_element false)))

(fn `UserConstructionScript`)