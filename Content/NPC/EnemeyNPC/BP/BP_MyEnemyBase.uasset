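; Base enemy NPC that loads stats from DT_EnemyAI by row name, registers on the minimap and sets up a regular or boss health widget.
; TakeDamage drives hit effects, player aggro and death, plus one-shot boss phase hooks at 70% and 40% health.
; Helpers handle state-based speed, attack montages and tier-based drops for non-aggressive enemies.
; Wizard-tower lightning lives here: scaled bolt actors damage other enemies using the building's attack value.
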(event `self.ReceiveBeginPlay`
  (`self.GetDataTables`)
  (`self.Add To Minimap`)
  ;[1 1 1] 원래는 init 안에 있음
  (`self.Init`)
  (if (`self.isBossMonster`)
    (bind _returnvalue (`|CreateWidget` "/Game/NPC/EnemeyNPC/Widgets/EnemyBoss_HealthWidget.EnemyBoss_HealthWidget_C"))
    (set `self.Boss UI Ref` _returnvalue)
    (`/Game/NPC/EnemeyNPC/Widgets/EnemyBoss_HealthWidget.Init` _returnvalue self)
    (else
      (bind _asenemy_ai_health_widget (cast `/Game/NPC/EnemeyNPC/Widgets/EnemyAI_HealthWidget` (`WidgetComponent.GetWidget` (`self.HealthWidget`))))
      (`/Game/NPC/EnemeyNPC/Widgets/EnemyAI_HealthWidget.Init` _asenemy_ai_health_widget self))))

(event `self.NpcDead`
  ;[1 1 1] 코멘트
  (`GameplayStatics.PlaySoundAtLocation` (`self.Die Sound`) (`self.K2_GetActorLocation`) (struct) 2.0 1.0 0.0 "/Game/NPC/EnemeyNPC/BP/EnemyNPC_SoundAttenuation.EnemyNPC_SoundAttenuation" null null null)
  (`parent.NpcDead`))

(event `/Game/NPC/EnemeyNPC/AI/Interface/BPI_AI_BehaviorTrees.SetSpeed`
  (params (State :type String))
  (bind _pawnmovement (`self.PawnMovement`))
  (switch `string` State
    (:`Attack`
      (set `FloatingPawnMovement.MaxSpeed` 0.0 _pawnmovement))
    (:`Chase`
      (set `FloatingPawnMovement.MaxSpeed` (`self.EnemyNpc_RunSpeed`) _pawnmovement))
    (:`Patrol`
      (set `FloatingPawnMovement.MaxSpeed` (`self.EnemyNpc_WalkSpeed`) _pawnmovement))))

(event `/Game/TopDown/Blueprints/Interface/BPI_Hitable.Take Damage`
  (params (IsPlayer :type Boolean) (damageValue :type "Float (double-precision)"))
  (bind _boss_ui_ref (`self.Boss UI Ref`))
  ;[1 1 1] 피격
  (`GameplayStatics.PlaySoundAtLocation` "/Game/Assets/Sounds/NPC/Enemy_Npc_Hit.Enemy_Npc_Hit" (`self.K2_GetActorLocation`) (struct) 2.0 1.0 0.0 "/Game/NPC/EnemeyNPC/BP/EnemyNPC_SoundAttenuation.EnemyNPC_SoundAttenuation" null null null)
  (`/Game/TopDown/Blueprints/Components/AC_HitEffectComponent.HitEffect` (`self.AC_HitEffectComponent`) "NewEnumerator0" damageValue)
  (`self.UpdateDamagedHealthBar` damageValue)
  (if (not (not IsPlayer))
    (`self.SetAttackTarget` (`GameplayStatics.GetPlayerCharacter` 0))
    (set `self.NeverStopChasing` false))
  (bind _output_get (set `self.IsNpcDead` (<= (`self.cur_health`) 0.0)))
  (if _output_get
    (if (`self.isBossMonster`)
      (`Widget.RemoveFromParent` (`self.Boss UI Ref`))
      (`self.NpcDead`)
      (else
        (`self.NpcDead`)))
    (elif (`self.isBossMonster`)
      (`|ExecutionSequence`
        (:`then_0`
          (`UserWidget.AddToViewport` _boss_ui_ref 0)
          (`KismetSystemLibrary.Delay` 5.0)
          (`Widget.RemoveFromParent` _boss_ui_ref))
        (:`then_1`
          (if (< (`self.cur_health`) (* (`self.EnemyNpc_MaxHealth`) 0.4))
            (`/Engine/EditorBlueprintResources/StandardMacros.DoOnce` false
              (:`Completed`
                (`KismetSystemLibrary.PrintString` "333")
                (`self.Enter Page 3`)
                (`Widget.RemoveFromParent` (`/Game/NPC/EnemeyNPC/Widgets/EnemyBoss_HealthWidget.Page3` (`self.Boss UI Ref`)))))
            (elif (< (`self.cur_health`) (* (`self.EnemyNpc_MaxHealth`) 0.7))
              (`/Engine/EditorBlueprintResources/StandardMacros.DoOnce` false
                (:`Completed`
                  (`KismetSystemLibrary.PrintString` "22")
                  (`self.Enter Page 2`)
                  (`Widget.RemoveFromParent` (`/Game/NPC/EnemeyNPC/Widgets/EnemyBoss_HealthWidget.Page2` (`self.Boss UI Ref`))))))))))))

(event `self.DropItem`
  ;[0.6886 0.2578 1] npc죽음 관련 노드
  ;;[0.05098 0.05098 0.05098] 자원 드롭 로직
  (if (not (`self.aggresive`))
    (`self.DropResource`)
    (`self.DropCoin`)))

(event `self.PlayDieEffectFun`
  ;[0.6886 0.2578 1] npc죽음 관련 노드
  ;;[1 1 1] die effect fun 실행 순서를 위한 노드
  (`/Game/TopDown/Blueprints/Components/AC_HitEffectComponent.PlayDieEffect` (`self.AC_HitEffectComponent`)))

(event `self.SpawnFirstThunder`
  (params (tunder_target :type "Actor Object Reference"))
  (bind _returnvalue (`self.K2_GetActorLocation`))
  (bind _whatstarget (`self.WhatsTarget`))
  ;[0.2776 1 0.9303] 번개
  ;;[1 1 1] 첫번째 번개 공격 (번개 BP때문에 BP로 구현)
  (set `self.WhatsTarget` tunder_target)
  (`/Engine/EditorBlueprintResources/StandardMacros.IsValid` _whatstarget
    (:`Is Valid`
      (`|SpawnActorFromClass` "/Game/Building/AttackBuilding/BP/Weapons/BP_Thunder_Base.BP_Thunder_Base_C" (`KismetMathLibrary.MakeTransform` _returnvalue (`KismetMathLibrary.FindLookAtRotation` _returnvalue (`self.K2_GetActorLocation` _whatstarget)) (`KismetMathLibrary.Conv_DoubleToVector` (/ (`self.GetDistanceTo` _whatstarget) (`self.ThunderScale`)))) "Undefined" "MultiplyWithRoot" null null 11.0 null)
      (bind _returnvalue_2 (`GameplayStatics.GetActorOfClass` "/Game/Building/AttackBuilding/BP/BP_WizardBuildingLv3.BP_WizardBuildingLv3_C"))
      (bind _asbp_my_enemy_base (cast `/Game/NPC/EnemeyNPC/BP/BP_MyEnemyBase` (`self.WhatsTarget`)))
      (`self.Take Damage` _asbp_my_enemy_base false (* (`/Game/Building/BP_BaseBuilding.Building PT Atk Dmg` _returnvalue_2) (/ 4.0 5.0)))
      (`self.SecondThunderAttacked` _asbp_my_enemy_base))))

(event `self.SpawnSecondThunder`
  (params (tunder_target :type "Actor Object Reference"))
  (bind _returnvalue (`self.K2_GetActorLocation`))
  (bind _whatstarget (`self.WhatsTarget`))
  ;[0.2776 1 0.9303] 번개
  ;;[1 1 1] 두번째 번개
  (set `self.WhatsTarget` null)
  (`/Engine/EditorBlueprintResources/StandardMacros.IsValid` _whatstarget
    (:`Is Valid`
      (`|SpawnActorFromClass` "/Game/Building/AttackBuilding/BP/Weapons/BP_Thunder_Base.BP_Thunder_Base_C" (`KismetMathLibrary.MakeTransform` _returnvalue (`KismetMathLibrary.FindLookAtRotation` _returnvalue (`self.K2_GetActorLocation` _whatstarget)) (`KismetMathLibrary.Conv_DoubleToVector` (/ (`self.GetDistanceTo` _whatstarget) 0.0))) "Undefined" "MultiplyWithRoot" null null 11.0 null)
      (bind _returnvalue_2 (`GameplayStatics.GetActorOfClass` "/Game/Building/AttackBuilding/BP/BP_WizardBuildingLv3.BP_WizardBuildingLv3_C"))
      (bind _asbp_my_enemy_base (cast `/Game/NPC/EnemeyNPC/BP/BP_MyEnemyBase` (`self.WhatsTarget`)))
      (`self.Take Damage` _asbp_my_enemy_base false (* (`/Game/Building/BP_BaseBuilding.Building PT Atk Dmg` _returnvalue_2) (/ 4.0 5.0))))))

(event `Enter Page 3`)

(event `Enter Page 2`)

(event `Add To Minimap`
  (bind _asbp_player (cast `/Game/TopDown/Blueprints/BP_Player` (`GameplayStatics.GetPlayerCharacter` 0))
    (:`then`
      (bind _minimap (`/Game/TopDown/Blueprints/BP_Player.GetMinimap` _asbp_player))
      (`/Engine/EditorBlueprintResources/StandardMacros.IsValid` _minimap
        (:`Is Valid`
          (`/Game/UMGMinimap/MinimapComponent/MinimapComponent.AddActor` :`self` _minimap :`POIActors` self :`Texture` "/Game/TopDown/Blueprints/UI/Textures/Minimap/Npc_Enemy_maker.Npc_Enemy_maker" :`TextureSize` (5.0 5.0) :`ToolTipOnHover` "적" :`Blink` true))
        (:`Is Not Valid`
          (`KismetSystemLibrary.Delay` 0.1 :!label _label)
          (`self.Add To Minimap`))))
    (:`CastFailed`
      (goto _label))))

(fn `Attack`
  (returns (`Animation Duration` :type "Float (double-precision)"))
  (if (`self.is_boss_skeleton`)
    (if (`self.IsNpcDead`)
      _
      (elif (`self.skeleton first skill playing`)
        (bind _attackmontage (`self.AttackMontage`)
          (:`then`
            (bind _returnvalue (`AnimInstance.Montage_Play` (`SkeletalMeshComponent.GetAnimInstance` (`self.Mesh`)) _attackmontage 1.0 "Duration" 0.0 true))
            (return _returnvalue))
          (:`else`))))
    (elif (not (`self.IsNpcDead`))
      (bind _attackmontage_2 (`self.AttackMontage`)
        (:`then`
          (bind _returnvalue_2 (`AnimInstance.Montage_Play` (`SkeletalMeshComponent.GetAnimInstance` (`self.Mesh`)) _attackmontage_2 (`self.EnemyNpc_AtkSpd`) "Duration" 0.0 true))
          (return _returnvalue_2))
        (:`else`
          (`KismetSystemLibrary.PrintString` (`KismetStringLibrary.Concat_StrStr` (`KismetSystemLibrary.GetObjectName` self) ": 공격 몽타주를 할당해주세요!") true true (struct :`R` 1.0 :`A` 1.0)))))))

(fn `DropCoin`
  (locals (CoinNum :type Integer))
  (switch `int` (`self.EnemyNpc_Tier`)
    (:`Default`
      (`KismetSystemLibrary.PrintString` "코인 드랍 불가능! \n데이터테이블 확인 바람." true true (struct :`R` 1.0 :`A` 1.0) 10.0))
    (:`1`
      (bind _output_get (set `local.CoinNum` (`KismetMathLibrary.RandomIntegerInRange` 0 1)))
      (if (!= _output_get 0)
        (bind _asbp_player (cast `/Game/TopDown/Blueprints/BP_Player` (`GameplayStatics.GetPlayerCharacter` 0) :!label _label))
        (`/Game/TopDown/Blueprints/BP_Player.ChangePlayerResource` _asbp_player "NewEnumerator6" (`local.CoinNum`))
        (bind _returnvalue (`|SpawnActorFromClass` "/Game/TopDown/Blueprints/BP_Message.BP_Message_C" (`KismetMathLibrary.MakeTransform` (`KismetSystemLibrary.GetComponentBounds` (`self.Mesh`))) "Undefined" "MultiplyWithRoot" null null))
        (`/Game/TopDown/Blueprints/BP_Message.GainItem` _returnvalue "/Game/Building/Widget/Texture/ResourceUI/CoinVer2.CoinVer2" (`local.CoinNum`))))
    (:`2`
      (set `local.CoinNum` (`KismetMathLibrary.RandomIntegerInRange` 1 3))
      (goto _label))
    (:`3`
      (set `local.CoinNum` (`KismetMathLibrary.RandomIntegerInRange` 3 5))
      (goto _label))))

(fn `GetDataTables`
  (bind _returnvalue (`|GetDataTableRow` "/Game/NPC/EnemeyNPC/DT_EnemyAI/DT_EnemyAI.DT_EnemyAI" (`self.Row Name`))
    (:`then`
      (set `self.EnemyNpcType` (break `/Game/NPC/EnemeyNPC/ST_EnemyAI/ST_EnemyAI` _returnvalue))
      (set `self.EnemyNpc_Tier` (`.EnemyNpc_Tier_72_8A10BAD448DB95BAD9A9769DCC581A20` (break `/Game/NPC/EnemeyNPC/ST_EnemyAI/ST_EnemyAI` _returnvalue)))
      (set `self.EnemyNpcName` (`.EnemyNpcName_34_21E3BE9947ACDA714B9CB8A44EB9FD75` (break `/Game/NPC/EnemeyNPC/ST_EnemyAI/ST_EnemyAI` _returnvalue)))
      (set `self.EnemyNpc_MaxHealth` (`.EnemyNpc_MaxHealth_73_A3186F5C4717757B61D465B7BC59B1AD` (break `/Game/NPC/EnemeyNPC/ST_EnemyAI/ST_EnemyAI` _returnvalue)))
      (set `self.EnemyNpc_WalkSpeed` (`.EnemyNpc_WalkSpeed_74_30906888497B6042683C449DEE75079A` (break `/Game/NPC/EnemeyNPC/ST_EnemyAI/ST_EnemyAI` _returnvalue)))
      (set `self.EnemyNpc_RunSpeed` (`.EnemyNpc_RunSpeed_63_93832079484F9CA58DD1C4AD241E2C1C` (break `/Game/NPC/EnemeyNPC/ST_EnemyAI/ST_EnemyAI` _returnvalue)))
      (set `self.EnemyNpc_AtkDmg` (`.EnemyNpc_AtkDmg_64_932E28AB484327D55D80A5B0F352DFA7` (break `/Game/NPC/EnemeyNPC/ST_EnemyAI/ST_EnemyAI` _returnvalue)))
      (set `self.EnemyNpc_AtkSpd` (`.EnemyNpc_AtkSpd_44_536C54714FE657A581EBE5BA23C1731E` (break `/Game/NPC/EnemeyNPC/ST_EnemyAI/ST_EnemyAI` _returnvalue)))
      (set `self.EnemyNpc_AtkDist` (`.EnemyNpc_AtkDist_45_970DCD12469952AAD26365A7224C3D71` (break `/Game/NPC/EnemeyNPC/ST_EnemyAI/ST_EnemyAI` _returnvalue)))
      (set `self.EnemyNpc_AtkRng` (`.EnemyNpc_AtkRng_46_FBA613BD4EC0FDCB9D2CCBAFF6923B80` (break `/Game/NPC/EnemeyNPC/ST_EnemyAI/ST_EnemyAI` _returnvalue)))
      (set `self.Lizard_HpRegen` (`.Lizard_HpRegen_65_5611DD3B426F3C9D3E35A4A9883BF811` (break `/Game/NPC/EnemeyNPC/ST_EnemyAI/ST_EnemyAI` _returnvalue)))
      (set `self.Lizard_RegenTime` (`.Lizard_RegenTime_66_0DAB566B45B1B0BB93536BB2026388FA` (break `/Game/NPC/EnemeyNPC/ST_EnemyAI/ST_EnemyAI` _returnvalue)))
      (set `self.Lizard_NoHitTime` (`.Lizard_NoHitTime_67_90206DA74B423A80E2422FA1CEFE0023` (break `/Game/NPC/EnemeyNPC/ST_EnemyAI/ST_EnemyAI` _returnvalue)))
      (set `self.PT_AtkDmg` (`.PT_AtkDmg_68_03D316084817D1FF296B05B2790B3A80` (break `/Game/NPC/EnemeyNPC/ST_EnemyAI/ST_EnemyAI` _returnvalue)))
      (set `self.PT_AtkRng` (`.PT_AtkRng_77_4AD21E8E45898380D53F2C991D5C6F33` (break `/Game/NPC/EnemeyNPC/ST_EnemyAI/ST_EnemyAI` _returnvalue)))
      (set `self.MgSk_SkillSpawnCount` (`.MgSk_SkillSpawnCount_57_1912802C44B4CC84AC27109D2F61055F` (break `/Game/NPC/EnemeyNPC/ST_EnemyAI/ST_EnemyAI` _returnvalue)))
      (set `self.IronMace_SkillAtkDmg` (`.IronMace_SkillAtkDmg_70_282635DF4DE01C767E0A1C9627BDB7D4` (break `/Game/NPC/EnemeyNPC/ST_EnemyAI/ST_EnemyAI` _returnvalue)))
      (set `self.Claw_SkillAtkDmg` (`.Claw_SkillAtkDmg_71_ADAF268E493FDB527CE451A60C01BC94` (break `/Game/NPC/EnemeyNPC/ST_EnemyAI/ST_EnemyAI` _returnvalue)))
      (set `self.PT_AtkRngDmg` (`.PT_AtkRngDmg_69_24F05C8E417110BA136DE2A417382FE1` (break `/Game/NPC/EnemeyNPC/ST_EnemyAI/ST_EnemyAI` _returnvalue)))
      (set `self.Skill_Atk_Spd` (`.Skill_Atk_Spd_82_DED963534A444D844E8976B1E83CE5F2` (break `/Game/NPC/EnemeyNPC/ST_EnemyAI/ST_EnemyAI` _returnvalue)))
      (set `self.Skill_Cool_Time` (`.Skill_Cool_Time_84_FAC927CC494FFB4C8D82A1BB1DB213FD` (break `/Game/NPC/EnemeyNPC/ST_EnemyAI/ST_EnemyAI` _returnvalue)))
      (set `self.Aggression_Run_Speed` (`.Aggression_Run_Speed_88_B6F4B84246AF0BBBC703998C9B0A7CD4` (break `/Game/NPC/EnemeyNPC/ST_EnemyAI/ST_EnemyAI` _returnvalue)))
      (set `self.Boss Skill 1 Dmg` (`.Boss_Skill1_Dmg_98_B4E4AF1041DED213EF7D299DB63C1BE0` (break `/Game/NPC/EnemeyNPC/ST_EnemyAI/ST_EnemyAI` _returnvalue)))
      (set `self.Boss Skill 2 Dmg` (`.Boss_Skill2_Dmg_97_3C74C11A496EFBD34911E192DAA2A8F7` (break `/Game/NPC/EnemeyNPC/ST_EnemyAI/ST_EnemyAI` _returnvalue)))
      (set `self.Boss Skill 4 Dmg` (`.Boss_Skill4_Dmg_100_E9A8FD2944B96ABDD389718769C345AD` (break `/Game/NPC/EnemeyNPC/ST_EnemyAI/ST_EnemyAI` _returnvalue)))
      (set `self.Boss Skill 3 Dmg` (`.Boss_Skill3_Dmg_99_2AA9059E4E3637099EF6A1ADD9B94E8C` (break `/Game/NPC/EnemeyNPC/ST_EnemyAI/ST_EnemyAI` _returnvalue))))))

(fn `UserConstructionScript`)