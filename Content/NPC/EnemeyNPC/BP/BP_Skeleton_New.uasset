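; BP_Skeleton_New is a skeleton enemy NPC Blueprint that deals sword damage to player and building targets on overlap.
; When SwordCollision begins overlapping, it checks the other component's tag.
; PlayerAllies components lead to a cast to BP_Player and a DamagePlayer call, while BuildingAllies components send TakeDamageMessage to the owning actor, both using EnemyNpcAtkDmg.
; The construction script only calls its parent.
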(event `self.SwordCollision.OnComponentBeginOverlap`
  (params (OverlappedComponent :type "PrimitiveComponent Object Reference") (OtherActor :type "Actor Object Reference") (OtherComp :type "PrimitiveComponent Object Reference") (OtherBodyIndex :type Integer) (bFromSweep :type Boolean) (SweepResult :type "HitResult Structure (by ref)"))
  (bind _enemy_npc_atk_dmg (`self.Enemy Npc Atk Dmg`))
  ;[1 1 1] 검 공격 피격
  (`|ExecutionSequence`
    (:`then_0`
      (if (`ActorComponent.ComponentHasTag` OtherComp "PlayerAllies")
        (bind _asbp_player (cast `/Game/TopDown/Blueprints/BP_Player` OtherActor))
        (`/Game/TopDown/Blueprints/BP_Player.DamagePlayer` _asbp_player _enemy_npc_atk_dmg)))
    (:`then_1`
      (if (`ActorComponent.ComponentHasTag` OtherComp "BuildingAllies")
        (message `/Game/TopDown/Blueprints/Interface/BPI_Hitable.Take Damage` OtherActor false _enemy_npc_atk_dmg)))))

(fn `UserConstructionScript`
  (`parent.UserConstructionScript`))