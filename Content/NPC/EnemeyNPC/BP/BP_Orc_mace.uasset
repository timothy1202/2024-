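; Mace-wielding orc enemy NPC that alternates a normal downward melee attack with a periodic 360-degree mace skill.
; A looping timer started on BeginPlay fires the skill, pausing itself if a normal attack is flagged.
; Attack plays the normal montage unless the orc is dead or skilling, then passes its duration to NormalAttack.
; NormalAttack clears the attack flag and re-enters any pending skill, which unpauses the timer.
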(event `self.ReceiveBeginPlay`
  ;[1 1 1] 철퇴 스킬
  (`parent.ReceiveBeginPlay`)
  (bind _returnvalue (`KismetSystemLibrary.K2_SetTimerDelegate` (delegate `Mace Skill`) 7.0 true)))

(event `Mace Skill`
  ;[1 1 1] 철퇴 스킬
  (set `self.isMaceSkilling` true)
  (if (`self.isNormalAttacking`) :!label _label
    (`KismetSystemLibrary.K2_PauseTimerHandle` (stale `self.ReceiveBeginPlay` _returnvalue))
    (else
      (`KismetSystemLibrary.K2_UnPauseTimerHandle` (stale `self.ReceiveBeginPlay` _returnvalue))
      (`self.PlayAnimMontage` "/Game/Animations/ORC_IRON_MACE_Animation/Mace_Skill_AttackStanding_Melee_Attack_360_High_Fixed_Montage.Mace_Skill_AttackStanding_Melee_Attack_360_High_Fixed_Montage")
      (set `self.isMaceSkilling` false))))

(event `NormalAttack`
  (params (Duration :type "Float (double-precision)"))
  ;[1 1 1] 기본 공격
  (set `self.isNormalAttacking` false)
  (if (`self.isMaceSkilling`)
    (goto _label)))

(fn `Attack`
  (returns (`Animation Duration` :type "Float (double-precision)"))
  (if (`self.IsNPCDead?`)
    _
    (elif (not (`self.isMaceSkilling`))
      (set `self.isNormalAttacking` true)
      (bind _returnvalue (`self.PlayAnimMontage` "/Game/Animations/ORC_IRON_MACE_Animation/Mace_Normal_AttackStanding_Melee_Attack_Downward_Fixed_Montage.Mace_Normal_AttackStanding_Melee_Attack_Downward_Fixed_Montage"))
      (`self.NormalAttack` _returnvalue)
      (return _returnvalue))))

(fn `UserConstructionScript`
  (`parent.UserConstructionScript`))