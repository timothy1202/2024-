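; Lizard wizard enemy NPC Blueprint that attacks with fireballs, built on a parent NPC class whose skill use it turns off at BeginPlay.
; Attack locks movement, plays a spell montage and passes its length to an event that restores walking afterward.
; A separate SpawnFireBall event spawns the projectile at the right-thumb socket.
; Tick watches for death and, once, stops movement, plays the death montage, calls NpcDead and destroys the actor after a delay.
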(event `self.ReceiveTick`
  (params (DeltaSeconds :type "Float (single-precision)"))
  ;[1 1 1] 플레이어 사망 체크
  (if (`self.IsNPCDead?`)
    (`/Engine/EditorBlueprintResources/StandardMacros.DoOnce` false
      (:`Completed`
        (`CharacterMovementComponent.DisableMovement` (`self.CharacterMovement`))
        (`self.PlayAnimMontage` "/Game/Assets/DrakeAssassin/Animations/Anim_DrakeAssassin_death_Montage.Anim_DrakeAssassin_death_Montage")
        (`self.NpcDead`)
        (`KismetSystemLibrary.Delay` 2.5)
        (`self.K2_DestroyActor`)))))

(event `SpawnFireBall`
  ;[1 1 1] 파이어 볼 생성
  (`|SpawnActorFromClass` "/Game/NPC/EnemeyNPC/BP/Weapon_BP/BP_Lizard_Fireball.BP_Lizard_Fireball_C" (`KismetMathLibrary.MakeTransform` (`SceneComponent.GetSocketLocation` (`self.Mesh`) "thumb_03_r_Socket") (`self.K2_GetActorRotation` self)) "Undefined" "MultiplyWithRoot" null null))

(event `self.ReceiveBeginPlay`
  ;[1 1 1] 부모의 스킬 사용 방지
  (set `self.PlaySkill` false)
  (`parent.ReceiveBeginPlay`))

(event `LizardWizard_NormalAttack`
  (params (duration :type "Float (double-precision)"))
  ;[1 1 1] 기본공격
  (`KismetSystemLibrary.Delay` duration)
  (`CharacterMovementComponent.SetMovementMode` (`self.CharacterMovement`) "MOVE_Walking" 0))

(fn `Attack`
  (returns (`Animation Duration` :type "Float (double-precision)"))
  (if (not (`self.IsNPCDead?`))
    (`CharacterMovementComponent.DisableMovement` (`self.CharacterMovement`))
    (bind _returnvalue (`self.PlayAnimMontage` "/Game/Assets/DrakeAssassin/Animations/Anim_DrakeAssassin_spell02_Montage.Anim_DrakeAssassin_spell02_Montage"))
    (`self.LizardWizard_NormalAttack` _returnvalue)
    (return _returnvalue)))

(fn `UserConstructionScript`
  (`parent.UserConstructionScript`))