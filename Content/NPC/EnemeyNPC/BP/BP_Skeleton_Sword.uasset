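; Sword-wielding skeleton enemy NPC that builds on a parent class for shared setup and behavior.
; BeginPlay loads data table row "6001", which feeds default settings such as walk speed.
; Attack plays a sword montage unless the NPC is dead.
; Tick, labeled death check and revive, spawns another skeleton with its behavior tree in place and clears the dead flag, with no condition in this graph.
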(event `self.ReceiveBeginPlay`
  ;[1 1 1] 코멘트
  (`/Game/NPC/EnemeyNPC/AI/Interface/BPI_AI_BehaviorTrees.GetDataTable` "6001")
  (`parent.ReceiveBeginPlay`))

(event `self.ReceiveTick`
  (params (DeltaSeconds :type "Float (single-precision)"))
  ;[1 1 1] 플레이어 사망 체크 & 부활
  (`parent.ReceiveTick` 0.0)
  (`AIBlueprintHelperLibrary.SpawnAIFromClass` "BP_Skeleton_Sword_C" "/Game/NPC/EnemeyNPC/AI/BT/BT_Skeleton_Sword.BT_Skeleton_Sword" (`self.K2_GetActorLocation`) (`self.K2_GetActorRotation`) false null)
  (set `self.IsNPCDead?` false))

(event `/Game/NPC/EnemeyNPC/AI/Interface/BPI_AI_BehaviorTrees.GetDataTable`
  (params (RowName :type Name))
  ;[1 1 1] 데이터 테이블 변수화
  (`parent.GetDataTable` RowName)
  (`self.DefaultSetting_SkSword`))

(event `DefaultSetting_SkSword`
  ;[1 1 1] 디폴트 세팅 설정
  (set `CharacterMovementComponent.MaxWalkSpeed` (`self.Enemy Npc Walk Speed`) (`self.CharacterMovement`)))

(fn `Attack`
  (returns (`Animation Duration` :type "Float (double-precision)"))
  (if (not (`self.IsNPCDead?`))
    (bind _returnvalue (`self.PlayAnimMontage` "/Game/Assets/SkeletonEnemy/Animations/Anim_Attack_Sword_1_Montage.Anim_Attack_Sword_1_Montage"))
    (return _returnvalue)))

(fn `UserConstructionScript`
  (`parent.UserConstructionScript`))