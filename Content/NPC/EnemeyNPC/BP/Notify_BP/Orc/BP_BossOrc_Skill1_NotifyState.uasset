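; Anim notify state for the Boss Orc's first skill, marking the window in which the mace attack is active.
; On begin, it enables query and physics collision on the owner's first mace collider and activates the matching trail effect.
; On end, it disables that collision, deactivates the trail and clears the boss's IsPlayingSkill flag.
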(fn `Received_NotifyBegin`
  (params (MeshComp :type "SkeletalMeshComponent Object Reference") (Animation :type "AnimSequenceBase Object Reference") (TotalDuration :type "Float (single-precision)") (EventReference :type "AnimNotifyEventReference Structure (by ref)"))
  (returns (ReturnValue :type Boolean))
  (bind _asbp_boss_orc (cast `/Game/NPC/EnemeyNPC/BP/hunt/BP_Boss_Orc` (`ActorComponent.GetOwner` MeshComp)))
  (`PrimitiveComponent.SetCollisionEnabled` (`/Game/NPC/EnemeyNPC/BP/hunt/BP_Boss_Orc.MaceCollsion1` _asbp_boss_orc) "QueryAndPhysics")
  (`ActorComponent.Activate` (`/Game/NPC/EnemeyNPC/BP/hunt/BP_Boss_Orc.TrailEffect1` _asbp_boss_orc) false)
  (return false))

(fn `Received_NotifyEnd`
  (params (MeshComp :type "SkeletalMeshComponent Object Reference") (Animation :type "AnimSequenceBase Object Reference") (EventReference :type "AnimNotifyEventReference Structure (by ref)"))
  (returns (ReturnValue :type Boolean))
  (bind _asbp_boss_orc (cast `/Game/NPC/EnemeyNPC/BP/hunt/BP_Boss_Orc` (`ActorComponent.GetOwner` MeshComp)))
  (`PrimitiveComponent.SetCollisionEnabled` (`/Game/NPC/EnemeyNPC/BP/hunt/BP_Boss_Orc.MaceCollsion1` _asbp_boss_orc) "NoCollision")
  (`ActorComponent.Deactivate` (`/Game/NPC/EnemeyNPC/BP/hunt/BP_Boss_Orc.TrailEffect1` _asbp_boss_orc))
  (set `EnemyBase.is_playing_skill` false _asbp_boss_orc)
  (return false))