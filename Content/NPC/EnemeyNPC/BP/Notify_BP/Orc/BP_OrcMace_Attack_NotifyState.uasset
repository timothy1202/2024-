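; Anim notify state that opens the orc mace's hit window during attack animations.
; On begin it casts the mesh owner to BP_Orc_mace and sets its MaceCollsion component to QueryAndPhysics.
; On end it sets that collision back to NoCollision, so the mace collides only within the notify's span.
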(fn `Received_NotifyBegin`
  (params (MeshComp :type "SkeletalMeshComponent Object Reference") (Animation :type "AnimSequenceBase Object Reference") (TotalDuration :type "Float (single-precision)") (EventReference :type "AnimNotifyEventReference Structure (by ref)"))
  (returns (ReturnValue :type Boolean))
  (bind _asbp_orc_mace (cast `/Game/NPC/EnemeyNPC/BP/hunt/BP_Orc_mace` (`ActorComponent.GetOwner` MeshComp)))
  (`PrimitiveComponent.SetCollisionEnabled` (`/Game/NPC/EnemeyNPC/BP/hunt/BP_Orc_mace.MaceCollsion` _asbp_orc_mace) "QueryAndPhysics")
  (return false))

(fn `Received_NotifyEnd`
  (params (MeshComp :type "SkeletalMeshComponent Object Reference") (Animation :type "AnimSequenceBase Object Reference") (EventReference :type "AnimNotifyEventReference Structure (by ref)"))
  (returns (ReturnValue :type Boolean))
  (bind _asbp_orc_mace (cast `/Game/NPC/EnemeyNPC/BP/hunt/BP_Orc_mace` (`ActorComponent.GetOwner` MeshComp)))
  (`PrimitiveComponent.SetCollisionEnabled` (`/Game/NPC/EnemeyNPC/BP/hunt/BP_Orc_mace.MaceCollsion` _asbp_orc_mace) "NoCollision")
  (return false))