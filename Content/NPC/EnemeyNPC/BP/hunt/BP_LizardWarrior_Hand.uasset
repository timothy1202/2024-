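; Melee lizard warrior enemy NPC, a child Blueprint that attacks players and allied buildings and regenerates health after taking damage.
; A looping cooldown timer, enabled by PlaySkill, flags the next Attack to spawn a sector indicator and play the skill montage instead of the normal one.
; Tag-filtered hand overlaps deal damage: left for claw skill, right for normal attack.
; Damage pauses healing, then a delay starts timed regeneration; death clears the skill timer.
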(event `self.LeftHandAttackCollision.OnComponentBeginOverlap`
  (params (OverlappedComponent :type "PrimitiveComponent Object Reference") (OtherActor :type "Actor Object Reference") (OtherComp :type "PrimitiveComponent Object Reference") (OtherBodyIndex :type Integer) (bFromSweep :type Boolean) (SweepResult :type "HitResult Structure (by ref)"))
  ;[1 1 1] 아군이 스킬에 닿으면 피해 입음
  (`|ExecutionSequence`
    (:`then_0`
      (if (`ActorComponent.ComponentHasTag` OtherComp "PlayerAllies")
        (bind _asbp_player (cast `/Game/TopDown/Blueprints/BP_Player` OtherActor))
        (`/Game/TopDown/Blueprints/BP_Player.DamagePlayer` _asbp_player (`self.Claw Skill Atk Dmg`))))
    (:`then_1`
      (if (`ActorComponent.ComponentHasTag` OtherComp "BuildingAllies")
        (bind _asbp_base_building (cast `/Game/Building/BP_BaseBuilding` OtherActor))
        (`/Game/Building/BP_BaseBuilding.Take Damage` _asbp_base_building (`self.Claw Skill Atk Dmg`))))))

(event `self.RightHandAttackCollision.OnComponentBeginOverlap`
  (params (OverlappedComponent :type "PrimitiveComponent Object Reference") (OtherActor :type "Actor Object Reference") (OtherComp :type "PrimitiveComponent Object Reference") (OtherBodyIndex :type Integer) (bFromSweep :type Boolean) (SweepResult :type "HitResult Structure (by ref)"))
  ;[1 1 1] 아군이 손에 닿으면 피해 입음
  (`|ExecutionSequence`
    (:`then_0`
      (if (`ActorComponent.ComponentHasTag` OtherComp "PlayerAllies")
        (bind _asbp_player (cast `/Game/TopDown/Blueprints/BP_Player` OtherActor))
        (`/Game/TopDown/Blueprints/BP_Player.DamagePlayer` _asbp_player (`self.Enemy Npc Atk Dmg`))))
    (:`then_1`
      (if (`ActorComponent.ComponentHasTag` OtherComp "BuildingAllies")
        (bind _asbp_base_building (cast `/Game/Building/BP_BaseBuilding` OtherActor))
        (`/Game/Building/BP_BaseBuilding.Take Damage` _asbp_base_building (`self.Enemy Npc Atk Dmg`))))))

(event `self.NpcDead`
  ;[1 1 1] 죽으면 스킬 실행 못하게
  (if (`self.IsNPCDead?`)
    (`KismetSystemLibrary.K2_ClearAndInvalidateTimerHandle` (`self.SkillHandle`))
    (`parent.NpcDead`)))

(event `self.ReceiveBeginPlay`
  ;[1 1 1] 자식 스킬 사용 안하게 & 근접 리자드맨 스킬
  (`parent.ReceiveBeginPlay`)
  (if (`self.PlaySkill`)
    (bind _returnvalue (`KismetSystemLibrary.K2_SetTimerDelegate` (delegate `HandAttackSkill`) (`self.Enemy Skill Cool Time`) true))
    (set `self.SkillHandle` _returnvalue)))

(event `HandAttackSkill`
  ;[1 1 1] 자식 스킬 사용 안하게 & 근접 리자드맨 스킬
  (set `self.isPlayingSkill` true))

(event `/Game/TopDown/Blueprints/Interface/BPI_Hitable.Take Damage`
  (params (damageValue :type "Float (double-precision)"))
  ;[1 0.9867 0.9186] 코멘트
  (`parent.Take Damage` damageValue)
  (set `self.CanRecover` false)
  (`KismetSystemLibrary.Delay` (`self.Lizard No Hit Time`))
  (set `self.CanRecover` true)
  (bind _returnvalue (`KismetSystemLibrary.K2_SetTimerDelegate` (delegate `GetHealed`) (`self.Lizard Regen Time`) true))
  (set `self.HealTimer` _returnvalue)
  (`self.Update Healed Health Bar` (`self.Lizard Hp Regen`)))

(event `GetHealed`
  (bind _healtimer (`self.HealTimer`))
  ;[1 0.9867 0.9186] 코멘트
  ;;[0.05098 0.05098 0.05098] 자힐
  (if (`self.CanRecover`)
    (if (< (`self.curHealth`) (`self.Enemy Npc Max Health`))
      (set `self.curHealth` (+ (`self.curHealth`) (`self.Lizard Hp Regen`)))
      (else
        (`KismetSystemLibrary.K2_ClearAndInvalidateTimerHandle` _healtimer)))
    (else
      (`KismetSystemLibrary.K2_ClearAndInvalidateTimerHandle` _healtimer))))

(fn `Attack`
  (returns (`Animation Duration` :type "Float (double-precision)"))
  (if (`self.IsNPCDead?`)
    _
    (elif (`self.isPlayingSkill`)
      (`|SpawnActorFromClass` "/Game/indicator/BP_CircularSectorIndicator_outline.BP_CircularSectorIndicator_outline_C" (`SceneComponent.K2_GetComponentToWorld` (`self.indicator`)) "Undefined" "MultiplyWithRoot" null null)
      (bind _returnvalue (`AnimInstance.Montage_Play` (`SkeletalMeshComponent.GetAnimInstance` (`self.Mesh`)) "/Game/Animations/Melee/DrakeWarrior_Skill_Montage.DrakeWarrior_Skill_Montage" (`self.Enemy Skill Atk Spd`) "Duration" 0.0 true))
      (set `self.isPlayingSkill` false)
      (return _returnvalue)
      (else
        (bind _returnvalue_2 (`AnimInstance.Montage_Play` (`SkeletalMeshComponent.GetAnimInstance` (`self.Mesh`)) "/Game/Assets/DrakeWarrior/Animation/LizardWarriorAttack_Montage.LizardWarriorAttack_Montage" (`self.Enemy Npc Atk Spd`) "Duration" 0.0 true))
        (return _returnvalue_2)))))

(fn `NpcDown`)

(fn `Update Healed Health Bar`
  (params (`Heal Amount` :type "Float (double-precision)"))
  (set `self.curHealth` (+ (`self.curHealth`) `Heal Amount`))
  (return))

(fn `UserConstructionScript`
  (`parent.UserConstructionScript`))