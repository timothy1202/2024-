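; Skeleton enemy NPC that attacks with both hands, damaging the player, allied buildings and the friendly base.
; Attack plays a double-attack montage and returns its duration.
; Left and right hand collision overlaps apply the NPC attack damage, checking component tags for player and buildings but only casting for the friendly base.
; When Resurrection is set, BeginPlay plays a recycle montage and delays parent initialization until it ends.
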(event `self.LeftHandAttackCollision.OnComponentBeginOverlap`
  (params (OverlappedComponent :type "PrimitiveComponent Object Reference") (OtherActor :type "Actor Object Reference") (OtherComp :type "PrimitiveComponent Object Reference") (OtherBodyIndex :type Integer) (bFromSweep :type Boolean) (SweepResult :type "HitResult Structure (by ref)"))
  (bind _enemynpc_atkdmg (`self.EnemyNpc_AtkDmg`))
  ;[1 1 1] 오른손 공격 피격
  (`|ExecutionSequence`
    (:`then_0`
      (if (`ActorComponent.ComponentHasTag` OtherComp "PlayerAllies")
        (bind _asbp_player (cast `/Game/TopDown/Blueprints/BP_Player` OtherActor))
        (`/Game/TopDown/Blueprints/BP_Player.DamagePlayer` _asbp_player _enemynpc_atkdmg)))
    (:`then_1`
      (if (`ActorComponent.ComponentHasTag` OtherComp "BuildingAllies")
        (bind _asbp_base_building (cast `/Game/Building/BP_BaseBuilding` OtherActor))
        (`/Game/Building/BP_BaseBuilding.Take Damage` _asbp_base_building false _enemynpc_atkdmg)))
    (:`then_2`
      (bind _asbp_my_friendly_base (cast `/Game/NPC/FriendlyNPC/BP/BP_MyFriendlyBase` OtherActor))
      (`/Game/NPC/FriendlyNPC/BP/BP_MyFriendlyBase.Take Damage` _asbp_my_friendly_base false _enemynpc_atkdmg))))

(event `self.RightHandAttackCollision.OnComponentBeginOverlap`
  (params (OverlappedComponent :type "PrimitiveComponent Object Reference") (OtherActor :type "Actor Object Reference") (OtherComp :type "PrimitiveComponent Object Reference") (OtherBodyIndex :type Integer) (bFromSweep :type Boolean) (SweepResult :type "HitResult Structure (by ref)"))
  (bind _enemynpc_atkdmg (`self.EnemyNpc_AtkDmg`))
  ;[1 1 1] 오른손 공격 피격
  (`|ExecutionSequence`
    (:`then_0`
      (if (`ActorComponent.ComponentHasTag` OtherComp "PlayerAllies")
        (bind _asbp_player (cast `/Game/TopDown/Blueprints/BP_Player` OtherActor))
        (`/Game/TopDown/Blueprints/BP_Player.DamagePlayer` _asbp_player _enemynpc_atkdmg)))
    (:`then_1`
      (if (`ActorComponent.ComponentHasTag` OtherComp "BuildingAllies")
        (bind _asbp_base_building (cast `/Game/Building/BP_BaseBuilding` OtherActor))
        (`/Game/Building/BP_BaseBuilding.Take Damage` _asbp_base_building false _enemynpc_atkdmg)))
    (:`then_2`
      (bind _asbp_my_friendly_base (cast `/Game/NPC/FriendlyNPC/BP/BP_MyFriendlyBase` OtherActor))
      (`/Game/NPC/FriendlyNPC/BP/BP_MyFriendlyBase.Take Damage` _asbp_my_friendly_base false _enemynpc_atkdmg))))

(event `self.ReceiveBeginPlay`
  ;[1 1 1] 코멘트
  (if (`self.resurrection?`)
    (bind _returnvalue (`AnimInstance.Montage_Play` (`SkeletalMeshComponent.GetAnimInstance` (`self.Mesh`)) "/Game/Animations/Anim_Recycle_Montage.Anim_Recycle_Montage" 1.0 "Duration" 0.0 true))
    (`KismetSystemLibrary.Delay` _returnvalue)
    (`parent.ReceiveBeginPlay`)
    (else
      (`parent.ReceiveBeginPlay`))))

(fn `Attack`
  (returns (`Animation Duration` :type "Float (double-precision)"))
  (bind _returnvalue (`AnimInstance.Montage_Play` (`SkeletalMeshComponent.GetAnimInstance` (`self.Mesh`)) "/Game/Assets/SkeletonEnemy/Animations/SK_Skeleton_AttackDouble_Montage.SK_Skeleton_AttackDouble_Montage" 1.0 "Duration" 0.0 true))
  (return _returnvalue))

(fn `UserConstructionScript`
  (`parent.UserConstructionScript`))