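; BP_LizardWizard is a ranged enemy NPC that attacks with fireballs, built on a parent NPC Blueprint.
; BeginPlay turns off PlaySkill to block the parent's skill and flags the NPC as long-range before running parent initialization.
; Attack plays a spell montage and returns its duration.
; A separate SpawnFireBall event spawns BP_Lizard_Fireball at the AttackDirection component's location and rotation.
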(event `SpawnFireBall`
  (bind _attackdirection (`self.AttackDirection`))
  ;[1 1 1] 파이어 볼 생성
  (`|SpawnActorFromClass` "/Game/NPC/EnemeyNPC/BP/Weapon_BP/BP_Lizard_Fireball.BP_Lizard_Fireball_C" (`KismetMathLibrary.MakeTransform` (`SceneComponent.K2_GetComponentLocation` _attackdirection) (`SceneComponent.K2_GetComponentRotation` _attackdirection)) "Undefined" "MultiplyWithRoot" null null))

(event `self.ReceiveBeginPlay`
  ;[1 1 1] 부모의 스킬 사용 방지
  (set `self.PlaySkill` false)
  (set `self.is_long_range_npc` true)
  (`parent.ReceiveBeginPlay`))

(fn `Attack`
  (returns (`Animation Duration` :type "Float (double-precision)"))
  (bind _returnvalue (`AnimInstance.Montage_Play` (`SkeletalMeshComponent.GetAnimInstance` (`self.Mesh`)) "/Game/Assets/DrakeAssassin/Animations/Anim_DrakeAssassin_spell02_Montage.Anim_DrakeAssassin_spell02_Montage" 1.0 "Duration" 0.0 true))
  (return _returnvalue))

(fn `UserConstructionScript`
  (`parent.UserConstructionScript`))