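; Skeleton archer enemy NPC that extends a parent NPC class, flagging itself as long-range on BeginPlay.
; Attack plays a bow montage, and ShootArrow spawns a BP_Arrow at the Arrow1 component, firing it at the AI blackboard's AttackTarget.
; DestroyActor, gated by FirstTimeToDie, spawns a BP_Skeleton_Hand at the capsule whether aggressive or not, then destroys the archer.
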(event `self.ReceiveBeginPlay`
  (set `self.bFirstTimeToDie?` true)
  (set `self.is_long_range_npc` true)
  (`parent.ReceiveBeginPlay`))

(event `ShootArrow`
  (bind (_returnvalue_location _returnvalue_rotation) (`KismetMathLibrary.BreakTransform` (`SceneComponent.K2_GetComponentToWorld` (`self.Arrow1`))))
  ;[1 1 1] 활 공격
  (bind _returnvalue (`|SpawnActorFromClass` "/Game/NPC/EnemeyNPC/BP/Weapon_BP/BP_Arrow.BP_Arrow_C" (`KismetMathLibrary.MakeTransform` _returnvalue_location _returnvalue_rotation) "AlwaysSpawn" "MultiplyWithRoot" null null))
  (bind `_as액터` (cast `Actor` (`BlackboardComponent.GetValueAsObject` (`AIBlueprintHelperLibrary.GetBlackboard` (`AIBlueprintHelperLibrary.GetAIController` self)) (`self.AttackTarget`))))
  (`/Game/NPC/EnemeyNPC/BP/Weapon_BP/BP_Arrow.ShootArrow` _returnvalue `_as액터`))

(event `self.DestroyActor`
  (bind _returnvalue (`SceneComponent.K2_GetComponentToWorld` (`self.CapsuleComponent`)))
  ;[1 1 1] 코멘트
  (if (`self.bFirstTimeToDie?`)
    (if (`self.aggresive`)
      (`|SpawnActorFromClass` "/Game/NPC/EnemeyNPC/BP/hunt/BP_Skeleton_Hand.BP_Skeleton_Hand_C" _returnvalue "Undefined" "MultiplyWithRoot" null true "6000" true null)
      (else
        (`|SpawnActorFromClass` "/Game/NPC/EnemeyNPC/BP/hunt/BP_Skeleton_Hand.BP_Skeleton_Hand_C" _returnvalue "Undefined" "MultiplyWithRoot" null true "6000" true null)))
    (`self.K2_DestroyActor`)))

(fn `Attack`
  (returns (`Animation Duration` :type "Float (double-precision)"))
  (bind _returnvalue (`AnimInstance.Montage_Play` (`SkeletalMeshComponent.GetAnimInstance` (`self.Mesh`)) "/Game/Assets/SkeletonEnemy/Animations/Anim_AttackBow_Montage.Anim_AttackBow_Montage" 1.0 "Duration" 0.0 true))
  (return _returnvalue))

(fn `UserConstructionScript`
  (`parent.UserConstructionScript`))