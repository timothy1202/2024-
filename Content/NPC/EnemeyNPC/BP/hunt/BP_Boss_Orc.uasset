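; Orc boss NPC that fights the player, buildings and the friendly base with a mace and area skills.
; Entering phase 2 or 3 starts looping timers that flag special skills, which the Attack override plays as montages, prioritizing phase 3 and otherwise using the parent attack.
; Mace overlaps deal damage or, on landscape when armed, spawn a ground shockwave.
; Helper functions spawn the normal attack shockwave and circle indicator.
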(event `self.ReceiveBeginPlay`
  ;[1 1 1] 코멘트
  (`parent.ReceiveBeginPlay`)
  (`BlackboardComponent.SetValueAsFloat` (`AIBlueprintHelperLibrary.GetBlackboard` (`AIBlueprintHelperLibrary.GetAIController` self)) (`self.StopDistance`) 400.0)
  (set `self.MaceDamge` (`self.Boss Skill 2 Dmg`)))

(event `self.MaceCollsion1.OnComponentBeginOverlap`
  (params (OverlappedComponent :type "PrimitiveComponent Object Reference") (OtherActor :type "Actor Object Reference") (OtherComp :type "PrimitiveComponent Object Reference") (OtherBodyIndex :type Integer) (bFromSweep :type Boolean) (SweepResult :type "HitResult Structure (by ref)"))
  ;[1 1 1] 코멘트
  (bind _asbp_player (cast `/Game/TopDown/Blueprints/BP_Player` OtherActor)
    (:`then`
      (`/Game/TopDown/Blueprints/BP_Player.DamagePlayer` _asbp_player (`self.MaceDamge`)))
    (:`CastFailed`
      (bind _asbase_building (cast `BaseBuilding` OtherActor)
        (:`then`
          (message `/Game/TopDown/Blueprints/Interface/BPI_Hitable.Take Damage` _asbase_building false (`self.MaceDamge`)))
        (:`CastFailed`
          (bind _asbp_my_friendly_base (cast `/Game/NPC/FriendlyNPC/BP/BP_MyFriendlyBase` OtherActor)
            (:`then`
              (`/Game/NPC/FriendlyNPC/BP/BP_MyFriendlyBase.Take Damage` _asbp_my_friendly_base false (`self.MaceDamge`)))
            (:`CastFailed`
              (if (and (`self.ActorHasTag` OtherActor "Landscape") (`self.readyToSpawnSkill3Effect`))
                (`self.Spawn Skill 2 Effect`)))))))))

(event `self.Enter Page 3`
  ;[1 1 1] 코멘트
  (`KismetSystemLibrary.K2_SetTimerDelegate` (delegate `Activate Page 3`) 15.0 true))

(event `Activate Page 3`
  ;[1 1 1] 코멘트
  (set `self.Playing_page_three_skill` true))

(event `self.Enter Page 2`
  ;[1 1 1] 코멘트
  (`KismetSystemLibrary.K2_SetTimerDelegate` (delegate `Activate Page2`) 10.0 true))

(event `Activate Page2`
  ;[1 1 1] 코멘트
  (set `self.Playing_page_two_skill` true))

(fn `Attack`
  (returns (`Animation Duration` :type "Float (double-precision)"))
  (bind _returnvalue (`self.CheckHighestATPAginstPlayer`))
  (set `self.is_highest_atp_player` _returnvalue)
  (if (`self.IsNpcDead`)
    _
    (elif (`self.Playing_page_three_skill`)
      (bind _returnvalue_2 (`AnimInstance.Montage_Play` (`SkeletalMeshComponent.GetAnimInstance` (`self.Mesh`)) "/Game/Animations/BOSS_ORC_HAM_Animation/Skill3_roaringRoaring_Attack.Skill3_roaringRoaring_Attack" 1.4 "Duration" 0.0 true))
      (return _returnvalue_2)
      (elif (`self.Playing_page_two_skill`)
        (set `self.MaceDamge` (`self.Boss Skill 3 Dmg`))
        (bind _returnvalue_3 (`AnimInstance.Montage_Play` (`SkeletalMeshComponent.GetAnimInstance` (`self.Mesh`)) "/Game/Animations/BOSS_ORC_HAM_Animation/SKill2_Combo_HAMSkill1_Combo_attack_Ham.SKill2_Combo_HAMSkill1_Combo_attack_Ham" (`self.Skill_Atk_Spd`) "Duration" 0.0 true))
        (return _returnvalue_3)
        (else
          (bind _animation_duration (`parent.Attack`))
          (return _animation_duration))))))

(fn `Spawn Normal Attack Effect`
  (bind (_returnvalue_x _returnvalue_y _returnvalue_z) (`KismetMathLibrary.BreakVector` (`SceneComponent.K2_GetComponentLocation` (`self.CapsuleComponent`))))
  (`GameplayStatics.PlaySoundAtLocation` "/Game/Assets/Sounds/NPC/Lizard/Boss_Orc_Lizard_Combo_JumpLanding_Explosion.Boss_Orc_Lizard_Combo_JumpLanding_Explosion" (`self.K2_GetActorLocation`) (struct) 1.0 1.0 0.0 "/Game/NPC/EnemeyNPC/BP/EnemyNPC_SoundAttenuation.EnemyNPC_SoundAttenuation" null null null)
  (`|SpawnActorFromClass` "/Game/NPC/EnemeyNPC/BP/Effect/BP_Boss_GroundAttack_Effect.BP_Boss_GroundAttack_Effect_C" (`KismetMathLibrary.MakeTransform` (`KismetMathLibrary.MakeVector` _returnvalue_x _returnvalue_y (- _returnvalue_z 165.0))) "AlwaysSpawn" "MultiplyWithRoot" null self (`self.Boss Skill 1 Dmg`) null))

(fn `Spawn Skill 2 Effect`
  (bind (_returnvalue_x _returnvalue_y _returnvalue_z) (`KismetMathLibrary.BreakVector` (`SceneComponent.GetSocketLocation` (`self.TrailEffect1`) "None")))
  (`|SpawnActorFromClass` "/Game/NPC/EnemeyNPC/BP/Effect/BP_Boss_GroundAttack_Effect.BP_Boss_GroundAttack_Effect_C" (`KismetMathLibrary.MakeTransform` (`KismetMathLibrary.MakeVector` _returnvalue_x _returnvalue_y (- _returnvalue_z 300.0)) (struct) (1.0 1.0 5.0)) "AlwaysSpawn" "MultiplyWithRoot" null self (`self.Boss Skill 3 Dmg`) null)
  (`GameplayStatics.PlaySoundAtLocation` "/Game/Assets/Sounds/NPC/Lizard/Boss_Orc_Lizard_Combo_JumpLanding_Explosion.Boss_Orc_Lizard_Combo_JumpLanding_Explosion" (`self.K2_GetActorLocation`) (struct) 1.0 1.0 0.0 "/Game/NPC/EnemeyNPC/BP/EnemyNPC_SoundAttenuation.EnemyNPC_SoundAttenuation" null null null)
  (`KismetSystemLibrary.PrintString` "sss"))

(fn `Spawn Skill 3 Effect`
  (bind (_returnvalue_x _returnvalue_y _returnvalue_z) (`KismetMathLibrary.BreakVector` (`SceneComponent.K2_GetComponentLocation` (`self.CapsuleComponent`))))
  (`|SpawnActorFromClass` "/Game/NPC/EnemeyNPC/BP/Effect/BP_Boss_Orc_Circle_Indicator.BP_Boss_Orc_Circle_Indicator_C" (`KismetMathLibrary.MakeTransform` (`KismetMathLibrary.MakeVector` _returnvalue_x _returnvalue_y (- _returnvalue_z 150.0))) "AlwaysSpawn" "MultiplyWithRoot" null (`self.Boss Skill 4 Dmg`) null))

(fn `UserConstructionScript`
  (`parent.UserConstructionScript`))