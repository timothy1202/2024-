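; Ranged skeleton wizard enemy NPC that shoots fireballs and summons BP_Skeleton_Hand minions at random nearby points.
; A looping cooldown timer only raises the skill flag, and is cleared on death.
; Attack picks the montage from that flag, with boss skeletons also checking highest-player and first-skill flags.
; Separate events spawn the fireball and minion, and a helper function spawns the boss spawn effect near ground height.
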(event `SpawnSkeletonFireBall`
  (bind _attackdirection (`self.AttackDirection`))
  ;[1 1 1] 파이어볼 공격
  (`|SpawnActorFromClass` "/Game/NPC/EnemeyNPC/BP/Weapon_BP/BP_Skeleton_Fireball.BP_Skeleton_Fireball_C" (`KismetMathLibrary.MakeTransform` (`SceneComponent.K2_GetComponentLocation` _attackdirection) (`SceneComponent.K2_GetComponentRotation` _attackdirection)) "Undefined" "MultiplyWithRoot" null null))

(event `self.ReceiveBeginPlay`
  ;[1 1 1] 근접 스켈레톤 소환
  (set `self.is_long_range_npc` true)
  (`parent.ReceiveBeginPlay`)
  (bind _returnvalue (`KismetSystemLibrary.K2_SetTimerDelegate` (delegate `SpawnActorAtRandomLocation`) (`self.Skill_Cool_Time`) true))
  (set `self.SpawnTimerHandle` _returnvalue))

(event `SpawnActorAtRandomLocation`
  ;[1 1 1] 근접 스켈레톤 소환
  (set `self.is_playing_skill` true))

(event `SpawnSk`
  (bind (_returnvalue_x _returnvalue_y _returnvalue_z) (`KismetMathLibrary.BreakVector` (`self.K2_GetActorLocation`)))
  ;[1 1 1] 스폰
  (bind _output_get (set `self.EnemySpawnLocation` (`KismetMathLibrary.MakeVector` (+ _returnvalue_x (`KismetMathLibrary.RandomFloatInRange` -400.0 400.0)) (+ _returnvalue_y (`KismetMathLibrary.RandomFloatInRange` -400.0 400.0)) _returnvalue_z)))
  (if (`self.aggresive`)
    (`|SpawnActorFromClass` "/Game/NPC/EnemeyNPC/BP/hunt/BP_Skeleton_Hand.BP_Skeleton_Hand_C" (`KismetMathLibrary.MakeTransform` _output_get) "Undefined" "MultiplyWithRoot" null true "6000" true null)
    (else
      (`|SpawnActorFromClass` "/Game/NPC/EnemeyNPC/BP/hunt/BP_Skeleton_Hand.BP_Skeleton_Hand_C" (`KismetMathLibrary.MakeTransform` _output_get) "Undefined" "MultiplyWithRoot" null true "6000" true null)))
  (`KismetSystemLibrary.Delay` 1.0))

(event `self.NpcDead`
  ;[1 1 1] 죽으면 스킬 실행 못하게
  (if (`self.IsNpcDead`)
    (`KismetSystemLibrary.K2_ClearAndInvalidateTimerHandle` (`self.SpawnTimerHandle`))
    (`parent.NpcDead`)))

(fn `Attack`
  (returns (`Animation Duration` :type "Float (double-precision)"))
  (if (`self.IsNpcDead`)
    _
    (elif (`self.is_boss_skeleton`)
      (if (and (`self.is_playing_skill`) (`self.is_highest_atp_player`))
        (bind _returnvalue (`AnimInstance.Montage_Play` (`SkeletalMeshComponent.GetAnimInstance` (`self.Mesh`)) (`self.Second Skill Montage`) (`self.Skill_Atk_Spd`) "Duration" 0.0 true :!label _label))
        (return _returnvalue)
        (elif (`self.skeleton first skill playing`)
          (bind _returnvalue_2 (`AnimInstance.Montage_Play` (`SkeletalMeshComponent.GetAnimInstance` (`self.Mesh`)) (`self.AttackMontage`) 1.0 "Duration" 0.0 true))
          (set `self.skeleton first skill playing` false)
          (return _returnvalue_2)))
      (elif (`self.is_playing_skill`)
        (goto _label)
        (else
          (bind _returnvalue_3 (`AnimInstance.Montage_Play` (`SkeletalMeshComponent.GetAnimInstance` (`self.Mesh`)) "/Game/Animations/Magic_Skeleton_animation/Magic_SK_Normal_AttackStanding_1H_Magic_Attack_01__1__Fixed_Montage.Magic_SK_Normal_AttackStanding_1H_Magic_Attack_01__1__Fixed_Montage" 1.0 "Duration" 0.0 true))
          (return _returnvalue_3))))))

(fn `Skeleton Spawn Effect`
  (bind _returnvalue (`self.GetTransform` self))
  (`|SpawnActorFromClass` "/Game/NPC/EnemeyNPC/BP/Effect/BP_Boss_Skeleton_Spawn_Effect.BP_Boss_Skeleton_Spawn_Effect_C" (`KismetMathLibrary.MakeTransform` (`KismetMathLibrary.MakeVector` (.x (.location _returnvalue)) (.y (.location _returnvalue)) 5.0)) "AlwaysSpawn" "MultiplyWithRoot" null null))

(fn `UserConstructionScript`
  (`parent.UserConstructionScript`))