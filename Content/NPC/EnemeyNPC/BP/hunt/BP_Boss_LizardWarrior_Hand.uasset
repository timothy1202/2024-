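; Lizard warrior boss NPC that adds phase-based skills to its parent's attack.
; BeginPlay plays a roar before parent initialization; looping timers target page skill flags, though page two's misspells "Active" as "Acitve".
; Attack returns montage duration, prioritizing page-three roar, then page-two claw skill with sector indicator, for the highest-ATP player, otherwise using parent attack.
; Helpers spawn ground-attack and circle-indicator actors, and an event enables a timed fire-attack buff.
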(event `make_visible_skill3`
  ;[1 1 1] 기본공격(불) 강화 이펙트
  (`SceneComponent.SetVisibility` (`self.Skill3_effect`) true false)
  (set `self.is_fire_attack` true)
  (`KismetSystemLibrary.Delay` 10.0)
  (`SceneComponent.SetVisibility` (`self.Skill3_effect`) false false)
  (set `self.is_fire_attack` false))

(event `self.ReceiveBeginPlay`
  (bind _boss_skill_1_dmg (`self.Boss Skill 1 Dmg`))
  ;[1 1 1] 코멘트
  (bind _returnvalue (`AnimInstance.Montage_Play` (`SkeletalMeshComponent.GetAnimInstance` (`self.Mesh`)) "/Game/Assets/Red_LizardMan_Animation/BossLizardSpawn_AnimationMutant_Roaring_Montage.BossLizardSpawn_AnimationMutant_Roaring_Montage" 1.0 "Duration" 0.0 true))
  (`KismetSystemLibrary.Delay` _returnvalue)
  (`parent.ReceiveBeginPlay`)
  (set `self.EnemyNpc_AtkDmg` _boss_skill_1_dmg)
  (set `self.Claw_SkillAtkDmg` _boss_skill_1_dmg))

(fn `Active Page Three`
  (set `self.Playing_page_three_skill` true))

(fn `Active Page Two`
  (set `self.Playing_page_two_skill` true))

(fn `Attack`
  (returns (`Animation Duration` :type "Float (double-precision)"))
  (bind (_returnvalue_location _returnvalue_rotation) (`KismetMathLibrary.BreakTransform` (`self.GetTransform`)))
  (bind _returnvalue (`self.CheckHighestATPAginstPlayer`))
  (set `self.is_highest_atp_player` _returnvalue)
  (if (`self.IsNpcDead`)
    _
    (elif (and (`self.Playing_page_three_skill`) (`self.is_highest_atp_player`))
      (bind _returnvalue_2 (`AnimInstance.Montage_Play` (`SkeletalMeshComponent.GetAnimInstance` (`self.Mesh`)) "/Game/Assets/Red_LizardMan_Animation/Skill_3_Roaring.Skill_3_Roaring" (`self.Skill_Atk_Spd`) "Duration" 0.0 true))
      (return _returnvalue_2)
      (elif (and (`self.Playing_page_two_skill`) (`self.is_highest_atp_player`))
        (`|SpawnActorFromClass` "/Game/indicator/BP_CircularSectorIndicator_outline.BP_CircularSectorIndicator_outline_C" (`KismetMathLibrary.MakeTransform` _returnvalue_location _returnvalue_rotation (0.25 0.25 0.25)) "Undefined" "MultiplyWithRoot" null null)
        (set `self.Claw_SkillAtkDmg` (`self.Boss Skill 3 Dmg`))
        (bind _returnvalue_3 (`AnimInstance.Montage_Play` (`SkeletalMeshComponent.GetAnimInstance` (`self.Mesh`)) "/Game/Animations/Melee/DrakeWarrior_Skill_Montage.DrakeWarrior_Skill_Montage" (`self.Skill_Atk_Spd`) "Duration" 0.0 true))
        (return _returnvalue_3)
        (else
          (bind _animation_duration (`parent.Attack`))
          (return _animation_duration))))))

(fn `Enter Page Three`
  (`KismetSystemLibrary.K2_SetTimer` null "Active Page Three" 20.0 true))

(fn `Enter Page Two`
  (`KismetSystemLibrary.K2_SetTimer` null "Acitve Page Two" 10.0 true))

(fn `Spawn Second Skill Effect`
  (bind (_returnvalue_x _returnvalue_y) (`KismetMathLibrary.BreakVector` (`SceneComponent.K2_GetComponentLocation` (`self.CapsuleComponent`))))
  (`|SpawnActorFromClass` "/Game/NPC/EnemeyNPC/BP/Effect/BP_Boss_GroundAttack_Effect.BP_Boss_GroundAttack_Effect_C" (`KismetMathLibrary.MakeTransform` (`KismetMathLibrary.MakeVector` _returnvalue_x _returnvalue_y)) "AlwaysSpawn" "MultiplyWithRoot" null self (`self.Boss Skill 2 Dmg`) null))

(fn `Spawn Third Skill Indicator Effect`
  (bind (_returnvalue_x _returnvalue_y) (`KismetMathLibrary.BreakVector` (`SceneComponent.K2_GetComponentLocation` (`self.CapsuleComponent`))))
  (`|SpawnActorFromClass` "/Game/NPC/EnemeyNPC/BP/Effect/BP_Boss_Lizard_Circle_Indicator.BP_Boss_Lizard_Circle_Indicator_C" (`KismetMathLibrary.MakeTransform` (`KismetMathLibrary.MakeVector` _returnvalue_x _returnvalue_y)) "AlwaysSpawn" "MultiplyWithRoot" null null))

(fn `UserConstructionScript`
  (`parent.UserConstructionScript`))