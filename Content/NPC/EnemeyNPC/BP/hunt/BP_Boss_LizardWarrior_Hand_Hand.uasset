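; Boss NPC Blueprint for a Lizard Warrior "Hand" variant, which flags itself as a boss monster on BeginPlay before running parent setup.
; It overrides Attack: while alive and in a page-two or page-three skill, it plays the DrakeWarrior skill montage at skill attack speed.
; Otherwise a living boss falls back to the parent attack.
; Both skill phases use the same montage, and Attack returns the resulting value.
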(event `self.ReceiveBeginPlay`
  (set `self.isBossMonster` true)
  (`parent.ReceiveBeginPlay`))

(fn `Attack`
  (returns (`Animation Duration` :type "Float (double-precision)"))
  (if (`self.IsNpcDead`)
    _
    (elif (`self.playing_page_three_skill`)
      (bind _returnvalue (`AnimInstance.Montage_Play` (`SkeletalMeshComponent.GetAnimInstance` (`self.Mesh`)) "/Game/Animations/Melee/DrakeWarrior_Skill_Montage.DrakeWarrior_Skill_Montage" (`self.Skill_Atk_Spd`) "Duration" 0.0 true))
      (return _returnvalue)
      (elif (`self.playing_page_two_skill`)
        (bind _returnvalue_2 (`AnimInstance.Montage_Play` (`SkeletalMeshComponent.GetAnimInstance` (`self.Mesh`)) "/Game/Animations/Melee/DrakeWarrior_Skill_Montage.DrakeWarrior_Skill_Montage" (`self.Skill_Atk_Spd`) "Duration" 0.0 true))
        (return _returnvalue_2)
        (else
          (bind _animation_duration (`parent.Attack`))
          (return _animation_duration))))))

(fn `UserConstructionScript`
  (`parent.UserConstructionScript`))