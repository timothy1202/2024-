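; Skeleton boss NPC that extends its parent enemy with phase-based skills.
; Looping timers set skill flags, though EnterPageTwo's misspelled "Acitve Page Two" doesn't match ActivePageTwo.
; Attack plays meteor or summon montages when a flag and top-player check pass, otherwise falling back to the parent attack.
; Helper functions spawn target-homing fireballs, a charged big fireball, sword and archer skeletons, and randomly placed meteor indicators.
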(event `self.ReceiveBeginPlay`
  ;[1 1 1] 코멘트
  (set `self.is_boss_skeleton` true)
  (set `self.isBossMonster` true)
  (`parent.ReceiveBeginPlay`)
  (`KismetSystemLibrary.K2_SetTimerDelegate` (delegate `First Skill`) 5.0 true))

(event `First Skill`
  ;[1 1 1] 코멘트
  (set `self.skeleton first skill playing` true))

(fn `Active Page Three`
  (set `self.Playing_page_three_skill` true))

(fn `Active Page Two`
  (set `self.Playing_page_two_skill` true))

(fn `Attack`
  (returns (`Animation Duration` :type "Float (double-precision)"))
  (bind _returnvalue (`self.CheckHighestATPAginstPlayer`))
  (set `self.is_highest_atp_player` _returnvalue)
  (if (`self.IsNpcDead`)
    _
    (elif (and (`self.Playing_page_three_skill`) (`self.is_highest_atp_player`))
      (bind _returnvalue_2 (`AnimInstance.Montage_Play` (`SkeletalMeshComponent.GetAnimInstance` (`self.Mesh`)) "/Game/Assets/Staff_Skeleton_Animation/Skill4_Meteo.Skill4_Meteo" 1.0 "Duration" 0.0 true))
      (return _returnvalue_2)
      (elif (and (`self.Playing_page_two_skill`) (`self.is_highest_atp_player`))
        (bind _returnvalue_3 (`AnimInstance.Montage_Play` (`SkeletalMeshComponent.GetAnimInstance` (`self.Mesh`)) "/Game/Assets/Staff_Skeleton_Animation/SKill3_Spawn_Skeleton_Montage.SKill3_Spawn_Skeleton_Montage" (`self.Skill_Atk_Spd`) "Duration" 0.0 true))
        (return _returnvalue_3)
        (else
          (bind _animation_duration (`parent.Attack`))
          (return _animation_duration))))))

(fn `Enter Page Three`
  (`KismetSystemLibrary.K2_SetTimer` null "Active Page Three" 15.0 true))

(fn `Enter Page Two`
  (`KismetSystemLibrary.K2_SetTimer` null "Acitve Page Two" 10.0 true))

(fn `Spawn Big Fire Ball`
  (params (NewParam :type "Actor Object Reference"))
  (locals (`whats Target` :type "Actor Object Reference"))
  (bind (_returnvalue_x _returnvalue_y _returnvalue_z) (`KismetMathLibrary.BreakVector` (`SceneComponent.K2_GetComponentLocation` (`self.CapsuleComponent`))))
  (set `local.whats Target` NewParam)
  (`/Engine/EditorBlueprintResources/StandardMacros.IsValid` (`local.whats Target`)
    (:`Is Valid`
      (cast `/Game/TopDown/Blueprints/BP_Player` (`local.whats Target`))
      (`|SpawnActorFromClass` "/Game/NPC/EnemeyNPC/BP/Weapon_BP/BP_SkeletonBoss_BigFireball_Charge.BP_SkeletonBoss_BigFireball_Charge_C" (`KismetMathLibrary.MakeTransform` (`KismetMathLibrary.MakeVector` _returnvalue_x _returnvalue_y (+ _returnvalue_z 300.0))) "Undefined" "MultiplyWithRoot" null null (`self.Boss Skill 2 Dmg`) null))))

(fn `Spawn Fire Ball`
  (params (NewParam :type "Actor Object Reference"))
  (locals (`whats Target` :type "Actor Object Reference"))
  (bind _whats_target (`local.whats Target`))
  (bind _whats_target_2 (`local.whats Target`))
  (bind _returnvalue (`SceneComponent.K2_GetComponentLocation` (`self.SpawnLoaction`)))
  (bind _returnvalue_2 (`SceneComponent.K2_GetComponentLocation` (`self.SpawnLoaction`)))
  (bind _returnvalue_3 (`SceneComponent.K2_GetComponentLocation` (`self.SpawnLoaction`)))
  (set `local.whats Target` NewParam)
  (`GameplayStatics.PlaySoundAtLocation` "/Game/Assets/Sounds/NPC/Skeleton/Boss_Sk_Skill1_FireBall.Boss_Sk_Skill1_FireBall" (`self.K2_GetActorLocation`) (struct) 1.0 1.0 0.0 null null null null)
  (`/Engine/EditorBlueprintResources/StandardMacros.IsValid` _whats_target
    (:`Is Valid`
      (bind _asbp_player (cast `/Game/TopDown/Blueprints/BP_Player` _whats_target_2)
        (:`then`
          (bind _returnvalue_4 (`|SpawnActorFromClass` "/Game/NPC/EnemeyNPC/BP/Weapon_BP/BP_BossSkeleton_HomingMissile_Base.BP_BossSkeleton_HomingMissile_Base_C" (`KismetMathLibrary.MakeTransform` _returnvalue_2 (`KismetMathLibrary.FindLookAtRotation` _returnvalue_2 (`self.K2_GetActorLocation` _whats_target)) (0.25 0.25 0.25)) "Undefined" "MultiplyWithRoot" null null (`self.Boss Skill 1 Dmg`) null))
          (`/Game/NPC/EnemeyNPC/BP/Weapon_BP/BP_BossSkeleton_HomingMissile_Base.SetArrowTarget` _returnvalue_4 (`local.whats Target`))
          (`/Game/NPC/EnemeyNPC/BP/Weapon_BP/BP_BossSkeleton_HomingMissile_Base.SetHomingTarget` _returnvalue_4 (`Character.CapsuleComponent` _asbp_player)))
        (:`CastFailed`
          (bind _asbp_base_building (cast `/Game/Building/BP_BaseBuilding` _whats_target_2)
            (:`then`
              (bind _returnvalue_5 (`|SpawnActorFromClass` "/Game/NPC/EnemeyNPC/BP/Weapon_BP/BP_BossSkeleton_HomingMissile_Base.BP_BossSkeleton_HomingMissile_Base_C" (`KismetMathLibrary.MakeTransform` _returnvalue_3 (`KismetMathLibrary.FindLookAtRotation` _returnvalue_3 (`self.K2_GetActorLocation` _whats_target)) (0.25 0.25 0.25)) "Undefined" "MultiplyWithRoot" null null (`self.Boss Skill 1 Dmg`) null))
              (`/Game/NPC/EnemeyNPC/BP/Weapon_BP/BP_BossSkeleton_HomingMissile_Base.SetArrowTarget` _returnvalue_5 (`local.whats Target`))
              (`/Game/NPC/EnemeyNPC/BP/Weapon_BP/BP_BossSkeleton_HomingMissile_Base.SetHomingTarget` _returnvalue_5 (`/Game/Building/BP_BaseBuilding.HitCollision` _asbp_base_building)))
            (:`CastFailed`
              (bind _asbp_my_friendly_base (cast `/Game/NPC/FriendlyNPC/BP/BP_MyFriendlyBase` _whats_target_2))
              (bind _returnvalue_6 (`|SpawnActorFromClass` "/Game/NPC/EnemeyNPC/BP/Weapon_BP/BP_BossSkeleton_HomingMissile_Base.BP_BossSkeleton_HomingMissile_Base_C" (`KismetMathLibrary.MakeTransform` _returnvalue (`KismetMathLibrary.FindLookAtRotation` _returnvalue (`self.K2_GetActorLocation` _whats_target)) (0.25 0.25 0.25)) "Undefined" "MultiplyWithRoot" null null (`self.Boss Skill 1 Dmg`) null))
              (`/Game/NPC/EnemeyNPC/BP/Weapon_BP/BP_BossSkeleton_HomingMissile_Base.SetArrowTarget` _returnvalue_6 (`local.whats Target`))
              (`/Game/NPC/EnemeyNPC/BP/Weapon_BP/BP_BossSkeleton_HomingMissile_Base.SetHomingTarget` _returnvalue_6 (`FriendlyBase.CapsuleComponent` _asbp_my_friendly_base)))))))))

(fn `Spawn Meteo`
  (bind (_returnvalue_x _returnvalue_y _returnvalue_z) (`KismetMathLibrary.BreakVector` (`self.K2_GetActorLocation`)))
  ;[1 1 1] 스폰
  (bind _output_get (set `self.EnemySpawnLocation` (`KismetMathLibrary.MakeVector` (+ _returnvalue_x (`KismetMathLibrary.RandomFloatInRange` -400.0 400.0)) (+ _returnvalue_y (`KismetMathLibrary.RandomFloatInRange` -400.0 400.0)) _returnvalue_z)))
  (`|SpawnActorFromClass` "/Game/NPC/EnemeyNPC/BP/Effect/BP_SkeletonBoss_Meteo_Indicator.BP_SkeletonBoss_Meteo_Indicator_C" (`KismetMathLibrary.MakeTransform` _output_get) "Undefined" "MultiplyWithRoot" null (`self.Boss Skill 4 Dmg`) null))

(fn `SPawn SK`
  (bind (_returnvalue_x _returnvalue_y _returnvalue_z) (`KismetMathLibrary.BreakVector` (`self.K2_GetActorLocation`)))
  ;[1 1 1] 스폰
  (bind _output_get (set `self.EnemySpawnLocation` (`KismetMathLibrary.MakeVector` (+ _returnvalue_x (`KismetMathLibrary.RandomFloatInRange` -400.0 400.0)) (+ _returnvalue_y (`KismetMathLibrary.RandomFloatInRange` -400.0 400.0)) _returnvalue_z)))
  (bind _returnvalue (- (.z _output_get) 100.0))
  (`|SpawnActorFromClass` "/Game/NPC/EnemeyNPC/BP/Effect/BP_Boss_Skeleton_Spawn_Effect.BP_Boss_Skeleton_Spawn_Effect_C" (`KismetMathLibrary.MakeTransform` (`KismetMathLibrary.MakeVector` (.x _output_get) (.y _output_get) _returnvalue)) "Undefined" "MultiplyWithRoot" null null)
  (`|SpawnActorFromClass` "/Game/NPC/EnemeyNPC/BP/Effect/BP_Boss_Skeleton_Spawn_Effect.BP_Boss_Skeleton_Spawn_Effect_C" (`KismetMathLibrary.MakeTransform` (+ (`KismetMathLibrary.MakeVector` (.x _output_get) (.y _output_get) _returnvalue) (70.0 70.0 0.0))) "Undefined" "MultiplyWithRoot" null null)
  (`|SpawnActorFromClass` "/Game/NPC/EnemeyNPC/BP/hunt/BP_Skeleton_Sword.BP_Skeleton_Sword_C" (`KismetMathLibrary.MakeTransform` (`KismetMathLibrary.MakeVector` (.x _output_get) (.y _output_get) (.z _output_get))) "Undefined" "MultiplyWithRoot" null true "6021" true null)
  (`|SpawnActorFromClass` "/Game/NPC/EnemeyNPC/BP/hunt/BP_Skeleton_Archer.BP_Skeleton_Archer_C" (`KismetMathLibrary.MakeTransform` (+ (`KismetMathLibrary.MakeVector` (.x _output_get) (.y _output_get) (.z _output_get)) (70.0 70.0 0.0))) "Undefined" "MultiplyWithRoot" null true "6022" true null))

(fn `UserConstructionScript`
  (`parent.UserConstructionScript`))