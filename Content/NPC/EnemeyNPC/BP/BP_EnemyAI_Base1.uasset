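; Base enemy NPC Blueprint that handles death and loot drops, with an Attack function that only returns zero.
; NpcDead disables collision, detaches the controller, drops loot, plays the death effect and montage, then calls DestroyActor after the montage's length.
; DropItem runs only when IsAggression is false, spawning a random number of BP_LootItemBase items evenly spaced around a random starting angle, passing each the NPC's tier.
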(event `NpcDead`
  ;[1 1 1] npc 죽음
  (`PrimitiveComponent.SetCollisionEnabled` (`self.RecognitionBoundary`) "NoCollision")
  (`PrimitiveComponent.SetCollisionEnabled` (`self.CapsuleComponent`) "NoCollision")
  (`PrimitiveComponent.SetCollisionEnabled` (`self.PlayerAimCollision`) "NoCollision")
  (`self.DetachFromControllerPendingDestroy`)
  ;;[1 1 1] 이 부분
  (`self.DropItem`)
  (`/Game/TopDown/Blueprints/Components/AC_HitEffectComponent.PlayDieEffect` (`self.AC_HitEffectComponent`))
  (bind _returnvalue (`self.PlayAnimMontage` (`self.DieMontage`)))
  (`KismetSystemLibrary.Delay` _returnvalue)
  (`self.Destroy Actor?`))

(fn `Attack`
  (returns (`Animation Duration` :type "Float (double-precision)"))
  (return 0.0))

(fn `Destroy Actor?`)

(fn `DropItem`
  (locals (Angle :type "Float (double-precision)" :default 0.0) (DesiredAngle :type "Float (double-precision)") (DropCount :type Integer))
  ;[0.05098 0.05098 0.05098] 자원 드롭 로직
  (if (not (`self.isAggression?`))
    (set `local.DropCount` (`KismetMathLibrary.RandomIntegerInRange` (`self.ItemMinDropCount`) (`self.ItemMaxDromCount`)))
    (set `local.Angle` (`KismetMathLibrary.RandomFloatInRange` 0.0 360.0))
    (for _index (range 1 (+ (`local.DropCount`) 1))
      (bind _returnvalue (`|SpawnActorFromClass` (`self.ItemType`) (`KismetMathLibrary.MakeTransform` (`self.K2_GetActorLocation`)) "Undefined" "MultiplyWithRoot" null null))
      (bind _asbp_loot_item_base (cast `/Game/TopDown/Blueprints/Items/Item/BP_LootItemBase` _returnvalue))
      (bind _output_get (set `local.DesiredAngle` (mod (+ (`local.Angle`) (* (/ 360 (`local.DropCount`)) _index)) 360.0)))
      (`/Game/TopDown/Blueprints/Items/Item/BP_LootItemBase.DropItem` _asbp_loot_item_base (`self.Enemy Npc Tier`) _output_get (`self.ItemDropDistance`)))))

(fn `UserConstructionScript`)