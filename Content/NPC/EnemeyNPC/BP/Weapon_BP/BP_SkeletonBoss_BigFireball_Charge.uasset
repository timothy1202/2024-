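; Charge stage of the skeleton boss's big fireball attack, which grows in place before handing off to the fired projectile.
; On BeginPlay it plays a skill sound and runs a timeline that scales the collision sphere.
; When the timeline finishes, it spawns BP_SkeletonBoss_BigFireball_Shoot rotated toward player 0, passes Damage along, and destroys itself.
; The Explode function is an empty stub.
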(event `self.ReceiveBeginPlay`
  (bind _returnvalue (`self.K2_GetActorLocation`))
  (`GameplayStatics.PlaySoundAtLocation` "/Game/Assets/Sounds/NPC/Skeleton/Boss_Sk_Skill2_1_WonKi-ok.Boss_Sk_Skill2_1_WonKi-ok" (`self.K2_GetActorLocation`) (struct) 1.0 1.0 0.0 null null null null)
  (bind (_direction `_새_트랙_0`) (`Timeline|불 커짐`)
    (:`Update`
      (`SceneComponent.SetWorldScale3D` (`self.SphereCollision`) (`KismetMathLibrary.Conv_DoubleToVector` `_새_트랙_0`)))
    (:`Finished`
      (`|SpawnActorFromClass` "/Game/NPC/EnemeyNPC/BP/Weapon_BP/BP_SkeletonBoss_BigFireball_Shoot.BP_SkeletonBoss_BigFireball_Shoot_C" (`KismetMathLibrary.MakeTransform` _returnvalue (`KismetMathLibrary.FindLookAtRotation` _returnvalue (`self.K2_GetActorLocation` (`GameplayStatics.GetPlayerCharacter` 0)))) "Undefined" "MultiplyWithRoot" null null (`self.Damage`) null)
      (`self.K2_DestroyActor`))))

(fn `Explode`)

(fn `UserConstructionScript`
  (`parent.UserConstructionScript`))