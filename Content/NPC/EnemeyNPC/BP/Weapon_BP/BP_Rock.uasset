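; BP_Rock is the rock projectile of the rock-throwing orc, dealing direct-hit and splash damage.
; RockCollision damages a player or building on overlap, briefly enables the ExplosionCollision sphere, then destroys the rock.
; ExplosionCollision applies ranged damage to overlapping players, buildings and friendly bases.
; Splash radius and both damage values come from GetActorOfClass on BP_Orc_ThrowRock, so from whichever orc it finds, not necessarily the thrower.
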(event `self.ReceiveBeginPlay`
  ;[1 1 1] 탄막 범위 설정
  (bind _returnvalue (`GameplayStatics.GetActorOfClass` "/Game/NPC/EnemeyNPC/BP/hunt/BP_Orc_ThrowRock.BP_Orc_ThrowRock_C"))
  (`SphereComponent.SetSphereRadius` (`self.ExplosionCollision`) (`EnemyBase.PT_AtkRng` _returnvalue) true))

(event `self.RockCollision.OnComponentBeginOverlap`
  (params (OverlappedComponent :type "PrimitiveComponent Object Reference") (OtherActor :type "Actor Object Reference") (OtherComp :type "PrimitiveComponent Object Reference") (OtherBodyIndex :type Integer) (bFromSweep :type Boolean) (SweepResult :type "HitResult Structure (by ref)"))
  ;[1 1 1] 돌이 플레이어 닿았는지
  (bind _asbp_player (cast `/Game/TopDown/Blueprints/BP_Player` OtherActor)
    (:`then`
      (bind _returnvalue (`GameplayStatics.GetActorOfClass` "/Game/NPC/EnemeyNPC/BP/hunt/BP_Orc_ThrowRock.BP_Orc_ThrowRock_C"))
      (`/Game/TopDown/Blueprints/BP_Player.DamagePlayer` _asbp_player (`EnemyBase.PT_AtkDmg` _returnvalue)))
    (:`CastFailed`
      (bind _asbp_base_building (cast `/Game/Building/BP_BaseBuilding` OtherActor))
      (bind _returnvalue_2 (`GameplayStatics.GetActorOfClass` "/Game/NPC/EnemeyNPC/BP/hunt/BP_Orc_ThrowRock.BP_Orc_ThrowRock_C"))
      (`/Game/Building/BP_BaseBuilding.Take Damage` _asbp_base_building false (`EnemyBase.PT_AtkDmg` _returnvalue_2))))
  (`PrimitiveComponent.SetCollisionEnabled` (`self.ExplosionCollision`) "QueryAndPhysics")
  (`/Engine/EditorBlueprintResources/StandardMacros.IsValid` self
    (:`Is Valid`
      (`PrimitiveComponent.SetCollisionEnabled` (`self.ExplosionCollision`) "NoCollision")
      (`self.K2_DestroyActor`))))

(event `self.ExplosionCollision.OnComponentBeginOverlap`
  (params (OverlappedComponent :type "PrimitiveComponent Object Reference") (OtherActor :type "Actor Object Reference") (OtherComp :type "PrimitiveComponent Object Reference") (OtherBodyIndex :type Integer) (bFromSweep :type Boolean) (SweepResult :type "HitResult Structure (by ref)"))
  ;[1 1 1] 탄만 범위 데미지
  (`|ExecutionSequence`
    (:`then_0`
      (bind _asbp_player (cast `/Game/TopDown/Blueprints/BP_Player` OtherActor))
      (bind _returnvalue (`GameplayStatics.GetActorOfClass` "/Game/NPC/EnemeyNPC/BP/hunt/BP_Orc_ThrowRock.BP_Orc_ThrowRock_C"))
      (`/Game/TopDown/Blueprints/BP_Player.DamagePlayer` _asbp_player (`EnemyBase.PT_AtkRngDmg` _returnvalue)))
    (:`then_1`
      (bind _asbp_base_building (cast `/Game/Building/BP_BaseBuilding` OtherActor))
      (bind _returnvalue_2 (`GameplayStatics.GetActorOfClass` "/Game/NPC/EnemeyNPC/BP/hunt/BP_Orc_ThrowRock.BP_Orc_ThrowRock_C"))
      (`/Game/Building/BP_BaseBuilding.Take Damage` _asbp_base_building false (`EnemyBase.PT_AtkRngDmg` _returnvalue_2)))
    (:`then_2`
      (bind _asbp_my_friendly_base (cast `/Game/NPC/FriendlyNPC/BP/BP_MyFriendlyBase` OtherActor))
      (bind _returnvalue_3 (`GameplayStatics.GetActorOfClass` "/Game/NPC/EnemeyNPC/BP/hunt/BP_Orc_ThrowRock.BP_Orc_ThrowRock_C"))
      (`/Game/NPC/FriendlyNPC/BP/BP_MyFriendlyBase.Take Damage` _asbp_my_friendly_base false (`EnemyBase.PT_AtkRngDmg` _returnvalue_3)))))

(fn `UserConstructionScript`)