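; Fireball projectile for the skeleton boss's big fireball skill, playing an attenuated sound at its location on spawn.
; Sphere overlaps apply Damage through a cast chain to the player, friendly base units or buildings, without exploding.
; Any other overlap spawns the explosion actor, stops a sound component and prints a debug string.
; A Landscape tag check is left unconnected, and the actor never destroys itself here.
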(event `self.ReceiveBeginPlay`
  (`GameplayStatics.PlaySoundAtLocation` "/Game/Assets/Sounds/NPC/Skeleton/Boss_Sk_Skill2_2_WonKi-ok.Boss_Sk_Skill2_2_WonKi-ok" (`self.K2_GetActorLocation`) (struct) 1.5 1.0 0.0 "/Game/NPC/EnemeyNPC/BP/EnemyNPC_SoundAttenuation.EnemyNPC_SoundAttenuation" null null null))

(event `self.SphereCollision.OnComponentBeginOverlap`
  (params (OverlappedComponent :type "PrimitiveComponent Object Reference") (OtherActor :type "Actor Object Reference") (OtherComp :type "PrimitiveComponent Object Reference") (OtherBodyIndex :type Integer) (bFromSweep :type Boolean) (SweepResult :type "HitResult Structure (by ref)"))
  (bind _asbp_player (cast `/Game/TopDown/Blueprints/BP_Player` OtherActor)
    (:`then`
      (`/Game/TopDown/Blueprints/BP_Player.DamagePlayer` _asbp_player (`self.Damage`)))
    (:`CastFailed`
      (bind _asbp_my_friendly_base (cast `/Game/NPC/FriendlyNPC/BP/BP_MyFriendlyBase` OtherActor)
        (:`then`
          (`/Game/NPC/FriendlyNPC/BP/BP_MyFriendlyBase.Take Damage` _asbp_my_friendly_base false (`self.Damage`)))
        (:`CastFailed`
          (bind _asbp_base_building (cast `/Game/Building/BP_BaseBuilding` OtherActor)
            (:`then`
              (`/Game/Building/BP_BaseBuilding.Take Damage` _asbp_base_building false (`self.Damage`)))
            (:`CastFailed`
              (`self.Explode`)
              (`AudioComponent.Stop` (`self.Boss_Sk_Skill2_2_WonKi-ok`))
              (`KismetSystemLibrary.PrintString` "Hello"))))))))

(fn `Explode`
  (`|SpawnActorFromClass` "/Game/NPC/EnemeyNPC/BP/Effect/BP_BigFireBall_Explode.BP_BigFireBall_Explode_C" (`KismetMathLibrary.MakeTransform` (`self.K2_GetActorLocation`)) "Undefined" "MultiplyWithRoot" null null))

(fn `UserConstructionScript`
  (`parent.UserConstructionScript`))