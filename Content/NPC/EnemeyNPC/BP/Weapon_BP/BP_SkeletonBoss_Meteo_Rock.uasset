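; BP_SkeletonBoss_Meteo_Rock is a damaging rock actor, named for the skeleton boss's meteor attack.
; It turns on query and physics collision on its Sphere after a short delay from BeginPlay.
; Sphere overlaps run a cast chain that applies Damage to the player, buildings or friendly bases, flagging hits on the latter two as non-player.
; The graph contains no movement or destruction logic.
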(event `self.ReceiveBeginPlay`
  (`KismetSystemLibrary.Delay` 0.5)
  (`PrimitiveComponent.SetCollisionEnabled` (`self.Sphere`) "QueryAndPhysics"))

(event `self.Sphere.OnComponentBeginOverlap`
  (params (OverlappedComponent :type "PrimitiveComponent Object Reference") (OtherActor :type "Actor Object Reference") (OtherComp :type "PrimitiveComponent Object Reference") (OtherBodyIndex :type Integer) (bFromSweep :type Boolean) (SweepResult :type "HitResult Structure (by ref)"))
  (bind _damage (`self.damage`))
  (bind _asbp_player (cast `/Game/TopDown/Blueprints/BP_Player` OtherActor)
    (:`then`
      (`/Game/TopDown/Blueprints/BP_Player.DamagePlayer` _asbp_player _damage))
    (:`CastFailed`
      (bind _asbp_base_building (cast `/Game/Building/BP_BaseBuilding` OtherActor)
        (:`then`
          (`/Game/Building/BP_BaseBuilding.Take Damage` _asbp_base_building false _damage))
        (:`CastFailed`
          (bind _asbp_my_friendly_base (cast `/Game/NPC/FriendlyNPC/BP/BP_MyFriendlyBase` OtherActor))
          (`/Game/NPC/FriendlyNPC/BP/BP_MyFriendlyBase.Take Damage` _asbp_my_friendly_base false (`self.damage`)))))))

(fn `UserConstructionScript`)