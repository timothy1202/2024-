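; BP_Arrow is an enemy arrow projectile that damages players and buildings, using the skeleton archer's attack damage.
; ShootArrow starts the trail, sets gravity scale from Speed, and launches along a suggested arc to the target's location at firing.
; Collision overlap with BP_Player or BP_BaseBuilding applies PTAtkDmg from whichever BP_Skeleton_Archer GetActorOfClass finds, not a tracked shooter, then destroys the arrow.
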(event `ShootArrow`
  (params (Target :type "Actor Object Reference"))
  (bind _projectilemovement (`self.ProjectileMovement`))
  ;[1 1 1] 포물선
  (`ActorComponent.Activate` (`self.FX_Weapon_trail`) false)
  (set `ProjectileMovementComponent.ProjectileGravityScale` (`self.Speed`) _projectilemovement)
  (bind _outlaunchvelocity (`GameplayStatics.SuggestProjectileVelocity_CustomArc` (`self.K2_GetActorLocation`) (`self.K2_GetActorLocation` Target) (`MovementComponent.GetGravityZ` _projectilemovement)))
  (set `MovementComponent.Velocity` _outlaunchvelocity (`self.ProjectileMovement`)))

(event `self.AttackCollision.OnComponentBeginOverlap`
  (params (OverlappedComponent :type "PrimitiveComponent Object Reference") (OtherActor :type "Actor Object Reference") (OtherComp :type "PrimitiveComponent Object Reference") (OtherBodyIndex :type Integer) (bFromSweep :type Boolean) (SweepResult :type "HitResult Structure (by ref)"))
  ;[1 1 1] 총알 플레이어 닿았는지
  (bind _asbp_player (cast `/Game/TopDown/Blueprints/BP_Player` OtherActor)
    (:`then`
      (bind _returnvalue (`GameplayStatics.GetActorOfClass` "/Game/NPC/EnemeyNPC/BP/hunt/BP_Skeleton_Archer.BP_Skeleton_Archer_C"))
      (`/Game/TopDown/Blueprints/BP_Player.DamagePlayer` _asbp_player (`EnemyBase.PT_AtkDmg` _returnvalue)))
    (:`CastFailed`
      (bind _asbp_base_building (cast `/Game/Building/BP_BaseBuilding` OtherActor))
      (bind _returnvalue_2 (`GameplayStatics.GetActorOfClass` "/Game/NPC/EnemeyNPC/BP/hunt/BP_Skeleton_Archer.BP_Skeleton_Archer_C"))
      (`/Game/Building/BP_BaseBuilding.Take Damage` _asbp_base_building false (`EnemyBase.PT_AtkDmg` _returnvalue_2))))
  (`/Engine/EditorBlueprintResources/StandardMacros.IsValid` self
    (:`Is Valid`
      (`ActorComponent.Deactivate` (`self.FX_Weapon_trail`))
      (`self.K2_DestroyActor`))))

(fn `UserConstructionScript`)