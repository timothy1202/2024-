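; Skeleton archer enemy NPC that extends a parent NPC class, loading data row 6002 on BeginPlay to set its walk speed.
; Attack plays a bow montage unless dead, while ShootArrow spawns BP_Arrow at the Arrow1 component, aimed at the blackboard's AttackPlayer actor.
; Tick, commented as death check and revival, spawns a new archer with its behavior tree in place and clears IsNPCDead, with no condition shown.
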(event `self.ReceiveBeginPlay`
  ;[1 1 1] 코멘트
  (`/Game/NPC/EnemeyNPC/AI/Interface/BPI_AI_BehaviorTrees.GetDataTable` "6002")
  (`parent.ReceiveBeginPlay`))

(event `ShootArrow`
  (bind (_returnvalue_location _returnvalue_rotation) (`KismetMathLibrary.BreakTransform` (`SceneComponent.K2_GetComponentToWorld` (`self.Arrow1`))))
  ;[1 1 1] 활 공격
  (bind _returnvalue (`|SpawnActorFromClass` "/Game/NPC/EnemeyNPC/BP/Weapon_BP/BP_Arrow.BP_Arrow_C" (`KismetMathLibrary.MakeTransform` _returnvalue_location _returnvalue_rotation) "AlwaysSpawn" "MultiplyWithRoot" null null))
  (bind `_as액터` (cast `Actor` (`BlackboardComponent.GetValueAsObject` (`AIBlueprintHelperLibrary.GetBlackboard` (`AIBlueprintHelperLibrary.GetAIController` self)) (`self.Attack Player`))))
  (`/Game/NPC/EnemeyNPC/BP/Weapon_BP/BP_Arrow.ShootArrow` _returnvalue `_as액터`))

(event `self.ReceiveTick`
  (params (DeltaSeconds :type "Float (single-precision)"))
  ;[1 1 1] 플레이어 사망 체크 & 부활
  (`parent.ReceiveTick` 0.0)
  (`AIBlueprintHelperLibrary.SpawnAIFromClass` "BP_Skeleton_Archer_C" "/Game/NPC/EnemeyNPC/AI/BT/BT_Skeleton_Archer.BT_Skeleton_Archer" (`self.K2_GetActorLocation`) (`self.K2_GetActorRotation`) false null)
  (set `self.IsNPCDead?` false))

(event `/Game/NPC/EnemeyNPC/AI/Interface/BPI_AI_BehaviorTrees.GetDataTable`
  (params (RowName :type Name))
  ;[1 1 1] 데이터 테이블 변수화
  (`parent.GetDataTable` RowName)
  (`self.DefaultSetting_SkArcher`))

(event `DefaultSetting_SkArcher`
  ;[1 1 1] 디폴트 세팅 설정
  (set `CharacterMovementComponent.MaxWalkSpeed` (`self.Enemy Npc Walk Speed`) (`self.CharacterMovement`)))

(fn `Attack`
  (returns (`Animation Duration` :type "Float (double-precision)"))
  (if (not (`self.IsNPCDead?`))
    (bind _returnvalue (`self.PlayAnimMontage` "/Game/Assets/SkeletonEnemy/Animations/Anim_AttackBow_Montage.Anim_AttackBow_Montage"))
    (return _returnvalue)))

(fn `UserConstructionScript`
  (`parent.UserConstructionScript`))