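; Base enemy NPC that loads stats from DT_EnemyAI, plays attack montages and tracks damage with a proximity health bar.
; Non-aggressive enemies target the player via RecognitionBoundary and blackboard; aggressive ones track the highest-ATP building or player, overridden by forward-trace obstacles.
; Wizard tower lightning chains to two nearby enemies with decreasing damage.
; Init, death, speed-change and controller-registration events are empty here, their logic left unwired.
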(event `self.ReceiveBeginPlay`
  (`self.GetDataTables`)
  (`self.Init Enemy Controller`)
  ;[0.05098 0 0.007123 1 14] 추후 Object Pooling 적용 시 호출X
  (`self.Init`))

(event `Init`
  ;[0.05098 0.05098 0.05098] 초기화 이벤트
)

(event `self.RecognitionBoundary.OnComponentBeginOverlap`
  (params (OverlappedComponent :type "PrimitiveComponent Object Reference") (OtherActor :type "Actor Object Reference") (OtherComp :type "PrimitiveComponent Object Reference") (OtherBodyIndex :type Integer) (bFromSweep :type Boolean) (SweepResult :type "HitResult Structure (by ref)"))
  ;[0.05098 0.05098 0.05098] 적 인지
  (if (`self.bAggressive`)
    _
    (elif (`ActorComponent.ComponentHasTag` OtherComp "Player")
      (`self.SetAttackTarget` (`GameplayStatics.GetPlayerCharacter` 0)))))

(event `RenewHighestATPTarget`
  ;[0.05098 0.05098 0.05098] 갈 수 있는 경로인지 계산하면서 ATP제일 높은 타겟 설정
  (bind _target (`self.Calculate Highest ATP`))
  (`self.SetAttackTarget` _target))

(event `self.RecognitionBoundary.OnComponentEndOverlap`
  (params (OverlappedComponent :type "PrimitiveComponent Object Reference") (OtherActor :type "Actor Object Reference") (OtherComp :type "PrimitiveComponent Object Reference") (OtherBodyIndex :type Integer))
  ;[0.05098 0.05098 0.05098] 적 인지
  (if (`self.bAggressive`)
    _
    (elif (`self.neverStopChasing`)
      _
      (elif (`ActorComponent.ComponentHasTag` OtherComp "Player")
        (`self.SetAttackTarget` (`GameplayStatics.GetPlayerCharacter` 0))))))

(event `/Game/NPC/EnemeyNPC/AI/Interface/BPI_AI_BehaviorTrees.SetSpeed`
  (params (IsChasing :type Boolean))
  ;[0.05098 0.05098 0.05098 1 15] 속도 변경 인터페이스 이벤트 - BT에서 실행 (BT에서 Casting안하기 위함)
)

(event `self.ReceiveTick`
  (params (DeltaSeconds :type "Float (single-precision)"))
  (bind (_highest_building _atp) (`self.Get Player ATP`))
  (bind (_highest_building_2 _atp_2) (`self.Get Highest Building ATP`))
  ;[1 1 1] 움직임 멈춤
  (if (not (`self.IsNPCDead?`))
    (if (`self.bAggressive`)
      (`self.DetectOtherObject`)
      (if (not (`self.DetectOtherObjects?`))
        (if (> _atp_2 _atp)
          (set `self.Highest ATP Building` _highest_building_2)
          (else
            (set `self.Highest ATP Building` _highest_building)))
        (`self.Check Distance` :!label _label))
      (else
        (goto _label)))))

(event `/Game/TopDown/Blueprints/Interface/BPI_Hitable.Take Damage`
  (params (IsPlayer :type Boolean) (damageValue :type "Float (double-precision)"))
  ;[0.05098 0.05098 0.05098] 피격
  (`/Game/TopDown/Blueprints/Components/AC_HitEffectComponent.HitEffect` (`self.AC_HitEffectComponent`) "NewEnumerator0" damageValue)
  (`self.Update Damaged Health Bar` damageValue)
  (if (not (not IsPlayer))
    (`self.SetAttackTarget` (`GameplayStatics.GetPlayerCharacter` 0))
    (set `self.neverStopChasing` true))
  (bind _output_get (set `self.IsNPCDead?` (<= (`self.curHealth`) 0.0)))
  (if _output_get
    (`self.NpcDead`)))

(event `NpcDead`
  ;[0.05098 0.05098 0.05098] npc 죽음
)

(event `DetectOtherObject`
  (bind _objectdetectarrow (`self.ObjectDetectArrow`))
  (bind _returnvalue (`SceneComponent.K2_GetComponentLocation` _objectdetectarrow))
  ;[1 1 1] 라인트레이스로 ATP높은거로 갈때 다른게 앞에 있는지 확인
  (bind (_outhit _returnvalue_2) (`KismetSystemLibrary.LineTraceSingleForObjects` :`Start` _returnvalue :`End` (+ _returnvalue (* (`SceneComponent.GetForwardVector` _objectdetectarrow) 80.0)) :`ObjectTypes` (`|MakeArray` "ObjectTypeQuery3" "ObjectTypeQuery10" :!type "EObjectTypeQuery Enum") :`DrawTime` 0.0))
  (if _returnvalue_2
    (bind (_bblockinghit _binitialoverlap _time _distance _location _impactpoint _normal _impactnormal _physmat _hitactor) (`GameplayStatics.BreakHitResult` _outhit))
    (if (and (!= _hitactor (`self.Highest ATP Building`)) (`self.ActorHasTag` _hitactor "EnemyDetect"))
      (set `self.DetectOtherObjects?` true)
      (set `self.Highest ATP Building` _hitactor))
    (else
      (set `self.DetectOtherObjects?` false))))

(event `NPC Thunder Attacked?`
  ;[1 1 1] 타워의 번개 공격
  (bind _output_get (set `self.FirstTunderTarget` (`self.Find First Tunder Target`)))
  (`/Engine/EditorBlueprintResources/StandardMacros.IsValid` _output_get
    (:`Is Valid`
      (`self.Spawn First Thunder` (`self.FirstTunderTarget`)))))

(event `second Thunder Attacked`
  ;[1 1 1] 두번째 번개 공격
  (bind _output_get (set `self.SecondTunderTarget` (`self.Find Second Tunder Target` (`self.FirstTunderTarget`))))
  (`/Engine/EditorBlueprintResources/StandardMacros.IsValid` _output_get
    (:`Is Valid`
      (`KismetSystemLibrary.DrawDebugSphere` (`self.K2_GetActorLocation` _output_get) 100.0 12 (struct :`R` 0.092374 :`G` 1.0 :`B` 0.120601 :`A` 1.0))
      (`self.Spawn Second Thunder` (`self.SecondTunderTarget`)))))

(event `/Game/TopDown/Blueprints/Interface/BPI_Spectator.OnSpectator`
  (params (bEnable :type Boolean))
  (bind _output_get (set `self.bSpectatorOn` bEnable))
  (`/Game/TopDown/Blueprints/Components/AC_HitEffectComponent.EnableSpectatorMode` (`self.AC_HitEffectComponent`) _output_get))

(fn `Attack`
  (returns (`Animation Duration` :type "Float (double-precision)"))
  (if (not (`self.IsNPCDead?`))
    (bind _attackmontage (`self.AttackMontage`)
      (:`then`
        (bind _returnvalue (`AnimInstance.Montage_Play` (`SkeletalMeshComponent.GetAnimInstance` (`self.Mesh`)) _attackmontage (`self.Enemy Npc Atk Spd`) "Duration" 0.0 true))
        (return _returnvalue))
      (:`else`
        (`KismetSystemLibrary.PrintString` (`KismetStringLibrary.Concat_StrStr` (`KismetSystemLibrary.GetObjectName` self) ": 공격 몽타주를 할당해주세요!") true true (struct :`R` 1.0 :`A` 1.0))))))

(fn `Calculate Highest ATP`
  (returns (Target :type "Actor Object Reference"))
  (locals (HighestATPTargetTemp :type "Actor Object Reference") (HighestATPValue :type Integer))
  (for _array_element (`self.ATPTargets`)
    (bind _returnvalue (message `ATPInterface.GetATP` _array_element))
    (if (and (> _returnvalue (`local.HighestATPValue`)) (`self.DetectObject` _array_element))
      (set `local.HighestATPValue` _returnvalue)
      (set `local.HighestATPTargetTemp` _array_element)))
  (return (`local.HighestATPTargetTemp`)))

(fn `Check Distance`
  (bind _healthwidget (`self.HealthWidget`))
  (if (and (< (`self.GetHorizontalDistanceTo` self (`GameplayStatics.GetPlayerCharacter` 0)) (`self.Show Health Dis`)) (not (`self.bSpectatorOn`)))
    (`SceneComponent.SetVisibility` _healthwidget true false)
    (else
      (`SceneComponent.SetVisibility` _healthwidget false false))))

(fn `Destroy Actor?`
  (`self.K2_DestroyActor`))

(fn `DetectObject`
  (params (Actor :type "Actor Object Reference"))
  (returns (bDetect :type Boolean))
  (locals (ObjectToDetect :type "Array of EObjectTypeQuery Enum") (Target :type "Actor Object Reference")))

(fn `DropItem`
  (locals (Angle :type "Float (double-precision)") (DesiredAngle :type "Float (double-precision)") (DropCount :type Integer))
  ;[0.05098 0.05098 0.05098] 자원 드롭 로직
  (if (not (`self.bAggressive`))
    (set `local.DropCount` (`KismetMathLibrary.RandomIntegerInRange` (`self.ItemMinDropCount`) (`self.ItemMaxDromCount`)))
    (set `local.Angle` (`KismetMathLibrary.RandomFloatInRange` 0.0 360.0))
    (for _index (range 1 (+ (`local.DropCount`) 1))
      (bind _returnvalue (`|SpawnActorFromClass` (`self.ItemType`) (`KismetMathLibrary.MakeTransform` (`self.K2_GetActorLocation`)) "Undefined" "MultiplyWithRoot" null null))
      (cast `/Game/TopDown/Blueprints/Items/Item/BP_LootItemBase` _returnvalue)
      (set `local.DesiredAngle` (mod (+ (`local.Angle`) (* (/ 360 (`local.DropCount`)) _index)) 360.0)))))

(fn `Find First Tunder Target`
  (returns (`Thunder Target` :type "Actor Object Reference"))
  (locals (`Local Dis` :type "Array of Float (double-precision)"))
  (bind _overlappingactors (`PrimitiveComponent.GetOverlappingActors` (`self.RecognitionBoundary`) "/Game/NPC/EnemeyNPC/BP/BP_EnemyAI_Base.BP_EnemyAI_Base_C"))
  (switch `int` (`KismetArrayLibrary.Array_Length` _overlappingactors)
    (:`Default`
      (for _array_element _overlappingactors
        (if (!= _array_element self)
          (`KismetArrayLibrary.Array_Add` (`local.Local Dis`) (`KismetMathLibrary.Vector_Distance` (`self.K2_GetActorLocation` _array_element) (`self.K2_GetActorLocation`)))
          (else
            (`KismetArrayLibrary.Array_Add` (`local.Local Dis`) 1000000.0))))
      (return (`|GetArrayItem` _overlappingactors (`KismetMathLibrary.MinOfFloatArray` (`local.Local Dis`)))))
    (:`0`
      (return null))
    (:`1`
      (return null))))

(fn `Find Second Tunder Target`
  (params (`First Target` :type "Actor Object Reference"))
  (returns (`Second Target` :type "Actor Object Reference"))
  (locals (`Local Dis` :type "Array of Float (double-precision)") (`First Tunder` :type "Actor Object Reference"))
  (bind _overlappingactors (`PrimitiveComponent.GetOverlappingActors` (`self.RecognitionBoundary`) "/Game/NPC/EnemeyNPC/BP/BP_EnemyAI_Base.BP_EnemyAI_Base_C"))
  (bind _output (`|GetArrayItem` _overlappingactors 1))
  (set `local.First Tunder` `First Target`)
  (switch `int` (`KismetArrayLibrary.Array_Length` _overlappingactors)
    (:`Default`
      (for _array_element _overlappingactors
        (if (or (== _array_element self) (== _array_element (`local.First Tunder`)))
          (`KismetArrayLibrary.Array_Add` (`local.Local Dis`) 1000000.0)
          (else
            (`KismetArrayLibrary.Array_Add` (`local.Local Dis`) (`KismetMathLibrary.Vector_Distance` (`self.K2_GetActorLocation` _array_element) (`self.K2_GetActorLocation`))))))
      (return (`|GetArrayItem` _overlappingactors (`KismetMathLibrary.MinOfFloatArray` (`local.Local Dis`)))))
    (:`0`
      (return null))
    (:`1`
      (return null))
    (:`2`
      (if (and (!= _output (`local.First Tunder`)) (!= (`|GetArrayItem` _overlappingactors 1) self))
        (return _output)
        (else
          (return null))))))

(fn `Get Highest Building ATP`
  (returns (`Highest Building` :type "Actor Object Reference") (ATP :type Integer))
  (locals (`Local ATP` :type "Array of Integer"))
  (bind _overlappingactors (`PrimitiveComponent.GetOverlappingActors` (`self.RecognitionBoundary`) "/Game/Building/BP_BaseBuilding.BP_BaseBuilding_C"))
  (bind (_indexofmaxvalue _maxvalue) (`KismetMathLibrary.MaxOfIntArray` (`local.Local ATP`)))
  (bind _output (`|GetArrayItem` _overlappingactors))
  (switch `int` (`KismetArrayLibrary.Array_Length` _overlappingactors)
    (:`Default`
      (for _array_element _overlappingactors
        (bind _asbp_base_building (cast `/Game/Building/BP_BaseBuilding` _array_element))
        (`KismetArrayLibrary.Array_Add` (`local.Local ATP`) (`/Game/Building/BP_BaseBuilding.ATP` _asbp_base_building)))
      (return (`|GetArrayItem` _overlappingactors _indexofmaxvalue) _maxvalue))
    (:`0`
      (return null 0))
    (:`1`
      (bind _asbp_base_building_2 (cast `/Game/Building/BP_BaseBuilding` _output))
      (return _output (`/Game/Building/BP_BaseBuilding.ATP` _asbp_base_building_2)))))

(fn `Get Player ATP`
  (returns (`Highest Building` :type "Actor Object Reference") (ATP :type Integer))
  (locals (`Local ATP` :type "Array of Integer"))
  (bind _overlappingactors (`PrimitiveComponent.GetOverlappingActors` (`self.RecognitionBoundary`) "/Game/TopDown/Blueprints/BP_Player.BP_Player_C"))
  (bind _output (`|GetArrayItem` _overlappingactors))
  (switch `int` (`KismetArrayLibrary.Array_Length` _overlappingactors)
    (:`0`
      (return null 0))
    (:`1`
      (bind _asbp_player (cast `/Game/TopDown/Blueprints/BP_Player` _output))
      (return _output (`/Game/TopDown/Blueprints/BP_Player.ATP` _asbp_player)))))

(fn `GetDataTables`
  (bind _returnvalue (`|GetDataTableRow` "/Game/NPC/EnemeyNPC/DT_EnemyAI/DT_EnemyAI.DT_EnemyAI" (`self.Row Name`))
    (:`then`
      (set `self.Enemy Npc Type` (break `/Game/NPC/EnemeyNPC/ST_EnemyAI/ST_EnemyAI` _returnvalue))
      (set `self.Enemy Npc Tier` (`.EnemyNpc_Tier_72_8A10BAD448DB95BAD9A9769DCC581A20` (break `/Game/NPC/EnemeyNPC/ST_EnemyAI/ST_EnemyAI` _returnvalue)))
      (set `self.Enemy Npc Name` (`.EnemyNpcName_34_21E3BE9947ACDA714B9CB8A44EB9FD75` (break `/Game/NPC/EnemeyNPC/ST_EnemyAI/ST_EnemyAI` _returnvalue)))
      (set `self.Enemy Npc Max Health` (`.EnemyNpc_MaxHealth_73_A3186F5C4717757B61D465B7BC59B1AD` (break `/Game/NPC/EnemeyNPC/ST_EnemyAI/ST_EnemyAI` _returnvalue)))
      (set `self.Enemy Npc Run Speed` (`.EnemyNpc_RunSpeed_63_93832079484F9CA58DD1C4AD241E2C1C` (break `/Game/NPC/EnemeyNPC/ST_EnemyAI/ST_EnemyAI` _returnvalue)))
      (set `self.Enemy Npc Walk Speed` (`.EnemyNpc_WalkSpeed_74_30906888497B6042683C449DEE75079A` (break `/Game/NPC/EnemeyNPC/ST_EnemyAI/ST_EnemyAI` _returnvalue)))
      (set `self.Enemy Npc Atk Dmg` (`.EnemyNpc_AtkDmg_64_932E28AB484327D55D80A5B0F352DFA7` (break `/Game/NPC/EnemeyNPC/ST_EnemyAI/ST_EnemyAI` _returnvalue)))
      (set `self.Enemy Npc Atk Dist` (`.EnemyNpc_AtkDist_45_970DCD12469952AAD26365A7224C3D71` (break `/Game/NPC/EnemeyNPC/ST_EnemyAI/ST_EnemyAI` _returnvalue)))
      (set `self.Enemy Npc Atk Spd` (`.EnemyNpc_AtkSpd_44_536C54714FE657A581EBE5BA23C1731E` (break `/Game/NPC/EnemeyNPC/ST_EnemyAI/ST_EnemyAI` _returnvalue)))
      (set `self.Lizard Hp Regen` (`.Lizard_HpRegen_65_5611DD3B426F3C9D3E35A4A9883BF811` (break `/Game/NPC/EnemeyNPC/ST_EnemyAI/ST_EnemyAI` _returnvalue)))
      (set `self.Enemy Npc Atk Rng` (`.EnemyNpc_AtkRng_46_FBA613BD4EC0FDCB9D2CCBAFF6923B80` (break `/Game/NPC/EnemeyNPC/ST_EnemyAI/ST_EnemyAI` _returnvalue)))
      (set `self.Iron Mace Skill Atk Dmg` (`.IronMace_SkillAtkDmg_70_282635DF4DE01C767E0A1C9627BDB7D4` (break `/Game/NPC/EnemeyNPC/ST_EnemyAI/ST_EnemyAI` _returnvalue)))
      (set `self.Mg Sk Skill Spawn Count` (`.MgSk_SkillSpawnCount_57_1912802C44B4CC84AC27109D2F61055F` (break `/Game/NPC/EnemeyNPC/ST_EnemyAI/ST_EnemyAI` _returnvalue)))
      (set `self.PT Atk Rng Dmg` (`.PT_AtkRngDmg_69_24F05C8E417110BA136DE2A417382FE1` (break `/Game/NPC/EnemeyNPC/ST_EnemyAI/ST_EnemyAI` _returnvalue)))
      (set `self.PT Atk Dmg` (`.PT_AtkDmg_68_03D316084817D1FF296B05B2790B3A80` (break `/Game/NPC/EnemeyNPC/ST_EnemyAI/ST_EnemyAI` _returnvalue)))
      (set `self.Claw Skill Atk Dmg` (`.Claw_SkillAtkDmg_71_ADAF268E493FDB527CE451A60C01BC94` (break `/Game/NPC/EnemeyNPC/ST_EnemyAI/ST_EnemyAI` _returnvalue)))
      (set `self.Lizard Regen Time` (`.Lizard_RegenTime_66_0DAB566B45B1B0BB93536BB2026388FA` (break `/Game/NPC/EnemeyNPC/ST_EnemyAI/ST_EnemyAI` _returnvalue)))
      (set `self.Lizard No Hit Time` (`.Lizard_NoHitTime_67_90206DA74B423A80E2422FA1CEFE0023` (break `/Game/NPC/EnemeyNPC/ST_EnemyAI/ST_EnemyAI` _returnvalue)))
      (set `self.PT Atk Rng` (`.PT_AtkRng_77_4AD21E8E45898380D53F2C991D5C6F33` (break `/Game/NPC/EnemeyNPC/ST_EnemyAI/ST_EnemyAI` _returnvalue)))
      (set `self.Enemy Skill Cool Time` (`.Skill_Cool_Time_84_FAC927CC494FFB4C8D82A1BB1DB213FD` (break `/Game/NPC/EnemeyNPC/ST_EnemyAI/ST_EnemyAI` _returnvalue)))
      (set `self.Enemy Skill Atk Spd` (`.Skill_Atk_Spd_82_DED963534A444D844E8976B1E83CE5F2` (break `/Game/NPC/EnemeyNPC/ST_EnemyAI/ST_EnemyAI` _returnvalue)))
      (set `self.Aggression Run Speed` (`.Aggression_Run_Speed_88_B6F4B84246AF0BBBC703998C9B0A7CD4` (break `/Game/NPC/EnemeyNPC/ST_EnemyAI/ST_EnemyAI` _returnvalue))))))

(fn `Init Enemy Controller`)

(fn `IsReachableTarget`
  (params (Actor :type "Actor Object Reference"))
  (returns (bPartial :type Boolean))
  (bind _returnvalue (`NavigationSystemV1.FindPathToLocationSynchronously` (`self.K2_GetActorLocation`) (`self.K2_GetActorLocation` Actor) null null))
  (if (and (`NavigationPath.IsValid` _returnvalue) (not (`NavigationPath.IsPartial` _returnvalue)))
    (return true)
    (else
      (return false))))

(fn `RenewATP`
  (params (TargetActor :type "Actor Object Reference") (TargetComponent :type "PrimitiveComponent Object Reference") (BeginOverlap :type Boolean))
  (locals (Target :type "Actor Object Reference") (TargetComp :type "PrimitiveComponent Object Reference"))
  (set `local.TargetComp` TargetComponent)
  (set `local.Target` TargetActor)
  (if BeginOverlap
    (`KismetArrayLibrary.Array_AddUnique` (`self.ATPTargets`) (`local.Target`))
    (elif (not (`ActorComponent.ComponentHasTag` (`local.TargetComp`) "Player"))
      (`KismetArrayLibrary.Array_RemoveItem` (`self.ATPTargets`) (`local.Target`) :!label _label)
      (elif (not (`self.neverStopChasing`))
        (goto _label)))))

(fn `SetAttackTarget`
  (params (AttackTarget :type "Actor Object Reference"))
  (bind _returnvalue (`AIBlueprintHelperLibrary.GetBlackboard` (`AIBlueprintHelperLibrary.GetAIController` self)))
  (bind _output_get (set `self.HighestATPTarget` AttackTarget))
  (`/Engine/EditorBlueprintResources/StandardMacros.IsValid` _output_get
    (:`Is Valid`
      (`BlackboardComponent.SetValueAsObject` _returnvalue (`self.AttackTarget`) _output_get))
    (:`Is Not Valid`
      (`BlackboardComponent.SetValueAsObject` _returnvalue (`self.AttackTarget`) null))))

(fn `Spawn First Thunder`
  (params (`Thunder Target` :type "Actor Object Reference"))
  (locals (`Whats Target` :type "Actor Object Reference") (Scale :type "Float (double-precision)" :default 800.0))
  (bind _returnvalue (`self.K2_GetActorLocation`))
  (bind _whats_target (`local.Whats Target`))
  (set `local.Whats Target` `Thunder Target`)
  (`/Engine/EditorBlueprintResources/StandardMacros.IsValid` _whats_target
    (:`Is Valid`
      (`|SpawnActorFromClass` "/Game/Building/AttackBuilding/BP/Weapons/BP_Thunder_Base.BP_Thunder_Base_C" (`KismetMathLibrary.MakeTransform` _returnvalue (`KismetMathLibrary.FindLookAtRotation` _returnvalue (`self.K2_GetActorLocation` _whats_target)) (`KismetMathLibrary.Conv_DoubleToVector` (/ (`self.GetDistanceTo` _whats_target) (`local.Scale`)))) "Undefined" "MultiplyWithRoot" null null 10.0 null)
      (bind _returnvalue_2 (`GameplayStatics.GetActorOfClass` "/Game/Building/AttackBuilding/BP/BP_WizardBuildingLv3.BP_WizardBuildingLv3_C"))
      (bind _asbp_enemy_ai_base_new (cast `/Game/NPC/EnemeyNPC/BP/BP_EnemyAI_Base_New` (`local.Whats Target`)))
      (`self.Take Damage` _asbp_enemy_ai_base_new false (* (`/Game/Building/BP_BaseBuilding.Building PT Atk Dmg` _returnvalue_2) (/ 4.0 5.0)) false)
      (`self.second Thunder Attacked` _asbp_enemy_ai_base_new))))

(fn `Spawn Second Thunder`
  (params (`Thunder Target` :type "Actor Object Reference"))
  (locals (`Whats Target` :type "Actor Object Reference") (Scale :type "Float (double-precision)" :default 800.0))
  (bind _returnvalue (`self.K2_GetActorLocation`))
  (bind _whats_target (`local.Whats Target`))
  (set `local.Whats Target` `Thunder Target`)
  (`/Engine/EditorBlueprintResources/StandardMacros.IsValid` _whats_target
    (:`Is Valid`
      (`|SpawnActorFromClass` "/Game/Building/AttackBuilding/BP/Weapons/BP_Thunder_Base.BP_Thunder_Base_C" (`KismetMathLibrary.MakeTransform` _returnvalue (`KismetMathLibrary.FindLookAtRotation` _returnvalue (`self.K2_GetActorLocation` _whats_target)) (`KismetMathLibrary.Conv_DoubleToVector` (/ (`self.GetDistanceTo` _whats_target) (`local.Scale`)))) "Undefined" "MultiplyWithRoot" null null 10.0 null)
      (bind _returnvalue_2 (`GameplayStatics.GetActorOfClass` "/Game/Building/AttackBuilding/BP/BP_WizardBuildingLv3.BP_WizardBuildingLv3_C"))
      (bind _asbp_enemy_ai_base_new (cast `/Game/NPC/EnemeyNPC/BP/BP_EnemyAI_Base_New` (`local.Whats Target`)))
      (`self.Take Damage` _asbp_enemy_ai_base_new false (* (`/Game/Building/BP_BaseBuilding.Building PT Atk Dmg` _returnvalue_2) (/ 3.0 5.0)) false))))

(fn `Update Damaged Health Bar`
  (params (damage :type "Float (double-precision)"))
  (set `self.curHealth` (- (`self.curHealth`) damage))
  (return))

(fn `UserConstructionScript`)