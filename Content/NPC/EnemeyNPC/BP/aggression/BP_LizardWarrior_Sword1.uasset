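; BP_LizardWarrior_Sword1 is a sword-wielding lizard warrior enemy NPC that switches off its parent's skill use at BeginPlay.
; Attack plays the DrakeWarrior attack montage at the NPC's attack speed while it is alive.
; SwordCollision overlaps apply attack damage to players and buildings through allied component tags, and EndSwordAttackDamage disables that collision.
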(event `self.ReceiveBeginPlay`
  ;[1 1 1] 부모의 스킬 사용 방지
  (set `self.PlaySkill` false)
  (`parent.ReceiveBeginPlay`))

(event `self.SwordCollision.OnComponentBeginOverlap`
  (params (OverlappedComponent :type "PrimitiveComponent Object Reference") (OtherActor :type "Actor Object Reference") (OtherComp :type "PrimitiveComponent Object Reference") (OtherBodyIndex :type Integer) (bFromSweep :type Boolean) (SweepResult :type "HitResult Structure (by ref)"))
  (bind _enemy_npc_atk_dmg (`self.Enemy Npc Atk Dmg`))
  ;[1 1 1] 아군이 칼에 닿으면 데미지 입음
  (`|ExecutionSequence`
    (:`then_0`
      (if (`ActorComponent.ComponentHasTag` OtherComp "PlayerAllies")
        (bind _asbp_player (cast `/Game/TopDown/Blueprints/BP_Player` OtherActor))
        (`/Game/TopDown/Blueprints/BP_Player.DamagePlayer` _asbp_player _enemy_npc_atk_dmg)))
    (:`then_1`
      (if (`ActorComponent.ComponentHasTag` OtherComp "BuildingAllies")
        (bind _asbp_base_building (cast `/Game/Building/BP_BaseBuilding` OtherActor))
        (`/Game/Building/BP_BaseBuilding.Take Damage` _asbp_base_building _enemy_npc_atk_dmg)))))

(event `EndSwordAttackDamage`
  ;[1 1 1] 칼 콜리전 취소
  (`PrimitiveComponent.SetCollisionEnabled` (`self.SwordCollision`) "NoCollision"))

(fn `Attack`
  (returns (`Animation Duration` :type "Float (double-precision)"))
  (if (not (`self.IsNPCDead?`))
    (bind _returnvalue (`AnimInstance.Montage_Play` (`SkeletalMeshComponent.GetAnimInstance` (`self.Mesh`)) "/Game/Animations/Melee/DrakeWarrior_Attack_Montage.DrakeWarrior_Attack_Montage" (`self.Enemy Npc Atk Spd`) "Duration" 0.0 true))
    (return _returnvalue)))

(fn `UserConstructionScript`
  (`parent.UserConstructionScript`))