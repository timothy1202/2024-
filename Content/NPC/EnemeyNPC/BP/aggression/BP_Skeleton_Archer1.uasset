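; Skeleton archer enemy NPC that fights with a bow and comes back as a sword skeleton when it dies.
; Attack plays the bow montage at the NPC's attack speed while alive.
; ShootArrow spawns a BP_Arrow at the Arrow1 component and fires it at the blackboard's AttackPlayer target.
; On first death, DestroyActor spawns an AI BP_Skeleton_Sword in its place, clearing that skeleton's FirstTimeToDie flag.
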(event `self.ReceiveBeginPlay`
  (set `self.bFirstTimeToDie?` true)
  (`parent.ReceiveBeginPlay`))

(event `ShootArrow`
  (bind (_returnvalue_location _returnvalue_rotation) (`KismetMathLibrary.BreakTransform` (`SceneComponent.K2_GetComponentToWorld` (`self.Arrow1`))))
  ;[1 1 1] 활 공격
  (bind _returnvalue (`|SpawnActorFromClass` "/Game/NPC/EnemeyNPC/BP/Weapon_BP/BP_Arrow.BP_Arrow_C" (`KismetMathLibrary.MakeTransform` _returnvalue_location _returnvalue_rotation) "AlwaysSpawn" "MultiplyWithRoot" null null))
  (bind `_as액터` (cast `Actor` (`BlackboardComponent.GetValueAsObject` (`AIBlueprintHelperLibrary.GetBlackboard` (`AIBlueprintHelperLibrary.GetAIController` self)) (`self.Attack Player`))))
  (`/Game/NPC/EnemeyNPC/BP/Weapon_BP/BP_Arrow.ShootArrow` _returnvalue `_as액터`))

(fn `Attack`
  (returns (`Animation Duration` :type "Float (double-precision)"))
  (if (not (`self.IsNPCDead?`))
    (bind _returnvalue (`AnimInstance.Montage_Play` (`SkeletalMeshComponent.GetAnimInstance` (`self.Mesh`)) "/Game/Assets/SkeletonEnemy/Animations/Anim_AttackBow_Montage.Anim_AttackBow_Montage" (`self.Enemy Npc Atk Spd`) "Duration" 0.0 true))
    (return _returnvalue)))

(fn `Destroy Actor?`
  (bind _capsulecomponent (`self.CapsuleComponent`))
  (if (`self.bFirstTimeToDie?`)
    (bind _returnvalue (`AIBlueprintHelperLibrary.SpawnAIFromClass` "/Game/NPC/EnemeyNPC/BP/hunt/BP_Skeleton_Sword.BP_Skeleton_Sword_C" null (`SceneComponent.K2_GetComponentLocation` _capsulecomponent) (`SceneComponent.K2_GetComponentRotation` _capsulecomponent) false null))
    (bind _asbp_skeleton_sword (cast `/Game/NPC/EnemeyNPC/BP/hunt/BP_Skeleton_Sword` _returnvalue))
    (set `/Game/NPC/EnemeyNPC/BP/hunt/BP_Skeleton_Sword.bFirstTimeToDie?` false _asbp_skeleton_sword)
    (`self.K2_DestroyActor`)
    (else
      (`parent.Destroy Actor?`))))

(fn `UserConstructionScript`
  (`parent.UserConstructionScript`))