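; Orc enemy NPC variant that attacks by throwing rocks.
; Attack plays a standing one-handed magic attack montage at the NPC's attack speed, provided the NPC is not dead.
; A separate ThrowRock event spawns a BP_Rock at the Arrow1 component's world location and rotation, always spawning regardless of collision.
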(event `ThrowRock`
  (bind (_returnvalue_location _returnvalue_rotation) (`KismetMathLibrary.BreakTransform` (`SceneComponent.K2_GetComponentToWorld` (`self.Arrow1`))))
  ;[1 1 1] 돌 투척
  (`|SpawnActorFromClass` "/Game/NPC/EnemeyNPC/BP/Weapon_BP/BP_Rock.BP_Rock_C" (`KismetMathLibrary.MakeTransform` _returnvalue_location _returnvalue_rotation) "AlwaysSpawn" "MultiplyWithRoot" null null))

(fn `Attack`
  (returns (`Animation Duration` :type "Float (double-precision)"))
  (if (not (`self.IsNPCDead?`))
    (bind _returnvalue (`AnimInstance.Montage_Play` (`SkeletalMeshComponent.GetAnimInstance` (`self.Mesh`)) "/Game/Animations/ORC_STONE_animation/Orc_Attack_AnimationStanding_1H_Magic_Attack_03_Fixed_Montage.Orc_Attack_AnimationStanding_1H_Magic_Attack_03_Fixed_Montage" (`self.Enemy Npc Atk Spd`) "Duration" 0.0 true))
    (return _returnvalue)))

(fn `UserConstructionScript`
  (`parent.UserConstructionScript`))