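; Skeleton wizard enemy NPC that attacks with fireballs and summons BP_Skeleton_Hand minions.
; A looping cooldown timer flags the skill as ready, so the next Attack plays the area-spell montage instead of the normal one.
; Separate events spawn the fireball at AttackDirection and the minion at a random nearby XY offset; neither is called within this graph.
; NpcDead clears the timer once IsNPCDead is set.
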(event `SpawnSkeletonFireBall`
  (bind _attackdirection (`self.AttackDirection`))
  ;[1 1 1] 파이어볼 공격
  (`|SpawnActorFromClass` "/Game/NPC/EnemeyNPC/BP/Weapon_BP/BP_Skeleton_Fireball.BP_Skeleton_Fireball_C" (`KismetMathLibrary.MakeTransform` (`SceneComponent.K2_GetComponentLocation` _attackdirection) (`SceneComponent.K2_GetComponentRotation` _attackdirection)) "Undefined" "MultiplyWithRoot" null null))

(event `self.ReceiveBeginPlay`
  ;[1 1 1] 근접 스켈레톤 소환
  (`parent.ReceiveBeginPlay`)
  (bind _returnvalue (`KismetSystemLibrary.K2_SetTimerDelegate` (delegate `SpawnActorAtRandomLocation`) (`self.Enemy Skill Cool Time`) true))
  (set `self.SpawnTimerHandle` _returnvalue))

(event `SpawnActorAtRandomLocation`
  ;[1 1 1] 근접 스켈레톤 소환
  (set `self.isPlayingSkill` true))

(event `SpawnSk`
  (bind (_returnvalue_x _returnvalue_y _returnvalue_z) (`KismetMathLibrary.BreakVector` (`self.K2_GetActorLocation`)))
  ;[1 1 1] 스폰
  (bind _output_get (set `self.EnemySpawnLocation` (`KismetMathLibrary.MakeVector` (+ _returnvalue_x (`KismetMathLibrary.RandomFloatInRange` -400.0 400.0)) (+ _returnvalue_y (`KismetMathLibrary.RandomFloatInRange` -400.0 400.0)) _returnvalue_z)))
  (`AIBlueprintHelperLibrary.SpawnAIFromClass` "/Game/NPC/EnemeyNPC/BP/hunt/BP_Skeleton_Hand.BP_Skeleton_Hand_C" null _output_get (struct) false null)
  (`KismetSystemLibrary.Delay` 1.0))

(event `self.NpcDead`
  ;[1 1 1] 죽으면 스킬 실행 못하게
  (if (`self.IsNPCDead?`)
    (`KismetSystemLibrary.K2_ClearAndInvalidateTimerHandle` (`self.SpawnTimerHandle`))
    (`parent.NpcDead`)))

(fn `Attack`
  (returns (`Animation Duration` :type "Float (double-precision)"))
  (if (`self.IsNPCDead?`)
    _
    (elif (`self.isPlayingSkill`)
      (bind _returnvalue (`AnimInstance.Montage_Play` (`SkeletalMeshComponent.GetAnimInstance` (`self.Mesh`)) "/Game/Animations/Magic_Skeleton_animation/Magic_SK_Skill_SpellStanding_2H_Magic_Area_Attack_01_Fixed_Montage.Magic_SK_Skill_SpellStanding_2H_Magic_Area_Attack_01_Fixed_Montage" (`self.Enemy Skill Atk Spd`) "Duration" 0.0 true))
      (set `self.isPlayingSkill` false)
      (return _returnvalue)
      (else
        (bind _returnvalue_2 (`AnimInstance.Montage_Play` (`SkeletalMeshComponent.GetAnimInstance` (`self.Mesh`)) "/Game/Animations/Magic_Skeleton_animation/Magic_SK_Normal_AttackStanding_1H_Magic_Attack_01__1__Fixed_Montage.Magic_SK_Normal_AttackStanding_1H_Magic_Attack_01__1__Fixed_Montage" (`self.Enemy Npc Atk Spd`) "Duration" 0.0 true))
        (return _returnvalue_2)))))

(fn `UserConstructionScript`
  (`parent.UserConstructionScript`))