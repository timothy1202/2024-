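; Mace-wielding orc enemy NPC that damages allied players and buildings when its mace collision overlaps them.
; A looping cooldown timer arms a skill flag, cleared on death.
; Attack plays a 360 skill montage when the flag is set, otherwise a downward swing.
; Overlap damage picks skill or normal values from that flag, which Attack resets immediately after starting the skill montage.
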(event `self.MaceCollsion.OnComponentBeginOverlap`
  (params (OverlappedComponent :type "PrimitiveComponent Object Reference") (OtherActor :type "Actor Object Reference") (OtherComp :type "PrimitiveComponent Object Reference") (OtherBodyIndex :type Integer) (bFromSweep :type Boolean) (SweepResult :type "HitResult Structure (by ref)"))
  ;[1 1 1] 아군이 스킬에 닿으면 피해 입음
  (`|ExecutionSequence`
    (:`then_0`
      (if (`ActorComponent.ComponentHasTag` OtherComp "PlayerAllies")
        (bind _asbp_player (cast `/Game/TopDown/Blueprints/BP_Player` OtherActor))
        (if (`self.isPlayingSkill`)
          (`/Game/TopDown/Blueprints/BP_Player.DamagePlayer` _asbp_player (`self.Iron Mace Skill Atk Dmg`))
          (else
            (`/Game/TopDown/Blueprints/BP_Player.DamagePlayer` _asbp_player (`self.Enemy Npc Atk Dmg`))))))
    (:`then_1`
      (if (`ActorComponent.ComponentHasTag` OtherComp "BuildingAllies")
        (bind _asbp_base_building (cast `/Game/Building/BP_BaseBuilding` OtherActor))
        (if (`self.isPlayingSkill`)
          (`/Game/Building/BP_BaseBuilding.Take Damage` _asbp_base_building (`self.Iron Mace Skill Atk Dmg`))
          (else
            (`/Game/Building/BP_BaseBuilding.Take Damage` _asbp_base_building (`self.Enemy Npc Atk Dmg`))))))))

(event `self.ReceiveBeginPlay`
  ;[1 1 1] 철퇴 스킬
  (`parent.ReceiveBeginPlay`)
  (bind _returnvalue (`KismetSystemLibrary.K2_SetTimerDelegate` (delegate `Mace Skill`) (`self.Enemy Skill Cool Time`) true))
  (set `self.SkillHandle` _returnvalue))

(event `Mace Skill`
  ;[1 1 1] 철퇴 스킬
  (set `self.isPlayingSkill` true))

(event `self.NpcDead`
  ;[1 1 1] 죽으면 스킬 실행 못하게
  (if (`self.IsNPCDead?`)
    (`KismetSystemLibrary.K2_ClearAndInvalidateTimerHandle` (`self.SkillHandle`))
    (`parent.NpcDead`)))

(fn `Attack`
  (returns (`Animation Duration` :type "Float (double-precision)"))
  (if (`self.IsNPCDead?`)
    _
    (elif (`self.isPlayingSkill`)
      (bind _returnvalue (`AnimInstance.Montage_Play` (`SkeletalMeshComponent.GetAnimInstance` (`self.Mesh`)) "/Game/Animations/ORC_IRON_MACE_Animation/Mace_Skill_AttackStanding_Melee_Attack_360_High_Fixed_Montage.Mace_Skill_AttackStanding_Melee_Attack_360_High_Fixed_Montage" (`self.Enemy Skill Atk Spd`) "Duration" 0.0 true))
      (set `self.isPlayingSkill` false)
      (return _returnvalue)
      (else
        (bind _returnvalue_2 (`AnimInstance.Montage_Play` (`SkeletalMeshComponent.GetAnimInstance` (`self.Mesh`)) "/Game/Animations/ORC_IRON_MACE_Animation/Mace_Normal_AttackStanding_Melee_Attack_Downward_Fixed_Montage.Mace_Normal_AttackStanding_Melee_Attack_Downward_Fixed_Montage" (`self.Enemy Npc Atk Spd`) "Duration" 0.0 true))
        (return _returnvalue_2)))))

(fn `UserConstructionScript`
  (`parent.UserConstructionScript`))