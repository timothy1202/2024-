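; BP_Spawner is an NPC wave spawner that places units in a grid formation relative to its Arrow component.
; BeginPlay caches per-enemy wave values and clear rewards from the DT_Wave row named by RowName.
; SpawnNpc wraps SpawnUnitCount units into rows of MaxColumnUnitNum, and Spawn creates each as an aggressive actor using SpawnRowName.
; Unconnected nodes hold triggers for waves 1, 16 and 30, including boss summon cinematics.
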(event `self.ReceiveBeginPlay`
  (`self.GetDataTables`))

(event `Spawn Npc`
  ;[1 1 1] 건설 시 스폰
  (for _index (range (`self.Spawn Unit Count`))
    (set `self.Now Index` _index)
    (bind _output_get (set `self.Column Count` (mod _index (`self.Max Column Unit Num`))))
    (if (== _output_get 0)
      (`/Engine/EditorBlueprintResources/StandardMacros.IncrementInt` (`self.Row Count`)
        (:`  `
          _)))
    (`self.Spawn` (`self.Column Count`))))

(event `Spawn`
  (params (Index :type Integer))
  (bind (_returnvalue_location _returnvalue_rotation) (`KismetMathLibrary.BreakTransform` (`SceneComponent.K2_GetComponentToWorld` (`self.Arrow`))))
  ;[1 1 1] 코멘트
  (set `self.My Index` Index)
  (`|SpawnActorFromClass` (`self.Class`) (`KismetMathLibrary.MakeTransform` (+ (* (`SceneComponent.GetForwardVector` (`self.Arrow`)) (* (`self.Row Count`) 150)) (* (`SceneComponent.GetRightVector` (`self.Arrow`)) (* (`self.My Index`) 100)) _returnvalue_location) _returnvalue_rotation) "AdjustIfPossibleButAlwaysSpawn" "MultiplyWithRoot" null (`self.Spawn Row Name`) true null))

(event `Key|Seven`
  (params (Key :type "Key Structure"))
  ;[1 1 1] Wave1
)

(event `Key|Eight`
  (params (Key :type "Key Structure"))
  ;[1 1 1] Wave16
)

(event `Key|Nine`
  (params (Key :type "Key Structure"))
  ;[1 1 1] Wave30
)

(fn `GetDataTables`
  (locals (NewLocalVar :type Integer))
  (bind _returnvalue (`|GetDataTableRow` "/Game/NPC/SpawnWave/Wave/DT_Wave/DT_Wave.DT_Wave" (`self.Row Name`))
    (:`then`
      (set `self.Wave Skeleton Hand` (break `/Game/NPC/SpawnWave/Wave/ST_Wave/ST_Wave` _returnvalue))
      (set `self.Wave Skeleton Sword` (`.BP_Skeleton_Sword_134_9358F4F54EDBF65E625833942029D71B` (break `/Game/NPC/SpawnWave/Wave/ST_Wave/ST_Wave` _returnvalue)))
      (set `self.Wave Skeleton Archer` (`.BP_Skeleton_Archer_135_4585B8FF4A8A25DD5A506A9BB5BBC973` (break `/Game/NPC/SpawnWave/Wave/ST_Wave/ST_Wave` _returnvalue)))
      (set `self.Wave Skeleton Wizard` (`.BP_Skeleton_Wizard_136_33236DA54D4B681E6A85DC9EFC3437F3` (break `/Game/NPC/SpawnWave/Wave/ST_Wave/ST_Wave` _returnvalue)))
      (set `self.Wave Orc Hand` (`.BP_Orc_Hand_138_34B33C6A4DDCB87C0D01DF850F2EAAE1` (break `/Game/NPC/SpawnWave/Wave/ST_Wave/ST_Wave` _returnvalue)))
      (set `self.Wave Skeleton Boss Staff` (`.Skeleton_Boss_Staff_137_6186EF8B4FFF5F8F5588B9ACCE110E13` (break `/Game/NPC/SpawnWave/Wave/ST_Wave/ST_Wave` _returnvalue)))
      (set `self.Wave Orc Throw Rock` (`.BP_Orc_ThrowRock_139_E49B307A475F2FB872703B8C35669B27` (break `/Game/NPC/SpawnWave/Wave/ST_Wave/ST_Wave` _returnvalue)))
      (set `self.Wave Orc Mace` (`.BP_Orc_mace_140_D7BD70C846F6D49CDC678681AD515141` (break `/Game/NPC/SpawnWave/Wave/ST_Wave/ST_Wave` _returnvalue)))
      (set `self.Wave Boss Orc` (`.BP_Boss_Orc_141_976AC907474501801116DFA6F0C0B0C8` (break `/Game/NPC/SpawnWave/Wave/ST_Wave/ST_Wave` _returnvalue)))
      (set `self.Wave Lizard Warrior Sword` (`.BP_LizardWarrior_Sword_142_7C62782243BE1162C162CEA887F7E21F` (break `/Game/NPC/SpawnWave/Wave/ST_Wave/ST_Wave` _returnvalue)))
      (set `self.Wave Lizard Wizard` (`.BP_LizardWizard_143_04E5072C469784011E26D499249EC1B7` (break `/Game/NPC/SpawnWave/Wave/ST_Wave/ST_Wave` _returnvalue)))
      (set `self.Wave Lizard Warrior Hand` (`.BP_LizardWarrior_Hand_144_6C1A48064A57006E7D3E5FA00F896C9E` (break `/Game/NPC/SpawnWave/Wave/ST_Wave/ST_Wave` _returnvalue)))
      (set `self.Wave Boss Lizard Warrior Hand` (`.BP_Boss_LizardWarrior_Hand_145_C619576B46FC87D0DDA1109C86917A6B` (break `/Game/NPC/SpawnWave/Wave/ST_Wave/ST_Wave` _returnvalue)))
      (set `self.Wave Clear Gold` (`.Wave_Clear_Gold_146_D7DC4F5B48F8CAACF5DD2BB1170ABCA5` (break `/Game/NPC/SpawnWave/Wave/ST_Wave/ST_Wave` _returnvalue)))
      (set `self.Wave Clear Skeleton Crystal` (`.Wave_Clear_Skeleton_Crystal_147_BB7BA4004669A9956437B4AA59D29247` (break `/Game/NPC/SpawnWave/Wave/ST_Wave/ST_Wave` _returnvalue)))
      (set `self.Wave Clear Orc Crystal` (`.Wave_Clear_Orc_Crystal_148_22BF37564AB8FA7B9407DCACAEECB23F` (break `/Game/NPC/SpawnWave/Wave/ST_Wave/ST_Wave` _returnvalue)))
      (set `self.Wave Clear Lizard Crystal` (`.Wave_Clear_Lizard_Crystal_149_54A2239D490CE09130DE128890997867` (break `/Game/NPC/SpawnWave/Wave/ST_Wave/ST_Wave` _returnvalue))))))

(fn `UserConstructionScript`)