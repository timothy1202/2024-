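; BP_TutorialMap_VideoPlay is a one-shot trigger for the tutorial map that starts a tutorial video when the player enters its sphere.
; On overlap with a BP_Player, it opens a hard-coded movement and camera-rotation clip on TutoMediaPlayer, then calls the player's TutoMediaPlay.
; It then shows and enables collision on the linked NextCircle, if valid, and destroys itself, so triggers can chain in sequence.
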(event OnComponentBeginOverlap(Sphere)
  (params (OverlappedComponent :type Primitive%20Component%20Object%20Reference) (OtherActor :type Actor%20Object%20Reference) (OtherComp :type Primitive%20Component%20Object%20Reference) (OtherBodyIndex :type Integer) (bFromSweep :type Boolean) (SweepResult :type Hit%20Result%20Structure%20%28by%20ref%29))
  (bind _nextcircle (Variables|Default|GetnextCircle))
  (bind _asbp_player (Utilities|Casting|CastToBP_Player OtherActor))
  (Variables|Default|SetBP%20Player _asbp_player)
  (CallFunction|PlayVideo)
  (Utilities|IsValid _nextcircle
    (:Is%20Valid
      (Rendering|SetVisibility (Variables|BP_TutorialMap_VideoPlay_C|GetDefaultSceneRoot _nextcircle) true true)
      (Collision|SetCollisionEnabled (Variables|BP_TutorialMap_VideoPlay_C|GetSphere _nextcircle) "QueryAndPhysics"))
    (:Is%20Not%20Valid
      _))
  (Actor|DestroyActor))

(fn ConstructionScript)

(fn PlayVideo
  (Development|PrintString "비디오 재생")
  (Media|MediaPlayer|OpenSource (Variables|Default|GetTutoMediaPlayer) "/Game/03-MediaPlay/TutoMedia/01-CharacterMove_cameraRotate.01-CharacterMove_cameraRotate")
  (Default|TutoMediaPlay (Variables|Default|GetBP%20Player)))