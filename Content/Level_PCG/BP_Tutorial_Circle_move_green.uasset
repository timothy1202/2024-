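; Green tutorial circle marker linked to a building, chaining the construction steps of the tutorial.
; Its Watched event casts the linked Building to wall, attack tower, barracks or archery range and plays the matching media and Korean explanation through BP_Player.
; Tick polls the building's Built flag, then once either reveals and enables collision on the next linked Circle and destroys itself, or calls CallFinishTuto when no valid Circle exists.
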(event Custom|Watched
  ;[1 1 1] 코멘트
  (Utilities|Casting|CastToBP_Wall_Door_BuildingBase (Variables|Default|Getbuilding)
    (:then
      (Default|TutoMediaPlay (Variables|Default|GetBP%20Player) "/Game/03-MediaPlay/TutoMedia/08-WallConstruct.08-WallConstruct" "08. 방어벽 건설 " "방어벽은 몬스터의 침입을 막을 수 있는 건물입니다.  
 
건물 업그레이드를 통해, 체력을 올릴 수 있습니다. 
 
‘Tab키’를 눌러, 건물 수리키를 누르세요. 골드를 지불하여, 체력을 닳은 건물들을 수리할 수 있습니다."))
    (:CastFailed
      (Utilities|Casting|CastToBP_LongRangeAttackBuilding_Base (Variables|Default|Getbuilding)
        (:then
          (Default|TutoMediaPlay (Variables|Default|GetBP%20Player) "/Game/03-MediaPlay/TutoMedia/09-AttackBuildingConstruct.09-AttackBuildingConstruct" "09. 공격 타워 건설 " "화살을 발사하는 공격 타워 건물입니다.  
 
건물 업그레이드를 통해, 총 8가지 형태 중 하나로 업그레이드할 수 있습니다.  
 
크게 공격 특화, 디버프 특화로 나뉩니다."))
        (:CastFailed
          (Utilities|Casting|CastToBP_Barracks_Building (Variables|Default|Getbuilding)
            (:then
              (Default|TutoMediaPlay (Variables|Default|GetBP%20Player) "/Game/03-MediaPlay/TutoMedia/10-UnitBuildingConstruct_sword.10-UnitBuildingConstruct_sword" "10. 막사 건설" "검사를 육성하는 건물입니다. 건물 업그레이드를 통해, 검사 수가 늘어나고, 검사의 직업을 선택할 수 있습니다. 
 
‘Ctrl 키’를 누른 상태로 원 안에 검사가 포함되면, 소집됩니다. 소집된 검사는 플레이어를 따라다닙니다. 
 
다시 ‘Ctrl 키’를 누르면 해당 장소에 소집되었던 검사가 대형을 갖춰 대기합니다."))
            (:CastFailed
              (Utilities|Casting|CastToBP_Archery_Building (Variables|Default|Getbuilding))
              (Default|TutoMediaPlay (Variables|Default|GetBP%20Player) "/Game/03-MediaPlay/TutoMedia/11-UnitBuildingConstruct_Archer_Muster.11-UnitBuildingConstruct_Archer_Muster" "11. 양궁장 건설" "궁수를 육성하는 건물입니다. 건물 업그레이드를 통해, 궁수 수가 늘어나고, 궁수의 직업을 선택할 수 있습니다. 
 
‘Ctrl 키’를 누른 상태로 원 안에 궁수가 포함되면, 소집됩니다. 소집된 궁수는 플레이어를 따라다닙니다. 
 
다시 ‘Ctrl 키’를 누르면 해당 장소에 소집되었던 궁수가 대형을 갖춰 대기합니다."))))))))

(event EventBeginPlay
  (bind _asbp_player (Utilities|Casting|CastToBP_Player (Game|GetPlayerCharacter 0)))
  (Variables|Default|SetBP%20Player _asbp_player))

(event EventTick
  (params (DeltaSeconds :type Float%20%28single-precision%29))
  (bind _circle (Variables|Default|Getcircle))
  (if (Variables|/Script/GraduationWork2024.BaseBuilding|GetbBuilt (Variables|Default|Getbuilding))
    (Utilities|FlowControl|Sequence
      (:then_0
        (Utilities|FlowControl|DoOnce false
          (:Completed
            (Utilities|IsValid _circle
              (:Is%20Valid
                (Rendering|SetVisibility (Variables|/Game/Level_PCG/BP_Tutorial_Circle_move.BP_Tutorial_Circle_move_C|GetDefaultSceneRoot _circle) true true)
                (Collision|SetCollisionEnabled (Variables|/Game/Level_PCG/BP_Tutorial_Circle_move.BP_Tutorial_Circle_move_C|GetSphere _circle) "QueryAndPhysics")
                (Actor|DestroyActor))
              (:Is%20Not%20Valid
                (Default|CallFinishTuto)))))))))

(fn ConstructionScript)