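; Tutorial waypoint circle that advances a movement tutorial when the player enters its sphere.
; On overlap by BP_Player, it makes the linked next Circle visible and enables that circle's sphere collision, forming a sequential chain.
; If no next Circle is valid, it calls Watched on the linked VideoCircle, if valid.
; The actor destroys itself after either branch.
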(event OnComponentBeginOverlap(Sphere)
  (params (OverlappedComponent :type Primitive%20Component%20Object%20Reference) (OtherActor :type Actor%20Object%20Reference) (OtherComp :type Primitive%20Component%20Object%20Reference) (OtherBodyIndex :type Integer) (bFromSweep :type Boolean) (SweepResult :type Hit%20Result%20Structure%20%28by%20ref%29))
  (bind _circle (Variables|Default|Getcircle))
  (bind _videocircle (Variables|Default|GetvideoCircle))
  (Utilities|Casting|CastToBP_Player OtherActor)
  (Utilities|IsValid _circle
    (:Is%20Valid
      (Rendering|SetVisibility (Variables|BP_Tutorial_Circle_move_C|GetDefaultSceneRoot _circle) true true)
      (Collision|SetCollisionEnabled (Variables|BP_Tutorial_Circle_move_C|GetSphere _circle) "QueryAndPhysics"))
    (:Is%20Not%20Valid
      (Utilities|IsValid _videocircle
        (:Is%20Valid
          (Default|Watched _videocircle))
        (:Is%20Not%20Valid
          _))))
  (Actor|DestroyActor))

(fn ConstructionScript)