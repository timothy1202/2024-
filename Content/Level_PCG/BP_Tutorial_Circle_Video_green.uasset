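; Tutorial step actor that shows the player the headquarters construction and shop videos through the player's TutoMediaPlay.
; A watch event plays the construction video, and Tick waits for the referenced Building to be built, then plays the shop video once.
; Tick then polls the player's EquipType; on the target type, presumably the sword, it reveals MoveCircle, enables its sphere collision and destroys itself.
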(event Custom|watch
  (Default|TutoMediaPlay (Variables|Default|GetBP%20Player) "/Game/03-MediaPlay/TutoMedia/06-HeadQuaterConstruct.06-HeadQuaterConstruct" "06. 본부 건물 건설" "건물 토대 가운데로 다가가 ‘B키’를 누르세요. 건물 건설 UI에 뜬 ‘망치’ 아이콘을 클릭하세요.   
 
자원이 충분하다면 건물을 업그레이드할 수 있습니다."))

(event EventBeginPlay
  (bind _asbp_player (Utilities|Casting|CastToBP_Player (Game|GetPlayerCharacter 0)))
  (Variables|Default|SetBP%20Player _asbp_player))

(event EventTick
  (params (DeltaSeconds :type Float%20%28single-precision%29))
  (bind _movecircle (Variables|Default|GetmoveCircle))
  (if (Variables|/Script/GraduationWork2024.BaseBuilding|GetbBuilt (Variables|Default|GetBuilding))
    (Utilities|FlowControl|Sequence
      (:then_0
        (Utilities|FlowControl|DoOnce false
          (:Completed
            (Default|TutoMediaPlay (Variables|Default|GetBP%20Player) "/Game/03-MediaPlay/TutoMedia/07-Shop.07-Shop" "07. 상점 이용 " "건설된 본부 건물에 다가가 상호 작용키를 누르세요.‘Tab키’ - 건물 상호작용 변경 
 
구매할 장비를 클릭해 아이템 구매 후 장비를 아이템 장착 버튼을 클릭하세요.  
 
왼쪽에 장착한 아이템을 확인할 수 있습니다. 
칼을 구매하세요!")
            (bind _asbp_player (Utilities|Casting|CastToBP_Player (Game|GetPlayerCharacter 0)))
            (Variables|Default|SetPlayer _asbp_player))))
      (:then_1
        (if (Utilities|Enum|Equal(Enum) (Variables|/Game/TopDown/Blueprints/BP_Player.BP_Player_C|GetEquipType (Variables|Default|GetPlayer)) "NewEnumerator0")
          (Rendering|SetVisibility (Variables|/Game/Level_PCG/BP_Tutorial_Circle_move.BP_Tutorial_Circle_move_C|GetDefaultSceneRoot _movecircle) true true)
          (Collision|SetCollisionEnabled (Variables|/Game/Level_PCG/BP_Tutorial_Circle_move.BP_Tutorial_Circle_move_C|GetSphere _movecircle) "QueryAndPhysics")
          (Actor|DestroyActor))))))

(fn ConstructionScript)