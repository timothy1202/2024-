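; BP_DottestCircle is an animated decal actor, apparently a dotted-circle indicator.
; On BeginPlay it starts two timelines: one drives the decal's world scale uniformly, despite its location-themed naming, and the other adds its track value to the actor's yaw on each update.
; A SetActorLocation node with a zero offset is left unconnected and never runs.
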(event `self.ReceiveBeginPlay`
  (bind (_returnvalue_roll _returnvalue_pitch _returnvalue_yaw) (`KismetMathLibrary.BreakRotator` (`self.K2_GetActorRotation`)))
  (`|ExecutionSequence`
    (:`then_0`
      (bind (_direction _locatoinchanger) (`Timeline|ActorMoveTimeline`)
        (:`Update`
          (`SceneComponent.SetWorldScale3D` (`self.Decal`) (`KismetMathLibrary.Conv_DoubleToVector` _locatoinchanger)))))
    (:`then_1`
      (bind (_direction_2 `_새_트랙_0`) (`Timeline|ActorRotateTimeline`)
        (:`Update`
          (`self.K2_SetActorRotation` (`KismetMathLibrary.MakeRotator` _returnvalue_roll _returnvalue_pitch (+ _returnvalue_yaw `_새_트랙_0`))))))))

(fn `UserConstructionScript`)