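; Area actor that changes the level's directional light color as the player moves between two points inside its volume.
; BeginPlay caches the first DirectionalLight in the level, and Area overlap events flag whether the player is inside.
; While inside, Tick projects the player mesh's position onto the PointA–PointB line, clamps the ratio and lerps between two colors, printing debug strings.
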(event `self.ReceiveBeginPlay`
  (bind _outactors (`GameplayStatics.GetAllActorsOfClass` "/Script/Engine.DirectionalLight"))
  (set `self.DirectionalLight` (`|GetArrayItem` _outactors)))

(event `self.ReceiveTick`
  (params (DeltaSeconds :type "Float (single-precision)"))
  (bind _returnvalue (`SceneComponent.K2_GetComponentLocation` (`self.PointA`)))
  (if (`self.isPlayerInArea?`)
    (set `self.VectorAP` (- _returnvalue (`SceneComponent.K2_GetComponentLocation` (`Character.Mesh` (`GameplayStatics.GetPlayerCharacter` 0)))))
    (set `self.VectorAB` (- _returnvalue (`SceneComponent.K2_GetComponentLocation` (`self.PointB`))))
    (set `self.VectorProjectionF` (`KismetMathLibrary.Dot_VectorVector` (`self.VectorAP`) (`KismetMathLibrary.Normal` (`self.VectorAB`))))
    (set `self.VactorRatio` (/ (`self.VectorProjectionF`) (`KismetMathLibrary.VSize` (`self.VectorAB`))))
    (if (<= (`self.VactorRatio`) 0.0)
      (set `self.VactorRatio` 0.0)
      (elif (>= (`self.VactorRatio`) 1.0)
        (set `self.VactorRatio` 1.0)))
    (`KismetSystemLibrary.PrintString` (`KismetStringLibrary.Concat_StrStr` "VectorRatioValue : " (`KismetStringLibrary.Conv_DoubleToString` (`self.VactorRatio`))))
    (`LightComponent.SetLightColor` (`Light.LightComponent` (`self.DirectionalLight`)) (`KismetMathLibrary.LinearColorLerp` (`self.DirectionalLightColorA`) (`self.DirectionalLightColorB`) (`self.VactorRatio`)) true)))

(event `self.Area.OnComponentBeginOverlap`
  (params (OverlappedComponent :type "PrimitiveComponent Object Reference") (OtherActor :type "Actor Object Reference") (OtherComp :type "PrimitiveComponent Object Reference") (OtherBodyIndex :type Integer) (bFromSweep :type Boolean) (SweepResult :type "HitResult Structure (by ref)"))
  (if (== OtherActor (`GameplayStatics.GetPlayerCharacter` 0))
    (set `self.isPlayerInArea?` true)
    (`KismetSystemLibrary.PrintString` "PlayerInArea")))

(event `self.Area.OnComponentEndOverlap`
  (params (OverlappedComponent :type "PrimitiveComponent Object Reference") (OtherActor :type "Actor Object Reference") (OtherComp :type "PrimitiveComponent Object Reference") (OtherBodyIndex :type Integer))
  (if (== OtherActor (`GameplayStatics.GetPlayerCharacter` 0))
    (set `self.isPlayerInArea?` false)
    (`KismetSystemLibrary.PrintString` "PlayerOutArea")))

(fn `UserConstructionScript`)