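; Enemy NPC for a headquarters attack that wields a sword and shows a health bar when the player is near.
; BeginPlay caches the health widget and flags the NPC as going to the player.
; WieldSword spawns a sword on the hand socket, while Attack plays a slash montage and fires OnAttackEnd on completion or interruption.
; HealthSphere overlaps with the player toggle health bar visibility.
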(event `self.ReceiveBeginPlay`
  ;[1 1 1] HP바
  (bind _asai_health_widget (cast `/Game/EnemyNPC/AI_HealthWidget` (`WidgetComponent.GetUserWidgetObject` (`self.HealthWidget`))))
  (set `self.As AI Health Widget` _asai_health_widget)
  (set `self.isGoingToPlayer` true))

(event `Attack`
  (`|PlayMontage` (`self.Mesh`) "/Game/Animations/Melee/Montage_Sword_Slash.Montage_Sword_Slash"
    (:`OnCompleted`
      _)
    (:`OnInterrupted`
      _))
  (`self.OnAttackEnd`))

(event `WieldSword`
  (bind _returnvalue (`|SpawnActorFromClass` "/Game/Weapons/BP_Sword.BP_Sword_C" (`self.GetTransform`) "Undefined" "MultiplyWithRoot" null null))
  (`self.K2_AttachToComponent` _returnvalue (`self.Mesh`) "hand_r_sword_socket" "SnapToTarget" "SnapToTarget" "SnapToTarget" true)
  (set `self.IsWieldingSword` true))

(event `self.HealthSphere.OnComponentBeginOverlap`
  (params (OverlappedComponent :type "PrimitiveComponent Object Reference") (OtherActor :type "Actor Object Reference") (OtherComp :type "PrimitiveComponent Object Reference") (OtherBodyIndex :type Integer) (bFromSweep :type Boolean) (SweepResult :type "HitResult Structure (by ref)"))
  ;[1 1 1] 플레이어가 가까이가면 HP바 보임
  (cast `/Game/TopDown/Blueprints/BP_Player` OtherActor)
  (`SceneComponent.SetVisibility` (`self.HealthWidget`) true false))

(event `self.HealthSphere.OnComponentEndOverlap`
  (params (OverlappedComponent :type "PrimitiveComponent Object Reference") (OtherActor :type "Actor Object Reference") (OtherComp :type "PrimitiveComponent Object Reference") (OtherBodyIndex :type Integer))
  ;[1 1 1] 플레이어가 가까이가면 HP바 보임
  (cast `/Game/TopDown/Blueprints/BP_Player` OtherActor)
  (`SceneComponent.SetVisibility` (`self.HealthWidget`) false false))

(fn `UserConstructionScript`)