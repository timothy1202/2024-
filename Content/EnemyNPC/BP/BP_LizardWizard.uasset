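; BP_LizardWizard is an enemy NPC that attacks by casting fireballs.
; Attack plays the DrakeAssassin spell montage and returns the result of that play call.
; A separate SpawnFireBall event spawns BP_Fireball at a right-thumb socket on the mesh, using the actor's rotation.
; Nothing in this Blueprint calls that event, and its BeginPlay, overlap and Tick events are disabled stubs.
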(event `SpawnFireBall`
  (`|SpawnActorFromClass` "/Game/EnemyNPC/BP/Weapon_BP/BP_Fireball.BP_Fireball_C" (`KismetMathLibrary.MakeTransform` (`SceneComponent.GetSocketLocation` (`self.Mesh`) "thumb_03_r_Socket") (`self.K2_GetActorRotation` self)) "Undefined" "MultiplyWithRoot" null null))

(fn `Attack`
  (returns (`Animation Duration` :type "Float (double-precision)"))
  (bind _returnvalue (`self.PlayAnimMontage` "/Game/Assets/DrakeAssassin/Animations/Anim_DrakeAssassin_spell02_Montage.Anim_DrakeAssassin_spell02_Montage"))
  (return _returnvalue))

(fn `UserConstructionScript`
  (`parent.UserConstructionScript`))