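; BP_Skeleton_Fireball is a fireball projectile, apparently for a skeleton enemy, that explodes on contact.
; Its Sphere's overlap with BP_Player spawns P_Explosion at the fireball's location and destroys the actor.
; A Sphere hit on anything other than BP_Player does the same, so missed shots also clean up.
; The graph applies no damage, and a node setting ExplodeCollision's collision profile is never run.
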(event `self.Sphere.OnComponentBeginOverlap`
  (params (OverlappedComponent :type "PrimitiveComponent Object Reference") (OtherActor :type "Actor Object Reference") (OtherComp :type "PrimitiveComponent Object Reference") (OtherBodyIndex :type Integer) (bFromSweep :type Boolean) (SweepResult :type "HitResult Structure (by ref)"))
  ;[1 1 1] 총알 플레이어 닿았는지
  (cast `/Game/TopDown/Blueprints/BP_Player` OtherActor)
  (`GameplayStatics.SpawnEmitterAtLocation` "/Game/StarterContent/Particles/P_Explosion.P_Explosion" (`self.K2_GetActorLocation`))
  (`/Engine/EditorBlueprintResources/StandardMacros.IsValid` self
    (:`Is Valid`
      (`self.K2_DestroyActor`))))

(event `self.Sphere.OnComponentHit`
  (params (HitComponent :type "PrimitiveComponent Object Reference") (OtherActor :type "Actor Object Reference") (OtherComp :type "PrimitiveComponent Object Reference") (NormalImpulse :type "Vector Structure") (Hit :type "HitResult Structure (by ref)"))
  ;[1 1 1] 플레이어 안 닿아도 총알이 삭제된게
  (cast `/Game/TopDown/Blueprints/BP_Player` OtherActor
    (:`CastFailed`
      (`GameplayStatics.SpawnEmitterAtLocation` "/Game/StarterContent/Particles/P_Explosion.P_Explosion" (`self.K2_GetActorLocation`))
      (`/Engine/EditorBlueprintResources/StandardMacros.IsValid` self
        (:`Is Valid`
          (`self.K2_DestroyActor`))))))

(fn `UserConstructionScript`)