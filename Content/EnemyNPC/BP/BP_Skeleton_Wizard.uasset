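; Skeleton wizard enemy that fights with fireballs and continually summons skeleton hand minions around itself.
; From BeginPlay, a looping one-second timer spawns behavior-tree-driven BP_Skeleton_Hand AI at random XY offsets near the wizard, at its height.
; Attack only plays the bow attack montage and returns its result.
; A separate SpawnSkeletonFireBall event launches the fireball actor from the mesh's bow socket, using the wizard's rotation.
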(event `SpawnSkeletonFireBall`
  (`|SpawnActorFromClass` "/Game/EnemyNPC/BP/Weapon_BP/BP_Skeleton_Fireball.BP_Skeleton_Fireball_C" (`KismetMathLibrary.MakeTransform` (`SceneComponent.GetSocketLocation` (`self.Mesh`) "SKT_Bow") (`self.K2_GetActorRotation` self)) "Undefined" "MultiplyWithRoot" null null))

(event `self.ReceiveBeginPlay`
  (`parent.ReceiveBeginPlay`)
  (`KismetSystemLibrary.K2_SetTimerDelegate` (delegate `SpawnActorAtRandomLocation`) 1.0 true))

(event `SpawnActorAtRandomLocation`
  (bind (_returnvalue_x _returnvalue_y _returnvalue_z) (`KismetMathLibrary.BreakVector` (`self.K2_GetActorLocation`)))
  (bind _output_get (set `self.EnemySpawnLocation` (`KismetMathLibrary.MakeVector` (+ _returnvalue_x (`KismetMathLibrary.RandomFloatInRange` -400.0 400.0)) (+ _returnvalue_y (`KismetMathLibrary.RandomFloatInRange` -400.0 400.0)) _returnvalue_z)))
  (`AIBlueprintHelperLibrary.SpawnAIFromClass` "/Game/EnemyNPC/BP/BP_Skeleton_Hand.BP_Skeleton_Hand_C" "/Game/EnemyNPC/AI/BT/BT_Skeleton_Hand.BT_Skeleton_Hand" _output_get (struct) false null))

(fn `Attack`
  (returns (`Animation Duration` :type "Float (double-precision)"))
  (bind _returnvalue (`self.PlayAnimMontage` "/Game/Assets/SkeletonEnemy/Animations/Anim_AttackBow_Montage.Anim_AttackBow_Montage"))
  (return _returnvalue))

(fn `UserConstructionScript`
  (`parent.UserConstructionScript`))