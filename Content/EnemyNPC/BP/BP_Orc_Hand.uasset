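; BP_Orc_Hand is an orc enemy Blueprint with a two-handed melee ground attack.
; Attack plays the two-handed attack montage and returns the value from PlayAnimMontage.
; A separate HitGround event switches TwoHandAttackCollision to the HitGround profile, then back to NoCollision after a short delay.
; Nothing in this Blueprint calls HitGround, and its BeginPlay, overlap and Tick events are empty or disabled.
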(event `HitGround`
  (`PrimitiveComponent.SetCollisionProfileName` (`self.TwoHandAttackCollision`) "HitGround" true)
  (`KismetSystemLibrary.Delay` 3.0)
  (`PrimitiveComponent.SetCollisionProfileName` (`self.TwoHandAttackCollision`) "NoCollision" true))

(fn `Attack`
  (returns (`Animation Duration` :type "Float (double-precision)"))
  (bind _returnvalue (`self.PlayAnimMontage` "/Game/Assets/Orcs_Bundle/Orc_Hunter/Animations/Combat/Anim_Orc_MeleeAttack_TwoHanded_Orc_MeleeAttack_TwoHanded_Montage.Anim_Orc_MeleeAttack_TwoHanded_Orc_MeleeAttack_TwoHanded_Montage"))
  (return _returnvalue))

(fn `UserConstructionScript`
  (`parent.UserConstructionScript`))