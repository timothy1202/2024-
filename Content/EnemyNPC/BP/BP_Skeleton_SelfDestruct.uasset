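; Skeleton enemy NPC variant whose attack ends in self-destruction.
; Attack plays the double-attack montage, immediately triggers the SelfDestruct event and returns the montage play result.
; After a short delay, SelfDestruct switches its sphere to the SelfDestruct collision profile with an overlap update, then destroys the actor.
; No damage logic appears here; the only effect before destruction is that collision change.
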(event `SelfDestruct`
  (`KismetSystemLibrary.Delay` 1.5)
  (`PrimitiveComponent.SetCollisionProfileName` (`self.SelfDestructSphere`) "SelfDestruct" true)
  (`self.K2_DestroyActor`))

(fn `Attack`
  (returns (`Animation Duration` :type "Float (double-precision)"))
  (bind _returnvalue (`self.PlayAnimMontage` "/Game/Assets/SkeletonEnemy/Animations/SK_Skeleton_AttackDouble_Montage.SK_Skeleton_AttackDouble_Montage"))
  (`self.SelfDestruct`)
  (return _returnvalue))

(fn `UserConstructionScript`
  (`parent.UserConstructionScript`))