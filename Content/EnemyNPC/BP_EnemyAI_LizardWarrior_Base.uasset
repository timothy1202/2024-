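; Base Blueprint for the Lizard Warrior enemy NPC, providing its attack action.
; Attack plays the Drake Warrior attack animation on a loop directly on the mesh, bypassing any Anim Blueprint, and returns a fixed float.
; AttackRange overlap events are empty: the logic that toggles CanAttack on ABP_DemoLizardWarrior for BP_Player is disconnected and never runs.
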(event `self.AttackRange.OnComponentBeginOverlap`
  (params (OverlappedComponent :type "PrimitiveComponent Object Reference") (OtherActor :type "Actor Object Reference") (OtherComp :type "PrimitiveComponent Object Reference") (OtherBodyIndex :type Integer) (bFromSweep :type Boolean) (SweepResult :type "HitResult Structure (by ref)"))
  ;[1 1 1] 공격
)

(event `self.AttackRange.OnComponentEndOverlap`
  (params (OverlappedComponent :type "PrimitiveComponent Object Reference") (OtherActor :type "Actor Object Reference") (OtherComp :type "PrimitiveComponent Object Reference") (OtherBodyIndex :type Integer))
  ;[1 1 1] 공격
)

(fn `Attack`
  (returns (`Animation Duration` :type "Float (double-precision)"))
  (`SkeletalMeshComponent.PlayAnimation` (`self.Mesh`) "/Game/Assets/DrakeWarrior/Animation/Anim_DrakeWarrior_attack01.Anim_DrakeWarrior_attack01" true)
  (return 1.5))

(fn `UserConstructionScript`
  (`parent.UserConstructionScript`))