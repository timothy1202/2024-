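; BP_CircleIndicator is a decal-based circle indicator that animates a repeatedly growing radius.
; BeginPlay creates a dynamic material instance from the decal and sets its initial CircleIndicator2RadiusValue parameter.
; Tick writes a counter to that parameter and increments it after a short Delay, resetting it to zero past a threshold to loop the animation.
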(event `self.ReceiveBeginPlay`
  (bind _returnvalue (`DecalComponent.CreateDynamicMaterialInstance` (`self.Decal`)))
  (bind _output_get (set `self.OpacityValue_2` _returnvalue))
  (`MaterialInstanceDynamic.SetScalarParameterValue` _output_get "CircleIndicator2RadiusValue" (`self.ParameterValue_2`)))

(event `self.ReceiveTick`
  (params (DeltaSeconds :type "Float (single-precision)"))
  (bind _parametervalue_2 (`self.ParameterValue_2`))
  (if (> (`self.ParameterValue_2`) 0.5)
    (set `self.ParameterValue_2` 0.0)
    (else
      (`KismetSystemLibrary.Delay` 0.01)
      (`MaterialInstanceDynamic.SetScalarParameterValue` (`self.OpacityValue_2`) "CircleIndicator2RadiusValue" _parametervalue_2)
      (set `self.ParameterValue_2` (+ _parametervalue_2 0.01))
      (`KismetSystemLibrary.Delay` 0.01))))

(fn `UserConstructionScript`)