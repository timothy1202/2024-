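; BP_arrow_full is an indicator actor whose decal material animates by looping its opacity mask value, likely as an arrow effect.
; BeginPlay creates a dynamic material instance from the decal and sets the initial opacityMaskValue.
; Tick raises ParameterValue by 0.01 after a short Delay and writes it to the material, resetting to zero once it exceeds one.
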(event `self.ReceiveBeginPlay`
  (bind _returnvalue (`DecalComponent.CreateDynamicMaterialInstance` (`self.Decal`)))
  (bind _output_get (set `self.OpacityValue` _returnvalue))
  (`MaterialInstanceDynamic.SetScalarParameterValue` _output_get "opacityMaskValue" (`self.Parameter Value`)))

(event `self.ReceiveTick`
  (params (DeltaSeconds :type "Float (single-precision)"))
  (bind _parameter_value (`self.Parameter Value`))
  (if (> (`self.Parameter Value`) 1.0)
    (set `self.Parameter Value` 0.0)
    (else
      (`KismetSystemLibrary.Delay` 0.01)
      (`MaterialInstanceDynamic.SetScalarParameterValue` (`self.OpacityValue`) "opacityMaskValue" _parameter_value)
      (set `self.Parameter Value` (+ _parameter_value 0.01))
      (`KismetSystemLibrary.Delay` 0.01))))

(fn `UserConstructionScript`)