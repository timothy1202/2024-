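; Circular sector indicator actor that shows an outline and an animated fill area, then destroys itself.
; BeginPlay creates dynamic materials for Circem and Area, switching outline or fill mode by scalar parameter and passing both RadianAngle.
; After a short delay, a timeline drives the fill's AreaValue, then the actor is destroyed.
; Tick also writes AreaValue from a looping counter through Delay nodes, competing with the timeline.
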(event `self.ReceiveBeginPlay`
  (`|ExecutionSequence`
    (:`then_0`
      (bind _returnvalue (`DecalComponent.CreateDynamicMaterialInstance` (`self.Circem`)))
      (bind _output_get (set `self.CircumRef` _returnvalue))
      (`MaterialInstanceDynamic.SetScalarParameterValue` _output_get "Circum1Area0" 1.0))
    (:`then_1`
      (bind _returnvalue_2 (`DecalComponent.CreateDynamicMaterialInstance` (`self.Area`)))
      (bind _output_get_2 (set `self.AreaRef` _returnvalue_2))
      (`MaterialInstanceDynamic.SetScalarParameterValue` _output_get_2 "Circum1Area0" 0.0))
    (:`then_2`
      (`MaterialInstanceDynamic.SetScalarParameterValue` (`self.AreaRef`) "RadianValue" (`self.Radian Angle`))
      (`MaterialInstanceDynamic.SetScalarParameterValue` (`self.CircumRef`) "RadianValue" (`self.Radian Angle`)))
    (:`then_3`
      (`KismetSystemLibrary.Delay` 0.1)
      (bind (_direction _areavaluealpha) (`Timeline|타임라인`)
        (:`Update`
          (`MaterialInstanceDynamic.SetScalarParameterValue` (`self.AreaRef`) "AreaValue" _areavaluealpha))
        (:`Finished`
          (`KismetSystemLibrary.Delay` 0.1)
          (`self.K2_DestroyActor`))))))

(event `self.ReceiveTick`
  (params (DeltaSeconds :type "Float (single-precision)"))
  (bind _circularsectorradian (`self.CircularSectorRadian`))
  (if (> (`self.CircularSectorRadian`) 0.5)
    (set `self.CircularSectorRadian` 0.0)
    (else
      (`KismetSystemLibrary.Delay` 0.01)
      (`MaterialInstanceDynamic.SetScalarParameterValue` (`self.AreaRef`) "AreaValue" _circularsectorradian)
      (set `self.CircularSectorRadian` (+ _circularsectorradian 0.003))
      (`KismetSystemLibrary.Delay` 0.1))))

(fn `UserConstructionScript`)