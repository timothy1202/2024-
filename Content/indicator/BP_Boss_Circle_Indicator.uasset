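; BP_Boss_Circle_Indicator is a self-destroying circular area indicator, apparently for boss attacks, built from Circem (circumference) and Area components.
; BeginPlay gives each a dynamic material, with Circum1Area0 selecting ring or area mode.
; After a short delay, a timeline animates the area's AreaValue and destroys the actor when finished.
; Tick also writes AreaValue from a delayed, looping CircumRadian counter, competing with the timeline.
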(event `self.ReceiveBeginPlay`
  (`|ExecutionSequence`
    (:`then_0`
      (bind _returnvalue (`DecalComponent.CreateDynamicMaterialInstance` (`self.Circem`)))
      (bind _output_get (set `self.CircumRef` _returnvalue))
      (`MaterialInstanceDynamic.SetScalarParameterValue` _output_get "Circum1Area0" 1.0))
    (:`then_1`
      (bind _returnvalue_2 (`DecalComponent.CreateDynamicMaterialInstance` (`self.Area`)))
      (bind _output_get_2 (set `self.AreaRef` _returnvalue_2))
      (`MaterialInstanceDynamic.SetScalarParameterValue` _output_get_2 "Circum1Area0" 0.0))
    (:`then_2`
      (`KismetSystemLibrary.Delay` 0.1)
      (bind (_direction _areavaluealpha) (`Timeline|타임라인`)
        (:`Update`
          (`MaterialInstanceDynamic.SetScalarParameterValue` (`self.AreaRef`) "AreaValue" _areavaluealpha))
        (:`Finished`
          (`self.K2_DestroyActor`))))))

(event `self.ReceiveTick`
  (params (DeltaSeconds :type "Float (single-precision)"))
  (bind _circumradian (`self.CircumRadian`))
  (if (> (`self.CircumRadian`) 0.5)
    (set `self.CircumRadian` 0.0)
    (else
      (`KismetSystemLibrary.Delay` 0.01)
      (`MaterialInstanceDynamic.SetScalarParameterValue` (`self.AreaRef`) "AreaValue" _circumradian)
      (set `self.CircumRadian` (+ _circumradian 0.01))
      (`KismetSystemLibrary.Delay` 0.1))))

(fn `UserConstructionScript`)