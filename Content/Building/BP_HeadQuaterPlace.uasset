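; BP_HeadQuaterPlace is a child building-place Blueprint for the headquarters that opens a shop UI on interaction.
; It creates the shop through BuildUIWidget during property initialization.
; Toggling interaction adds and shows the widget if it is not already shown, or closes it, registering or removing it with the player.
; Build-info updates extend the parent logic by refreshing the shop with the assigned building's tier.
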(fn `ExecuteInteract`
  (params (Toggle :type Boolean))
  (bind _build_ui_widget (`self.Build_UI_Widget`))
  (bind _build_ui_widget_2 (`self.Build_UI_Widget`))
  (if Toggle
    (if (not (`/Game/Building/Widget/BuildingInfoUI/WP_MainBuildingUI.bShow` (`self.Build_UI_Widget`)))
      (`UserWidget.AddToViewport` _build_ui_widget_2 0)
      (`/Game/TopDown/Blueprints/BP_Player.AddWidget` (`self.Player`) _build_ui_widget_2)
      (`/Game/Building/Widget/BuildingInfoUI/WP_MainBuildingUI.ShowShopUI` _build_ui_widget_2))
    (else
      (`/Game/Building/Widget/BuildingInfoUI/WP_MainBuildingUI.CloseUI` _build_ui_widget)
      (`/Game/TopDown/Blueprints/BP_Player.RemoveWidget` (`self.Player`) _build_ui_widget))))

(fn `InitProperty`
  (`parent.InitProperty`)
  (`/Game/Building/Widget/BuildingInfoUI/WP_MainBuildingUI.CreateShop` (`self.Build_UI_Widget`) self))

(fn `UpdateBuildInfoWidget`
  (`parent.UpdateBuildInfoWidget`)
  (`/Game/Building/Widget/BuildingInfoUI/WP_MainBuildingUI.UpdateShopWidget` (`self.Build_UI_Widget`) (`/Game/Building/BP_BaseBuilding.Building Tier` (`self.AssignedBuilding`))))

(fn `UserConstructionScript`
  (`parent.UserConstructionScript`))