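; BP_BuildingPlace is a build spot that previews its attached BP_BaseBuilding and a build-info widget while the player stands in its trigger box.
; On BeginPlay it caches the first attached building, offsets the widget by its footprint diagonal and fills in its build data.
; Overlap registers the spot as the player's CurrentBuildPlace.
; Tick yaws the widget with the player's camera boom and accumulates build time while constructing, resetting it otherwise.
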(event `self.ReceiveBeginPlay`
  (`SceneComponent.SetVisibility` (`self.BuildInfoWidgetComponent`) false false)
  (bind _asbp_player (cast `/Game/TopDown/Blueprints/BP_Player` (`GameplayStatics.GetPlayerCharacter` 0)))
  (set `self.Player` _asbp_player)
  (`self.InitializeBuilding`))

(event `self.Box.OnComponentBeginOverlap`
  (params (OverlappedComponent :type "PrimitiveComponent Object Reference") (OtherActor :type "Actor Object Reference") (OtherComp :type "PrimitiveComponent Object Reference") (OtherBodyIndex :type Integer) (bFromSweep :type Boolean) (SweepResult :type "HitResult Structure (by ref)"))
  (if (`ActorComponent.ComponentHasTag` OtherComp "Player")
    (`self.SetBuildingVisibility` true)
    (set `/Game/TopDown/Blueprints/BP_Player.currentBuildPlace` self (`self.Player`))))

(event `self.Box.OnComponentEndOverlap`
  (params (OverlappedComponent :type "PrimitiveComponent Object Reference") (OtherActor :type "Actor Object Reference") (OtherComp :type "PrimitiveComponent Object Reference") (OtherBodyIndex :type Integer))
  (if (`ActorComponent.ComponentHasTag` OtherComp "Player")
    (`self.SetBuildingVisibility` false)
    (set `/Game/TopDown/Blueprints/BP_Player.currentBuildPlace` null (`self.Player`))))

(event `self.ReceiveTick`
  (params (DeltaSeconds :type "Float (single-precision)"))
  (`self.BuildingWidgetLogic`)
  (`self.ConstructLogic` DeltaSeconds))

(fn `BuildingWidgetLogic`
  (bind (_returnvalue_roll _returnvalue_pitch _returnvalue_yaw) (`KismetMathLibrary.BreakRotator` (`SceneComponent.K2_GetComponentRotation` (`GraduationWork2024Character.CameraBoom` (`self.Player`)))))
  (if (`self.IsWidgetOn`)
    (`SceneComponent.K2_SetWorldRotation` (`self.WidgetRot`) (`KismetMathLibrary.MakeRotator` 0.0 0.0 _returnvalue_yaw) false false)))

(fn `ConstructLogic`
  (params (time :type "Float (double-precision)"))
  (locals (deltaTime :type "Float (double-precision)"))
  (bind _output_get (set `local.deltaTime` time))
  (if (`self.bConstructing`)
    (set `self.curBuildingTime` (+ (`self.curBuildingTime`) _output_get))
    (else
      (set `self.curBuildingTime` 0.0))))

(fn `InitializeBuilding`
  (bind _output (`|GetArrayItem` (`self.GetAttachedActors` true)))
  (bind (_build_ui_info_buildingtexture _build_ui_info_buildingname _build_ui_info_buildingdetail _build_ui_info_buildtime) (break `/Game/Building/Data/Structure/ST_Building` (`/Game/Building/BP_BaseBuilding.Build_UI_Info` (`self.AssignedBuilding`))))
  (bind (_boxextent_x _boxextent_y) (`KismetMathLibrary.BreakVector` (`BoxComponent.BoxExtent` (`/Game/Building/BP_BaseBuilding.HitCollision` (`self.AssignedBuilding`)))))
  (`/Engine/EditorBlueprintResources/StandardMacros.IsValid` _output
    (:`Is Valid`
      (bind _asbp_base_building (cast `/Game/Building/BP_BaseBuilding` _output))
      (set `self.AssignedBuilding` _asbp_base_building)
      (`SceneComponent.K2_SetRelativeLocation` (`self.BuildInfoWidgetComponent`) (`KismetMathLibrary.MakeVector` 0.0 (+ (`KismetMathLibrary.Sqrt` (+ (`KismetMathLibrary.Square` _boxextent_x) (`KismetMathLibrary.Square` _boxextent_y))) (`self.offsetValue`)) 300.0) false false)
      (`self.SetWidget`)
      (set `self.maxBuildingTIme` _build_ui_info_buildtime))))

(fn `SetBuildingVisibility`
  (params (bVisible :type Boolean))
  (`self.AssignedBuilding`
    (:`then`
      (if bVisible
        (bind _output_get (set `self.IsWidgetOn` true))
        (`SceneComponent.SetVisibility` (`self.BuildInfoWidgetComponent`) _output_get false)
        (`/Game/Building/BP_BaseBuilding.Initialize` (`self.AssignedBuilding`) false)
        (`/Game/Building/Widget/WP_BuildInfo.SetTextNeedItems` (`self.Build_UI_Widget`) (`self.Player`))
        (else
          (bind _output_get_2 (set `self.IsWidgetOn` false))
          (`SceneComponent.SetVisibility` (`self.BuildInfoWidgetComponent`) _output_get_2 false)
          (`/Game/Building/BP_BaseBuilding.HideBuilding` (`self.AssignedBuilding`)))))
    (:`else`)))

(fn `SetConstructState`
  (params (bConstruct :type Boolean))
  (bind _output_get (set `self.bConstructing` bConstruct))
  (`SceneComponent.SetVisibility` (`self.BuildInfoWidgetComponent`) _output_get false))

(fn `SetWidget`
  (bind _assignedbuilding (`self.AssignedBuilding`))
  (bind _aswp_build_info (cast `/Game/Building/Widget/WP_BuildInfo` (`WidgetComponent.GetWidget` (`self.BuildInfoWidgetComponent`))))
  (bind _output_get (set `self.Build_UI_Widget` _aswp_build_info))
  (`/Game/Building/Widget/WP_BuildInfo.Init` _output_get (`/Game/Building/BP_BaseBuilding.Build_UI_Info` _assignedbuilding) (`/Game/Building/BP_BaseBuilding.buildingMaxHealth` _assignedbuilding)))

(fn `UserConstructionScript`)