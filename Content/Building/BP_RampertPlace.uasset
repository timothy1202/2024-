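; BP_RampertPlace is a build site, apparently for ramparts, that constructs a group of assigned buildings as one unit.
; Buildings register through InitializeBuilding, and the site forwards preview visibility, start and finish smoke effects, and final initialization to each.
; It sets up progress and info widgets without a health slot, and checks the player's wood, rock and fiber against costs.
; Finishing construction disables the box collision and hides the sphere.
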(event `self.ReceiveBeginPlay`
  (`parent.ReceiveBeginPlay`)
  (`self.SetWidget`))

(fn `CheckEnableToBuild`
  (bind _player (`self.Player`))
  (bind (_buildingtexture _buildinguiname _buildinguidetail _buildingtype _building_tier _buildingname _building_maxhealth _atp _building_atkdist _building_pt_atkdmg _building_pt_atk_spd _building_pt_atkrng _building_pt_atkrngdmg _construction_time _building_skill_cooltime _building_skill_rng _building_skill_duration _construction_cost_wood1 _construction_cost_wood2 _construction_cost_wood3 _construction_cost_stone1 _construction_cost_stone2 _construction_cost_stone3 _construction_cost_stam1) (break `/Game/Building/ST_Building/ST_Building` (`self.BuildingInfo`)))
  (if (`self.IsWidgetOn`)
    (if (and (>= (`/Game/TopDown/Blueprints/BP_Player.Wood` _player) _construction_cost_wood1) (>= (`/Game/TopDown/Blueprints/BP_Player.Rock` _player) _construction_cost_stone1) (>= (`/Game/TopDown/Blueprints/BP_Player.Fiber` _player) _construction_cost_stam1))
      (set `self.bEnableToBuild` true)
      (else
        (set `self.bEnableToBuild` false)))))

(fn `InitializeBuilding`
  (params (AssignedBuilding :type "/Game/Building/BP_BaseBuilding Object Reference"))
  (`KismetArrayLibrary.Array_Add` (`self.AssignedBuildings`) AssignedBuilding))

(fn `OnFinishConstruct`
  (`PrimitiveComponent.SetCollisionEnabled` (`self.Box`) "NoCollision")
  (`SceneComponent.SetVisibility` (`self.Sphere`) false false)
  (`self.SetConstructState` false)
  (set `self.bFinishConstruct` true)
  (for _array_element (`self.AssignedBuildings`)
    (`/Game/Building/BP_BaseBuilding.Initialize` _array_element true))
  (`self.PlayUpgradeEffect` "Finish"))

(fn `PlayUpgradeEffect`
  (params (ProgressType :type String))
  (switch `string` ProgressType
    (:`Start`
      (for _array_element (`self.AssignedBuildings`)
        (`/Game/Building/BP_BaseBuilding.PlayUpgradeEffect` _array_element (* (`/Game/Building/BP_BaseBuilding.upgradeEffectSmokeScale` _array_element) 0.5) (`SceneComponent.K2_GetComponentLocation` (`/Game/Building/BP_BaseBuilding.BuildingMesh` _array_element)))))
    (:`Finish`
      (for _array_element_2 (`self.AssignedBuildings`)
        (`/Game/Building/BP_BaseBuilding.PlayUpgradeEffect` _array_element_2 (`/Game/Building/BP_BaseBuilding.upgradeEffectSmokeScale` _array_element_2) (`SceneComponent.K2_GetComponentLocation` (`/Game/Building/BP_BaseBuilding.BuildingMesh` _array_element_2)))))))

(fn `SetBuildingMesh`
  (params (bVisible :type Boolean) (MeshNum :type Integer))
  (if (not (`KismetArrayLibrary.Array_IsEmpty` (`self.AssignedBuildings`)))
    (if bVisible
      (set `self.IsWidgetOn` true)
      (for _array_element (`self.AssignedBuildings`)
        (`/Game/Building/BP_BaseBuilding.Initialize` _array_element false))
      (else
        (set `self.IsWidgetOn` false)
        (for _array_element_2 (`self.AssignedBuildings`)
          (`/Game/Building/BP_BaseBuilding.HideBuilding` _array_element_2))))))

(fn `SetConstructProressBarVisibility`
  (params (bVisibility :type Boolean))
  (`SceneComponent.SetVisibility` (`self.BuildProgressWidget`) bVisibility false))

(fn `SetWidget`
  (bind _buildinginfo (`self.BuildingInfo`))
  (bind _aswp_build_progress_bar (cast `/Game/Building/Widget/WP_BuildProgressBar` (`WidgetComponent.GetWidget` (`self.BuildProgressWidget`))))
  (`/Game/Building/Widget/WP_BuildProgressBar.Init` _aswp_build_progress_bar self)
  (bind _aswp_build_info (cast `/Game/Building/Widget/WP_BuildInfo` (`WidgetComponent.GetWidget` (`self.BuildInfoWidgetComponent`))))
  (bind _output_get (set `self.Build_UI_Widget` _aswp_build_info))
  (`/Game/Building/Widget/WP_BuildInfo.DestroyHealthSlot` _output_get)
  (`/Game/Building/Widget/WP_BuildInfo.Init` _output_get _buildinginfo 0.0)
  (set `self.maxBuildingTIme` (`.Construction_Time_60_794AE2A74F885E75B0487E957855273F` (break `/Game/Building/ST_Building/ST_Building` _buildinginfo))))

(fn `UserConstructionScript`
  (`parent.UserConstructionScript`))