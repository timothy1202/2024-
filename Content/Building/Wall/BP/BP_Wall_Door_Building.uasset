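; BP_Wall_Door_Building is a door building for walls, built on a parent that supplies property setup, initialization and construction script.
; On BeginPlay it sets up properties, uses the building skeletal mesh as its active mesh and hides the build progress widget.
; When attached to a parent actor, it disables hit collision, hides mesh and health widget, and applies the translucent building collision profile.
; Otherwise it runs the normal initialization.
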(event `self.ReceiveBeginPlay`
  (`self.InitProperties`)
  (set `self.MyMesh` (`self.BuildingSkMesh`))
  (`SceneComponent.SetVisibility` (`self.BuildProgressWidget`) false false)
  (`/Engine/EditorBlueprintResources/StandardMacros.IsValid` (`self.GetAttachParentActor`)
    (:`Is Valid`
      (`PrimitiveComponent.SetCollisionEnabled` (`self.HitCollision`) "NoCollision")
      (`SceneComponent.SetVisibility` (`self.MyMesh`) false false)
      (`PrimitiveComponent.SetCollisionProfileName` (`self.MyMesh`) (`self.TranslucentBuilding`) true)
      (`SceneComponent.SetVisibility` (`self.HealthWidgetComponent`) false false))
    (:`Is Not Valid`
      (`self.Initialize` true))))

(fn `UserConstructionScript`
  (`parent.UserConstructionScript`))