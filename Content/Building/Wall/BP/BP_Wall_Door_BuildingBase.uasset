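; Castle gate building that opens for player allies, tracking overlapping "PlayerAllies" components in EnterCollision to drive the Open animation flag.
; When attached to a build place, it registers there and starts hidden with collision disabled and a translucent mesh profile; otherwise it initializes directly.
; Spawn and destroy overrides toggle EnterCollision after calling the parent.
; SetEnemyBlock and SetBuildProgressWidget are deliberately empty overrides, marked do-not-touch.
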(event `self.OnSpawned`
  (bind _returnvalue (`self.GetAttachParentActor`))
  ;[0.05098 0.05098 0.05098 1 30] 성문용 초기화 로직
  (set `self.MyMesh` (`self.BuildingSkMesh`))
  (`/Engine/EditorBlueprintResources/StandardMacros.IsValid` _returnvalue
    (:`Is Valid`
      (bind _asbp_building_place_base (cast `/Game/Building/BP_BuildingPlaceBase` _returnvalue))
      (`/Game/Building/BP_BuildingPlaceBase.InitializeBuildPlace` _asbp_building_place_base self)
      (`PrimitiveComponent.SetCollisionEnabled` (`self.HitCollision`) "NoCollision")
      (`PrimitiveComponent.SetCollisionEnabled` (`self.EnemyBlock`) "NoCollision")
      (`PrimitiveComponent.SetCollisionEnabled` (`self.EnterCollision`) "NoCollision")
      (`SceneComponent.SetVisibility` (`self.MyMesh`) false false)
      (`SceneComponent.SetVisibility` (`self.HealthWidgetComponent`) false false)
      (`PrimitiveComponent.SetCollisionProfileName` (`self.MyMesh`) (`self.TranslucentBuilding`) true))
    (:`Is Not Valid`
      (`self.Initialize` true))))

(event `self.EnterCollision.OnComponentBeginOverlap`
  (params (OverlappedComponent :type "PrimitiveComponent Object Reference") (OtherActor :type "Actor Object Reference") (OtherComp :type "PrimitiveComponent Object Reference") (OtherBodyIndex :type Integer) (bFromSweep :type Boolean) (SweepResult :type "HitResult Structure (by ref)"))
  ;[0.05098 0.05098 0.05098] 성문 애니메이션 로직
  (if (`ActorComponent.ComponentHasTag` OtherComp "PlayerAllies")
    (if (`KismetArrayLibrary.Array_IsEmpty` (`self.OverlappingComps`))
      (`|ExecutionSequence`
        (:`then_0`
          (`KismetArrayLibrary.Array_AddUnique` (`self.OverlappingComps`) OtherComp :!label _label))
        (:`then_1`
          (set `self.bOpen` true)))
      (else
        (goto _label)))))

(event `self.EnterCollision.OnComponentEndOverlap`
  (params (OverlappedComponent :type "PrimitiveComponent Object Reference") (OtherActor :type "Actor Object Reference") (OtherComp :type "PrimitiveComponent Object Reference") (OtherBodyIndex :type Integer))
  (bind _overlappingcomps (`self.OverlappingComps`))
  ;[0.05098 0.05098 0.05098] 성문 애니메이션 로직
  (if (`ActorComponent.ComponentHasTag` OtherComp "PlayerAllies")
    (`KismetArrayLibrary.Array_RemoveItem` _overlappingcomps OtherComp)
    (if (`KismetArrayLibrary.Array_IsEmpty` _overlappingcomps)
      (set `self.bOpen` false))))

(fn `On Spawn`
  (`parent.On Spawn`)
  (`PrimitiveComponent.SetCollisionEnabled` (`self.EnterCollision`) (`self.HitCollisionType`)))

(fn `OnDestroy`
  (`parent.OnDestroy`)
  (`PrimitiveComponent.SetCollisionEnabled` (`self.EnterCollision`) "NoCollision"))

(fn `SetBuildProgressWidget`)

(fn `SetEnemyBlock`)

(fn `UserConstructionScript`
  (`parent.UserConstructionScript`))