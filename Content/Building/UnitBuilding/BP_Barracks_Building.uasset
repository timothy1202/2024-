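; Barracks building that spawns a squad of units on construction and replaces them as they die.
; SpawnUnit lays units out in two offset rows from SpawnPoint, passing each a data table row and the building, and records the spots.
; NPCDestroyed queues each death with the next saved spot in round-robin order.
; SpawnNewNPC drains that queue recursively, one respawn per BuildingSkillCoolTime delay, with a flag preventing parallel runs.
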(event `self.SpawnUnit`
  (bind _returnvalue (`SceneComponent.K2_GetComponentToWorld` (`self.SpawnPoint`)))
  (bind _returnvalue_2 (`SceneComponent.K2_GetComponentToWorld` (`self.SpawnPoint`)))
  (bind _returnvalue_3 (+ (.x (.location _returnvalue)) 100.0))
  ;[1 1 1] 건설시 첫 스폰
  (for _index (range 1 (+ (`self.Last Index`) 1))
    (if (< _index 5)
      (bind _returnvalue_4 (+ (* (+ _index 1) 100) (.y (.location _returnvalue_2))))
      (`KismetArrayLibrary.Array_Add` (`self.SpawnLocations`) (`KismetMathLibrary.MakeVector` (.x (.location _returnvalue_2)) _returnvalue_4 (.z (.location _returnvalue_2))))
      (bind _returnvalue_5 (`|SpawnActorFromClass` (`self.UnitClass`) (`KismetMathLibrary.MakeTransform` (`KismetMathLibrary.MakeVector` (.x (.location _returnvalue_2)) _returnvalue_4 (.z (.location _returnvalue_2)))) "Undefined" "MultiplyWithRoot" null (`self.Spawn  DT Row Name`) self null))
      (`KismetArrayLibrary.Array_Add` (`self.Units`) _returnvalue_5)
      (else
        (bind _returnvalue_6 (+ (* (- _index 3) 100) (.y (.location _returnvalue))))
        (`KismetArrayLibrary.Array_Add` (`self.SpawnLocations`) (`KismetMathLibrary.MakeVector` _returnvalue_3 _returnvalue_6 (.z (.location _returnvalue))))
        (bind _returnvalue_7 (`|SpawnActorFromClass` (`self.UnitClass`) (`KismetMathLibrary.MakeTransform` (`KismetMathLibrary.MakeVector` _returnvalue_3 _returnvalue_6 (.z (.location _returnvalue)))) "Undefined" "MultiplyWithRoot" null (`self.Spawn  DT Row Name`) self null))
        (`KismetArrayLibrary.Array_Add` (`self.Units`) _returnvalue_7)))))

(event `self.NPCDestroyed`
  (params (`Destroyed NPC` :type "/Game/NPC/FriendlyNPC/BP/BP_MyFriendlyBase Object Reference"))
  ;[1 1 1] 코멘트
  (`parent.NPCDestroyed` `Destroyed NPC`)
  (if (> (`self.Location Index`) (`self.Last Index`))
    (set `self.Location Index` 0))
  (`KismetArrayLibrary.Array_Add` (`self.DeadLocations`) (`|GetArrayItem` (`self.SpawnLocations`) (`self.Location Index`)))
  (`KismetArrayLibrary.Array_Add` (`self.DeadNPCs`) `Destroyed NPC`)
  (set `self.Location Index` (+ (`self.Location Index`) 1))
  (if (not (`self.bIsRespawningInProgress`))
    (`self.SpawnNewNPC`)))

(event `self.SpawnNewNPC`
  ;[1 1 1] 코멘트
  (set `self.bIsRespawningInProgress` true)
  (if (`KismetArrayLibrary.Array_IsNotEmpty` (`self.DeadNPCs`))
    (`KismetSystemLibrary.Delay` (`self.Building Skill Cool Time`))
    (`KismetArrayLibrary.Array_Remove` (`self.DeadNPCs`))
    (bind _returnvalue (`|SpawnActorFromClass` (`self.UnitClass`) (`KismetMathLibrary.MakeTransform` (`|GetArrayItem` (`self.DeadLocations`))) "Undefined" "MultiplyWithRoot" null (`self.Spawn  DT Row Name`) self null))
    (`KismetArrayLibrary.Array_Add` (`self.Units`) _returnvalue)
    (`KismetArrayLibrary.Array_Remove` (`self.DeadLocations`))
    (`self.SpawnNewNPC`)
    (else
      (set `self.bIsRespawningInProgress` false))))

(fn `UserConstructionScript`
  (`parent.UserConstructionScript`))