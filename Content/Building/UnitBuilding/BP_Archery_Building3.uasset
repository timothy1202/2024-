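; Archery building, tier 3 by its name, that spawns a squad of fire archers and respawns them after death.
; FirstSpawnUnit lays units out in a grid beside SpawnPoint, filling rows of four, and records them in SpawnLocations and LiveNPCs.
; SpawnNewNPC works through the dead-unit queue by calling itself, respawning one at each saved death location after the building skill cooldown.
; Respawned units are not added back to LiveNPCs here.
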(event `self.First Spawn Unit`
  (bind _returnvalue (`SceneComponent.K2_GetComponentToWorld` (`self.SpawnPoint`)))
  (bind _returnvalue_2 (`SceneComponent.K2_GetComponentToWorld` (`self.SpawnPoint`)))
  (bind _returnvalue_3 (`SceneComponent.K2_GetComponentToWorld` (`self.SpawnPoint`)))
  (bind _returnvalue_4 (+ (.x (.location _returnvalue_2)) 100.0))
  (bind _returnvalue_5 (+ (.x (.location _returnvalue_3)) 200.0))
  ;[1 1 1] 불궁수 소환
  (for _index (range 1 (+ (`self.Last Index`) 1))
    (if (< _index 5)
      (bind _returnvalue_6 (+ (* (+ _index 1) 100) (.y (.location _returnvalue))))
      (`KismetArrayLibrary.Array_Add` (`self.SpawnLocations`) (`KismetMathLibrary.MakeVector` (.x (.location _returnvalue)) _returnvalue_6 (.z (.location _returnvalue))))
      (bind _returnvalue_7 (`|SpawnActorFromClass` (`self.SpawnedClass`) (`KismetMathLibrary.MakeTransform` (`KismetMathLibrary.MakeVector` (.x (.location _returnvalue)) _returnvalue_6 (.z (.location _returnvalue)))) "Undefined" "MultiplyWithRoot" null null))
      (`KismetArrayLibrary.Array_Add` (`self.LiveNPCs`) _returnvalue_7)
      (elif (< _index 9)
        (bind _returnvalue_8 (+ (* (- _index 3) 100) (.y (.location _returnvalue_2))))
        (`KismetArrayLibrary.Array_Add` (`self.SpawnLocations`) (`KismetMathLibrary.MakeVector` _returnvalue_4 _returnvalue_8 (.z (.location _returnvalue_2))))
        (bind _returnvalue_9 (`|SpawnActorFromClass` (`self.SpawnedClass`) (`KismetMathLibrary.MakeTransform` (`KismetMathLibrary.MakeVector` _returnvalue_4 _returnvalue_8 (.z (.location _returnvalue_2)))) "Undefined" "MultiplyWithRoot" null null))
        (`KismetArrayLibrary.Array_Add` (`self.LiveNPCs`) _returnvalue_9)
        (else
          (bind _returnvalue_10 (+ (* (- _index 7) 100) (.y (.location _returnvalue_3))))
          (`KismetArrayLibrary.Array_Add` (`self.SpawnLocations`) (`KismetMathLibrary.MakeVector` _returnvalue_5 _returnvalue_10 (.z (.location _returnvalue_3))))
          (bind _returnvalue_11 (`|SpawnActorFromClass` (`self.SpawnedClass`) (`KismetMathLibrary.MakeTransform` (`KismetMathLibrary.MakeVector` _returnvalue_5 _returnvalue_10 (.z (.location _returnvalue_3)))) "Undefined" "MultiplyWithRoot" null null))
          (`KismetArrayLibrary.Array_Add` (`self.LiveNPCs`) _returnvalue_11))))))

(event `self.SpawnNewNPC`
  ;[1 1 1] 코멘트
  (set `self.bIsRespawningInProgress` true)
  (if (`KismetArrayLibrary.Array_IsNotEmpty` (`self.DeadNPCs`))
    (`KismetSystemLibrary.Delay` (`self.Building Skill Cool Time`))
    (`KismetArrayLibrary.Array_Remove` (`self.DeadNPCs`))
    (`|SpawnActorFromClass` (`self.SpawnedClass`) (`KismetMathLibrary.MakeTransform` (`|GetArrayItem` (`self.DeadLocations`))) "Undefined" "MultiplyWithRoot" null null)
    (`KismetArrayLibrary.Array_Remove` (`self.DeadLocations`))
    (`self.SpawnNewNPC`)
    (else
      (set `self.bIsRespawningInProgress` false))))

(fn `UserConstructionScript`
  (`parent.UserConstructionScript`))