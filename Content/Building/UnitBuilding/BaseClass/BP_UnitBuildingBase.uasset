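; BP_UnitBuildingBase is a building base class that produces NPC units when built and destroys them when removed.
; On initialization, it spawns units in a grid oriented to SpawnPoint, saving each location and passing itself and a data table row name.
; NPCDestroyed queues a respawn at the next saved location by cycling index, not the dead unit's own spot.
; A self-recalling event drains that queue, respawning one unit per BuildingSkillCoolTime delay.
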(event `self.Initialize`
  (params (bBuild :type Boolean))
  (`parent.Initialize` bBuild)
  (if bBuild
    (`self.SpawnUnit`)))

(event `self.OnRemove`
  (`self.DestroyAllNPC`)
  (`parent.OnRemove`))

(event `SpawnUnit`
  ;[1 1 1] 건설 시 스폰
  (for _index (range (`self.Production Unit Count`))
    (bind _output_get (set `self.ColumnCount` (mod _index (`self.MaxColumnUnitNum`))))
    (if (== _output_get 0)
      (`/Engine/EditorBlueprintResources/StandardMacros.IncrementInt` (`self.RowCount`)
        (:`  `
          _)))
    (`self.Spawn` (`self.ColumnCount`))))

(event `NPCDestroyed`
  (params (`Destroyed NPC` :type "/Game/NPC/FriendlyNPC/BP/BP_MyFriendlyBase Object Reference"))
  ;[1 1 1] NPC가 죽을 시 리스폰 이벤트 트리거
  (`KismetArrayLibrary.Array_RemoveItem` (`self.Units`) `Destroyed NPC`)
  (if (> (`self.Location Index`) (`self.Production Unit Count`))
    (set `self.Location Index` 0))
  (`KismetArrayLibrary.Array_Add` (`self.DeadLocations`) (`|GetArrayItem` (`self.SpawnLocations`) (`self.Location Index`)))
  (`KismetArrayLibrary.Array_Add` (`self.DeadNPCs`))
  (set `self.Location Index` (+ (`self.Location Index`) 1))
  (if (not (`self.bIsRespawningInProgress`))
    (`self.SpawnNPCOnDie`)))

(event `SpawnNPCOnDie`
  ;[1 1 1] 리스폰 이벤트
  (set `self.bIsRespawningInProgress` true)
  (if (`KismetArrayLibrary.Array_IsNotEmpty` (`self.DeadNPCs`))
    (`KismetSystemLibrary.Delay` (`self.Building Skill Cool Time`))
    (`KismetArrayLibrary.Array_Remove` (`self.DeadNPCs`))
    (bind _returnvalue (`|SpawnActorFromClass` (`self.UnitClass`) (`KismetMathLibrary.MakeTransform` (`|GetArrayItem` (`self.DeadLocations`))) "Undefined" "MultiplyWithRoot" null (`self.Spawn  DT Row Name`) self null))
    (`KismetArrayLibrary.Array_Add` (`self.Units`) _returnvalue)
    (`KismetArrayLibrary.Array_Remove` (`self.DeadLocations`))
    (`self.SpawnNPCOnDie`)
    (else
      (set `self.bIsRespawningInProgress` false))))

(fn `DestroyAllNPC`
  (for _array_element (`self.Units`)
    (`self.K2_DestroyActor` _array_element)))

(fn `Spawn`
  (params (index :type Integer))
  (locals (MyIndex :type Integer))
  (bind (_returnvalue_location _returnvalue_rotation) (`KismetMathLibrary.BreakTransform` (`SceneComponent.K2_GetComponentToWorld` (`self.SpawnPoint`))))
  (bind _returnvalue (+ (* (`SceneComponent.GetForwardVector` (`self.SpawnPoint`)) (* (`self.RowCount`) 150)) (* (`SceneComponent.GetRightVector` (`self.SpawnPoint`)) (* (`local.MyIndex`) 100)) _returnvalue_location))
  ;[0.05098 0.05098 0.05098] 건물 회전에 따라 NPC생성
  (set `local.MyIndex` index)
  (`KismetArrayLibrary.Array_Add` (`self.SpawnLocations`) _returnvalue)
  (bind _returnvalue_2 (`|SpawnActorFromClass` (`self.UnitClass`) (`KismetMathLibrary.MakeTransform` _returnvalue _returnvalue_rotation) "AdjustIfPossibleButAlwaysSpawn" "MultiplyWithRoot" null (`self.Spawn  DT Row Name`) self null))
  (`KismetArrayLibrary.Array_Add` (`self.Units`) _returnvalue_2))

(fn `UserConstructionScript`
  (`parent.UserConstructionScript`))