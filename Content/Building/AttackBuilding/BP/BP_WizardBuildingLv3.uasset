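; BP_WizardBuildingLv3 is the level 3 wizard attack building, which fires thunder projectiles at a target.
; Its Spawn Missile function checks that the target is valid, then spawns BP_Thunder_Base and BP_Thunder_lining at the Sphere component, rotated toward the target.
; Both actors receive the target, but only BP_Thunder_lining is given the building's attack damage.
; The construction script just calls the parent's.
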(fn `Spawn Missile`
  (params (WhatsTarget :type "Actor Object Reference"))
  (locals (`Whats Target` :type "Actor Object Reference"))
  (bind _whats_target (`local.Whats Target`))
  (bind _returnvalue (`SceneComponent.K2_GetComponentLocation` (`self.Sphere`)))
  (bind _returnvalue_2 (`SceneComponent.K2_GetComponentLocation` (`self.Sphere`)))
  (set `local.Whats Target` WhatsTarget)
  (`/Engine/EditorBlueprintResources/StandardMacros.IsValid` _whats_target
    (:`Is Valid`
      (`|SpawnActorFromClass` "/Game/Building/AttackBuilding/BP/Weapons/BP_Thunder_Base.BP_Thunder_Base_C" (`KismetMathLibrary.MakeTransform` _returnvalue_2 (`KismetMathLibrary.FindLookAtRotation` _returnvalue_2 (`self.K2_GetActorLocation` _whats_target))) "Undefined" "MultiplyWithRoot" null (`local.Whats Target`) 10.0 null)
      (`|SpawnActorFromClass` "/Game/Building/AttackBuilding/BP/Weapons/BP_Thunder_lining.BP_Thunder_lining_C" (`KismetMathLibrary.MakeTransform` _returnvalue (`KismetMathLibrary.FindLookAtRotation` _returnvalue (`self.K2_GetActorLocation` (`local.Whats Target`)))) "Undefined" "MultiplyWithRoot" null (`local.Whats Target`) (`self.Building PT Atk Dmg`) null))))

(fn `UserConstructionScript`
  (`parent.UserConstructionScript`))