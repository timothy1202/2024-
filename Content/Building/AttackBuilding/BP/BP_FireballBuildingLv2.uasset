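; Level 2 fireball attack building that periodically shoots scaled-down fireballs at its current target.
; StartLogic sizes the range sphere and starts a looping timer from attack speed, which StopLogic clears.
; Each tick with a valid Target spawns a fireball aimed from the Sphere component, passing damage values and the target.
; FindHighestHpTarget returns the overlapping enemy with the most current health, though this file never calls it.
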(event `self.StartLogic`
  (`SphereComponent.SetSphereRadius` (`self.AttackRangeCol`) (`self.Building Atk Dist`) true)
  (bind _returnvalue (`KismetSystemLibrary.K2_SetTimerDelegate` (delegate `AttackFireBall`) (/ 1.0 (`self.Building PT Atk Spd`)) true))
  (set `self.FireBallHandle` _returnvalue))

(event `AttackFireBall`
  (bind _target (`self.Target`))
  (bind _returnvalue (`SceneComponent.K2_GetComponentLocation` (`self.Sphere`)))
  ;[1 1 1] 파이어볼 스폰
  (`/Engine/EditorBlueprintResources/StandardMacros.IsValid` _target
    (:`Is Valid`
      (bind _returnvalue_2 (`|SpawnActorFromClass` "/Game/Building/AttackBuilding/BP/Weapons/BP_Firball_Base.BP_Firball_Base_C" (`KismetMathLibrary.MakeTransform` _returnvalue (`KismetMathLibrary.FindLookAtRotation` _returnvalue (`self.K2_GetActorLocation` _target)) (0.25 0.25 0.25)) "Undefined" "MultiplyWithRoot" null null (`self.Building PT Atk Dmg`) null))
      (set `/Game/Building/AttackBuilding/BP/Weapons/BP_Firball_Base.PTDamage` (`self.Building PT Atk Rng Dmg`) _returnvalue_2)
      (`/Game/Building/AttackBuilding/BP/Weapons/BP_Firball_Base.SetFireBallTarget` _returnvalue_2 (`self.Target`)))))

(fn `Find Highest Hp Target`
  (returns (`Highest Hp Enemy` :type "Actor Object Reference"))
  (locals (`Local Hp` :type "Array of Float (double-precision)"))
  (bind _overlappingactors (`PrimitiveComponent.GetOverlappingActors` (`self.AttackRangeCol`) "/Game/NPC/EnemeyNPC/BP/BP_MyEnemyBase.BP_MyEnemyBase_C"))
  (switch `int` (`KismetArrayLibrary.Array_Length` _overlappingactors)
    (:`Default`
      (for _array_element _overlappingactors
        (bind _asenemy_base (cast `EnemyBase` _array_element))
        (`KismetArrayLibrary.Array_Add` (`local.Local Hp`) (`EnemyBase.cur_health` _asenemy_base)))
      (return (`|GetArrayItem` _overlappingactors (`KismetMathLibrary.MaxOfFloatArray` (`local.Local Hp`)))))
    (:`0`
      (return null))
    (:`1`
      (return (`|GetArrayItem` _overlappingactors)))))

(fn `StopLogic`
  (`KismetSystemLibrary.K2_ClearAndInvalidateTimerHandle` (`self.FireBallHandle`)))

(fn `UserConstructionScript`
  (`parent.UserConstructionScript`))