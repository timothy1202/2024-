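; BP_SlowBuildingLv3 is the level 3 slow attack building, which periodically fires slow balls at the enemy with the highest health.
; Until collapsed, Tick runs the distance check, reselects the highest-HP target and draws a debug sphere on it.
; StartLogic extends the parent with a looping timer that spawns a BP_SlowBall_Base from the Sphere component, aimed at the target, with its trail FX activated.
; StopLogic clears that timer.
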(event `self.StartLogic`
  (`parent.StartLogic`)
  (bind _returnvalue (`KismetSystemLibrary.K2_SetTimerDelegate` (delegate `Fire Slow Ball`) 5.0 true))
  (set `self.SlowSkillHandle` _returnvalue))

(event `Fire Slow Ball`
  (bind _target (`self.Target`))
  (bind _returnvalue (`SceneComponent.K2_GetComponentLocation` (`self.Sphere`)))
  ;[1 1 1] 슬로우 스킬
  (`/Engine/EditorBlueprintResources/StandardMacros.IsValid` _target
    (:`Is Valid`
      (bind _returnvalue_2 (`|SpawnActorFromClass` "/Game/Building/AttackBuilding/BP/Weapons/BP_SlowBall_Base.BP_SlowBall_Base_C" (`KismetMathLibrary.MakeTransform` _returnvalue (`KismetMathLibrary.FindLookAtRotation` _returnvalue (`self.K2_GetActorLocation` _target)) (0.25 0.25 0.25)) "Undefined" "MultiplyWithRoot" null _target 10.0 null))
      (`ActorComponent.Activate` (`/Game/Building/AttackBuilding/BP/Weapons/BP_HomingMissile_Base.FX_Weapon_trail` _returnvalue_2) false))))

(event `self.ReceiveTick`
  (params (DeltaSeconds :type "Float (single-precision)"))
  ;[1 1 1] 가장 체력 높은 적 설정
  (if (not (`self.bCollapse`))
    (`self.CheckDistance`)
    (bind _output_get (set `self.Target` (`self.Find Highest Hp Target`)))
    (`/Engine/EditorBlueprintResources/StandardMacros.IsValid` _output_get
      (:`Is Valid`
        (`KismetSystemLibrary.DrawDebugSphere` (`self.K2_GetActorLocation` _output_get))))))

(fn `StopLogic`
  (`parent.StopLogic`)
  (`KismetSystemLibrary.K2_ClearAndInvalidateTimerHandle` (`self.SlowSkillHandle`)))

(fn `UserConstructionScript`
  (`parent.UserConstructionScript`))