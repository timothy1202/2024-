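; Level 3 speed tower building that periodically casts an area skill, which the comments label as a slow skill.
; StartLogic runs parent logic, spawns BP_SpeedSkill at once, then starts a looping timer that respawns it every BuildingSkillCoolTime.
; Each spawn uses only the building's X and Y location, and its trailing duration Delay triggers nothing further.
; StopLogic runs parent logic and clears the timer.
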(event `self.StartLogic`
  (`parent.StartLogic`)
  (`self.Spawn Speed Range`) ; 첫 재생
  (bind _returnvalue (`KismetSystemLibrary.K2_SetTimerDelegate` (delegate `Spawn Speed Range`) (`self.Building Skill Cool Time`) true))
  (set `self.Speed Tower Handle` _returnvalue))

(event `Spawn Speed Range`
  (bind _returnvalue (`self.GetTransform` self))
  ;[1 1 1] 슬로우 스킬
  (`|SpawnActorFromClass` "/Game/Building/AttackBuilding/BP/Skills/BP_SpeedSkill.BP_SpeedSkill_C" (`KismetMathLibrary.MakeTransform` (`KismetMathLibrary.MakeVector` (.x (.location _returnvalue)) (.y (.location _returnvalue)))) "AlwaysSpawn" "MultiplyWithRoot" null null)
  (`KismetSystemLibrary.Delay` (`self.Building Skill Duration`)) ; 시전 종료 후 쿨타임 재생
)

(fn `StopLogic`
  (`parent.StopLogic`)
  (`KismetSystemLibrary.K2_ClearAndInvalidateTimerHandle` (`self.Speed Tower Handle`)))

(fn `UserConstructionScript`
  (`parent.UserConstructionScript`))