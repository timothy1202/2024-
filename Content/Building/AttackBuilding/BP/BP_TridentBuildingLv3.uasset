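; Level 3 Trident attack building that fires homing missiles at the weakest enemies in its range.
; Each Tick, unless collapsed, it runs a distance check, stores up to three lowest-health enemies overlapping its range collider, and draws debug spheres on them.
; StartLogic begins a looping one-second timer that spawns a missile for each stored target.
; Target selection repeatedly extracts the minimum health, returning all overlaps when three or fewer.
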(event `self.StartLogic`
  (`KismetSystemLibrary.K2_SetTimerDelegate` (delegate `AttackMinHp`) 1.0 true))

(event `AttackMinHp`
  ;[1 1 1] 호밍 미사일 스폰
  (for _array_element (`self.Targets`)
    (`self.Spawn Missile` _array_element)))

(event `self.ReceiveTick`
  (params (DeltaSeconds :type "Float (single-precision)"))
  ;[1 1 1] 가장 체력 낮은 적들 설정
  (if (not (`self.bCollapse`))
    (`self.CheckDistance`)
    (bind _output_get (set `self.Targets` (`self.Find Lowest Hp Target`)))
    (for _index (range (+ (`KismetArrayLibrary.Array_LastIndex` _output_get) 1))
      (if (`KismetArrayLibrary.Array_IsValidIndex` _output_get _index)
        (bind _output (`|GetArrayItem` _output_get _index))
        (`/Engine/EditorBlueprintResources/StandardMacros.IsValid` _output
          (:`Is Valid`
            (bind _asbp_enemy_ai_base (cast `/Game/NPC/EnemeyNPC/BP/BP_EnemyAI_Base` _output))
            (`KismetSystemLibrary.DrawDebugSphere` (`self.K2_GetActorLocation` _asbp_enemy_ai_base))))
        (else
          (break))))))

(fn `Find Lowest Hp Target`
  (returns (`Lowest Hp Enemies` :type "Array of Actor Object Reference"))
  (locals (`Local Hp` :type "Array of Float (double-precision)") (`lowest Actors` :type "Array of Actor Object Reference") (TmpActors :type "Array of Actor Object Reference"))
  (bind _local_hp (`local.Local Hp`))
  (bind _tmpactors (`local.TmpActors`))
  (bind _overlappingactors (`PrimitiveComponent.GetOverlappingActors` (`self.AttackRangeCol`) "/Game/NPC/EnemeyNPC/BP/BP_EnemyAI_Base.BP_EnemyAI_Base_C"))
  (bind _indexofminvalue (`KismetMathLibrary.MinOfFloatArray` _local_hp))
  (switch `int` (`KismetArrayLibrary.Array_Length` _overlappingactors)
    (:`Default`
      (bind _output_get (set `local.TmpActors` _overlappingactors))
      (for _array_element _output_get
        (bind _asbp_enemy_ai_base (cast `/Game/NPC/EnemeyNPC/BP/BP_EnemyAI_Base` _array_element))
        (`KismetArrayLibrary.Array_Add` (`local.Local Hp`) (`/Game/NPC/EnemeyNPC/BP/BP_EnemyAI_Base.curHealth` _asbp_enemy_ai_base)))
      (for _ (range 3)
        (`KismetArrayLibrary.Array_Add` (`local.lowest Actors`) (`|GetArrayItem` _tmpactors _indexofminvalue))
        (`KismetArrayLibrary.Array_Remove` _tmpactors _indexofminvalue)
        (`KismetArrayLibrary.Array_Remove` _local_hp _indexofminvalue))
      (return (`local.lowest Actors`)))
    (:`0`
      (return))
    (:`1`
      (return _overlappingactors))
    (:`2`
      (return _overlappingactors))
    (:`3`
      (return _overlappingactors))))

(fn `UserConstructionScript`
  (`parent.UserConstructionScript`))