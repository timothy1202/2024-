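; Base long-range attack building that automatically fires homing projectiles at the nearest enemy in range.
; Every Tick selects the closest BP_EnemyAI_Base overlapping AttackRangeCol and marks it with a debug sphere.
; StartLogic starts a looping timer that spawns the configured projectile class at the Sphere component, facing the current target.
; Spawned BP_HomingArrow_Base projectiles receive the enemy as target and its capsule as homing component.
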(event `self.StartLogic`
  (`KismetSystemLibrary.K2_SetTimerDelegate` (delegate `Attack`) 1.0 true))

(event `Attack`
  ;[1 1 1] 호밍 미사일 스폰
  (`self.Spawn Missile` (`self.Target`)))

(event `self.ReceiveTick`
  (params (DeltaSeconds :type "Float (single-precision)"))
  ;[1 1 1] 가장 가까운 적 설정
  (`parent.ReceiveTick` 0.0)
  (bind _output_get (set `self.Target` (`self.Find Closest Target`)))
  (`/Engine/EditorBlueprintResources/StandardMacros.IsValid` _output_get
    (:`Is Valid`
      (`KismetSystemLibrary.DrawDebugSphere` (`self.K2_GetActorLocation` _output_get)))))

(fn `Find Closest Target`
  (returns (`Closest Enemy` :type "Actor Object Reference"))
  (locals (local_Distances :type "Array of Float (double-precision)"))
  (bind _overlappingactors (`PrimitiveComponent.GetOverlappingActors` (`self.AttackRangeCol`) "/Game/NPC/EnemeyNPC/BP/BP_EnemyAI_Base.BP_EnemyAI_Base_C"))
  (switch `int` (`KismetArrayLibrary.Array_Length` _overlappingactors)
    (:`Default`
      (for _array_element _overlappingactors
        (`KismetArrayLibrary.Array_Add` (`local.local_Distances`) (`KismetMathLibrary.Vector_Distance` (`self.K2_GetActorLocation` _array_element) (`self.K2_GetActorLocation`))))
      (return (`|GetArrayItem` _overlappingactors (`KismetMathLibrary.MinOfFloatArray` (`local.local_Distances`)))))
    (:`0`
      (return null))
    (:`1`
      (return (`|GetArrayItem` _overlappingactors)))))

(fn `Spawn Missile`
  (params (WhatsTarget :type "Actor Object Reference"))
  (locals (`Whats Target` :type "Actor Object Reference"))
  (bind _whats_target (`local.Whats Target`))
  (bind _returnvalue (`SceneComponent.K2_GetComponentLocation` (`self.Sphere`)))
  (set `local.Whats Target` WhatsTarget)
  (`/Engine/EditorBlueprintResources/StandardMacros.IsValid` _whats_target
    (:`Is Valid`
      (bind _asbp_enemy_ai_base (cast `/Game/NPC/EnemeyNPC/BP/BP_EnemyAI_Base` (`local.Whats Target`)))
      (bind _returnvalue_2 (`|SpawnActorFromClass` (`self.SpawnedActor`) (`KismetMathLibrary.MakeTransform` _returnvalue (`KismetMathLibrary.FindLookAtRotation` _returnvalue (`self.K2_GetActorLocation` _whats_target)) (0.25 0.25 0.25)) "Undefined" "MultiplyWithRoot" null null))
      (bind _asbp_homing_arrow_base (cast `/Game/Building/AttackBuilding/BP/Weapons/BP_HomingArrow_Base` _returnvalue_2))
      (`/Game/Building/AttackBuilding/BP/Weapons/BP_HomingMissile_Base.SetArrowTarget` _asbp_homing_arrow_base (`local.Whats Target`))
      (`/Game/Building/AttackBuilding/BP/Weapons/BP_HomingMissile_Base.SetHomingTarget` _asbp_homing_arrow_base (`Character.CapsuleComponent` _asbp_enemy_ai_base)))))

(fn `UserConstructionScript`
  (`parent.UserConstructionScript`))