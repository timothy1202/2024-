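; Slow skill area actor that halves movement speed and attack speed of enemies entering its sphere.
; On BeginPlay it reads the first BP_SlowBuildingLv3 found in the world to set its lifespan and scale the sphere by attack range.
; Overlap applies the slow directly to EnemyBase stats, then doubles them back after a fixed Delay, which is shared across overlaps and runs on this temporary actor.
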(event `self.ReceiveBeginPlay`
  (bind _sphere (`self.Sphere`))
  (bind _returnvalue (`GameplayStatics.GetActorOfClass` "/Game/Building/AttackBuilding/BP/BP_SlowBuildingLv3.BP_SlowBuildingLv3_C"))
  (`self.SetLifeSpan` (`/Game/Building/BP_BaseBuilding.Building Skill Duration` _returnvalue))
  (`SceneComponent.SetWorldScale3D` _sphere (* (`SceneComponent.K2_GetComponentScale` _sphere) (/ (`/Game/Building/BP_BaseBuilding.Building PT Atk Rng` _returnvalue) 100.0))))

(event `self.Sphere.OnComponentBeginOverlap`
  (params (OverlappedComponent :type "PrimitiveComponent Object Reference") (OtherActor :type "Actor Object Reference") (OtherComp :type "PrimitiveComponent Object Reference") (OtherBodyIndex :type Integer) (bFromSweep :type Boolean) (SweepResult :type "HitResult Structure (by ref)"))
  ;[1 1 1] 스킬 효과 적용
  (bind _asenemy_base (cast `EnemyBase` OtherActor))
  (bind _pawnmovement (`EnemyBase.PawnMovement` _asenemy_base))
  (bind _maxspeed (`FloatingPawnMovement.MaxSpeed` _pawnmovement))
  (set `FloatingPawnMovement.MaxSpeed` (/ _maxspeed 2.0) _pawnmovement)
  (bind _enemynpc_atkspd (`EnemyBase.EnemyNpc_AtkSpd` _asenemy_base))
  (set `EnemyBase.EnemyNpc_AtkSpd` (/ _enemynpc_atkspd 2.0) _asenemy_base)
  (`KismetSystemLibrary.Delay` 5.0) ; 원래대로 복귀
  (set `FloatingPawnMovement.MaxSpeed` (* _maxspeed 2.0) _pawnmovement)
  (set `EnemyBase.EnemyNpc_AtkSpd` (* _enemynpc_atkspd 2.0) _asenemy_base))

(fn `UserConstructionScript`)