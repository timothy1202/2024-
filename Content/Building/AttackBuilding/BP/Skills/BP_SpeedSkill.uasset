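; BP_SpeedSkill is a timed area skill that boosts attack speed of players and buildings inside its sphere.
; On BeginPlay it plays a positioned sound until EndPlay and takes its lifespan from the first BP_SpeedBuildingLv3 found in the world.
; Sphere overlap multiplies attack speed by SpeedUp on entry and by its reciprocal on exit.
; Friendly NPC support is only a placeholder, and range-based sphere scaling is disconnected.
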(event `self.ReceiveBeginPlay`
  (bind _speedaudio (`self.SpeedAudio`))
  ;[1 1 1] 코멘트
  (`AudioComponent.SetSound` _speedaudio "/Game/Assets/Sounds/Building/Sound_LV3_AttackTower_Speed.Sound_LV3_AttackTower_Speed")
  (`AudioComponent.Play` _speedaudio 0.0)
  (`SceneComponent.K2_SetWorldLocation` _speedaudio (`self.K2_GetActorLocation`) false false)
  (bind _returnvalue (`GameplayStatics.GetActorOfClass` "/Game/Building/AttackBuilding/BP/BP_SpeedBuildingLv3.BP_SpeedBuildingLv3_C"))
  (`self.SetLifeSpan` (`/Game/Building/BP_BaseBuilding.Building Skill Duration` _returnvalue)))

(event `self.Sphere.OnComponentBeginOverlap`
  (params (OverlappedComponent :type "PrimitiveComponent Object Reference") (OtherActor :type "Actor Object Reference") (OtherComp :type "PrimitiveComponent Object Reference") (OtherBodyIndex :type Integer) (bFromSweep :type Boolean) (SweepResult :type "HitResult Structure (by ref)"))
  ;[1 1 1] 스킬 효과 적용
  (bind _asbp_player (cast `/Game/TopDown/Blueprints/BP_Player` OtherActor)
    (:`then`
      (set `/Game/TopDown/Blueprints/BP_Player.공격 속도` (* (`/Game/TopDown/Blueprints/BP_Player.공격 속도` _asbp_player) (`self.Speed Up`)) _asbp_player))
    (:`CastFailed`
      (bind _asbp_base_building (cast `/Game/Building/BP_BaseBuilding` OtherActor))
      (set `/Game/Building/BP_BaseBuilding.Building PT Atk Spd` (* (`/Game/Building/BP_BaseBuilding.Building PT Atk Spd` _asbp_base_building) (`self.Speed Up`)) _asbp_base_building))))

(event `self.Sphere.OnComponentEndOverlap`
  (params (OverlappedComponent :type "PrimitiveComponent Object Reference") (OtherActor :type "Actor Object Reference") (OtherComp :type "PrimitiveComponent Object Reference") (OtherBodyIndex :type Integer))
  ;[1 1 1] 스킬 효과 적용
  (bind _asbp_player (cast `/Game/TopDown/Blueprints/BP_Player` OtherActor)
    (:`then`
      (set `/Game/TopDown/Blueprints/BP_Player.공격 속도` (* (`/Game/TopDown/Blueprints/BP_Player.공격 속도` _asbp_player) (/ 1.0 (`self.Speed Up`))) _asbp_player))
    (:`CastFailed`
      (bind _asbp_base_building (cast `/Game/Building/BP_BaseBuilding` OtherActor))
      (set `/Game/Building/BP_BaseBuilding.Building PT Atk Spd` (* (`/Game/Building/BP_BaseBuilding.Building PT Atk Spd` _asbp_base_building) (/ 1.0 (`self.Speed Up`))) _asbp_base_building))))

(event `self.ReceiveEndPlay`
  (params (EndPlayReason :type "EEndPlayReason Enum" :default "Destroyed"))
  (`AudioComponent.Stop` (`self.SpeedAudio`)))

(fn `UserConstructionScript`)