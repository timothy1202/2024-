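; BP_Thunder_Base is an attack-building projectile that arcs toward a moving enemy and explodes with splash damage.
; SetFireBallTarget sets gravity scale from Speed and predicts launch velocity for the moving target, scaling flight time by distance over AttackRange.
; Explode briefly enables ExplosionCollision, spawns a particle system and calls the parent; overlapped Enemy-tagged components trigger fixed damage.
; The AttackRange lookup from the long-range building is disconnected.
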(event `SetFireBallTarget`
  (params (`Closest Target` :type "Actor Object Reference"))
  ;[1 1 1] 예측 포물선
  (set `ProjectileMovementComponent.ProjectileGravityScale` (`self.Speed`) (`self.ProjectileMovement`))
  (bind _outlaunchvelocity (`GameplayStatics.SuggestProjectileVelocity_MovingTarget` (`self.K2_GetActorLocation`) `Closest Target` (0.0 0.0 0.0) (`MovementComponent.GetGravityZ` (`self.ProjectileMovement`)) (`KismetMathLibrary.Lerp` 0.1 1.0 (/ (`self.GetDistanceTo` `Closest Target`) (`self.Attack Range`))) "ForDuration"))
  (set `MovementComponent.Velocity` _outlaunchvelocity (`self.ProjectileMovement`)))

(event `self.ReceiveBeginPlay`
  ;[1 1 1] 거리 설정
)

(event `self.ExplosionCollision.OnComponentBeginOverlap`
  (params (OverlappedComponent :type "PrimitiveComponent Object Reference") (OtherActor :type "Actor Object Reference") (OtherComp :type "PrimitiveComponent Object Reference") (OtherBodyIndex :type Integer) (bFromSweep :type Boolean) (SweepResult :type "HitResult Structure (by ref)"))
  ;[1 1 1] 폭발 데미지
  (if (`ActorComponent.ComponentHasTag` OtherComp "Enemy")
    (bind _asbp_enemy_ai_base (cast `/Game/NPC/EnemeyNPC/BP/BP_EnemyAI_Base` OtherActor))
    (`/Game/NPC/EnemeyNPC/BP/BP_EnemyAI_Base.EnemyTakeDamage` _asbp_enemy_ai_base 10.0)
    (`KismetSystemLibrary.PrintString` "splesh")))

(fn `Explode`
  (`PrimitiveComponent.SetCollisionEnabled` (`self.ExplosionCollision`) "QueryAndPhysics")
  (`NiagaraFunctionLibrary.SpawnSystemAtLocation` "/Game/dissolvingVFX/Particles/P_ExplosionD_04_Converted.P_ExplosionD_04_Converted" (`self.K2_GetActorLocation`) (struct) (0.01 0.01 0.01))
  (`/Engine/EditorBlueprintResources/StandardMacros.IsValid` self
    (:`Is Valid`
      (`PrimitiveComponent.SetCollisionEnabled` (`self.ExplosionCollision`) "NoCollision")
      (`parent.Explode`))))

(fn `UserConstructionScript`
  (`parent.UserConstructionScript`))