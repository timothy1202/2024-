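; Base projectile for attack-building weapons, flying either as an arcing shot or as a homing missile.
; SetArrowTarget starts the trail FX and solves an arc launch velocity with gravity scaled by Speed, while SetHomingTarget enables homing on a component.
; Any sphere overlap calls the empty Explode hook and destroys the projectile.
; Enemies first take fixed damage, plus a first-thunder reaction if IsThunder; the Damage variable is unused.
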(event `SetArrowTarget`
  (params (ClosestTarget :type "Actor Object Reference"))
  (bind _projectilemovement (`self.ProjectileMovement`))
  ;[1 1 1] 포물선
  (set `self.Closest Target` ClosestTarget)
  (`ActorComponent.Activate` (`self.FX_Weapon_trail`) false)
  (set `ProjectileMovementComponent.ProjectileGravityScale` (`self.Speed`) _projectilemovement)
  (bind _outlaunchvelocity (`GameplayStatics.SuggestProjectileVelocity_CustomArc` (`self.K2_GetActorLocation`) (`self.K2_GetActorLocation` ClosestTarget) (`MovementComponent.GetGravityZ` _projectilemovement) 0.3))
  (set `MovementComponent.Velocity` _outlaunchvelocity (`self.ProjectileMovement`)))

(event `self.SphereCollision.OnComponentBeginOverlap`
  (params (OverlappedComponent :type "PrimitiveComponent Object Reference") (OtherActor :type "Actor Object Reference") (OtherComp :type "PrimitiveComponent Object Reference") (OtherBodyIndex :type Integer) (bFromSweep :type Boolean) (SweepResult :type "HitResult Structure (by ref)"))
  ;[1 1 1] 총알 플레이어 닿았는지
  (bind _asbp_my_enemy_base (cast `/Game/NPC/EnemeyNPC/BP/BP_MyEnemyBase` OtherActor)
    (:`then`
      (if (`self.isThunder`)
        (`EnemyBase.FirstThunderAttacked` _asbp_my_enemy_base)
        (`KismetSystemLibrary.PrintString` "thunder"))
      (`/Game/NPC/EnemeyNPC/BP/BP_MyEnemyBase.Take Damage` _asbp_my_enemy_base false 10.0)
      (`self.Explode`)
      (`ActorComponent.Deactivate` (`self.FX_Weapon_trail`))
      (`self.K2_DestroyActor`))
    (:`CastFailed`
      (`self.Explode`)
      (`ActorComponent.Deactivate` (`self.FX_Weapon_trail`))
      (`self.K2_DestroyActor`))))

(event `SetHomingTarget`
  (params (Component :type "SceneComponent Object Reference"))
  (bind _projectilemovement (`self.ProjectileMovement`))
  ;[1 1 1] 유도탄 설정
  (set `ProjectileMovementComponent.bIsHomingProjectile` true _projectilemovement)
  (set `ProjectileMovementComponent.HomingAccelerationMagnitude` 7000.0 _projectilemovement)
  (set `ProjectileMovementComponent.HomingTargetComponent` Component _projectilemovement))

(fn `Explode`)

(fn `UserConstructionScript`)