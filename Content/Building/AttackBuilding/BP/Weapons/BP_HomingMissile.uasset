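; BP_HomingMissile is an attack-building projectile that arcs toward the player and can switch to homing.
; On BeginPlay it sets gravity scale from Speed, then launches along a suggested custom-arc velocity to the location of BP_Player.
; SetHomingTarget turns on ProjectileMovement homing toward a supplied component at fixed acceleration.
; Overlapping the player with AttackCollision only prints a debug string and destroys the missile, with no damage applied.
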(event `self.ReceiveBeginPlay`
  (bind _projectilemovement (`self.ProjectileMovement`))
  ;[1 1 1] 포물선
  (bind _returnvalue (`GameplayStatics.GetActorOfClass` "/Game/TopDown/Blueprints/BP_Player.BP_Player_C"))
  (set `ProjectileMovementComponent.ProjectileGravityScale` (`self.Speed`) _projectilemovement)
  (bind _outlaunchvelocity (`GameplayStatics.SuggestProjectileVelocity_CustomArc` (`self.K2_GetActorLocation`) (`self.K2_GetActorLocation` _returnvalue) (`MovementComponent.GetGravityZ` _projectilemovement)))
  (set `MovementComponent.Velocity` _outlaunchvelocity (`self.ProjectileMovement`)))

(event `self.AttackCollision.OnComponentBeginOverlap`
  (params (OverlappedComponent :type "PrimitiveComponent Object Reference") (OtherActor :type "Actor Object Reference") (OtherComp :type "PrimitiveComponent Object Reference") (OtherBodyIndex :type Integer) (bFromSweep :type Boolean) (SweepResult :type "HitResult Structure (by ref)"))
  ;[1 1 1] 총알 플레이어 닿았는지
  (cast `/Game/TopDown/Blueprints/BP_Player` OtherActor)
  (`KismetSystemLibrary.PrintString` "Hello")
  (`self.K2_DestroyActor`))

(event `SetHomingTarget`
  (params (NewParam :type "SceneComponent Object Reference"))
  (bind _projectilemovement (`self.ProjectileMovement`))
  ;[1 1 1] 유도탄 설정
  (set `ProjectileMovementComponent.bIsHomingProjectile` true _projectilemovement)
  (set `ProjectileMovementComponent.HomingAccelerationMagnitude` 2000.0 _projectilemovement)
  (set `ProjectileMovementComponent.HomingTargetComponent` NewParam _projectilemovement))

(fn `UserConstructionScript`)