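; Level 3 ballista attack building that targets the enemy with the highest current health within its attack range.
; While not collapsed, it runs CheckDistance each tick, then refreshes Target and draws a debug sphere on it.
; FindHighestHpTarget gathers BP_EnemyAI_Base actors overlapping AttackRangeCollision and picks the one with maximum CurHealth, with shortcuts for zero or one enemy.
; No firing logic is defined in these graphs.
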(event `self.ReceiveTick`
  (params (DeltaSeconds :type "Float (single-precision)"))
  ;[1 1 1] 가장 체력 높은 적 설정
  (if (not (`self.bCollapse`))
    (`self.CheckDistance`)
    (bind _output_get (set `self.Target` (`self.Find Highest Hp Target`)))
    (`/Engine/EditorBlueprintResources/StandardMacros.IsValid` _output_get
      (:`Is Valid`
        (`KismetSystemLibrary.DrawDebugSphere` (`self.K2_GetActorLocation` _output_get))))))

(fn `Find Highest Hp Target`
  (returns (`Highest Hp Enemy` :type "Actor Object Reference"))
  (locals (`Local Hp` :type "Array of Float (double-precision)"))
  (bind _overlappingactors (`PrimitiveComponent.GetOverlappingActors` (`self.AttackRangeCollision`) "/Game/NPC/EnemeyNPC/BP/BP_EnemyAI_Base.BP_EnemyAI_Base_C"))
  (switch `int` (`KismetArrayLibrary.Array_Length` _overlappingactors)
    (:`Default`
      (for _array_element _overlappingactors
        (bind _asbp_enemy_ai_base (cast `/Game/NPC/EnemeyNPC/BP/BP_EnemyAI_Base` _array_element))
        (`KismetArrayLibrary.Array_Add` (`local.Local Hp`) (`/Game/NPC/EnemeyNPC/BP/BP_EnemyAI_Base.curHealth` _asbp_enemy_ai_base)))
      (return (`|GetArrayItem` _overlappingactors (`KismetMathLibrary.MaxOfFloatArray` (`local.Local Hp`)))))
    (:`0`
      (return null))
    (:`1`
      (return (`|GetArrayItem` _overlappingactors)))))

(fn `UserConstructionScript`
  (`parent.UserConstructionScript`))