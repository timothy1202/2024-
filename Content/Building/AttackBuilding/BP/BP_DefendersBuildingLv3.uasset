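; Level 3 defender (attack tower) building Blueprint that adds a healing skill on top of its parent building's logic.
; On start it spawns a BP_HealSkill actor at its horizontal position, gives it a reference back to the building, and plays heal audio at the building's location.
; On destroy it removes that skill actor and stops the audio before running the parent cleanup.
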(event `/Game/Building/BP_BaseBuilding.StartLogic`
  (bind _healaudio (`self.HealAudio`))
  ;[1 1 1] 코멘트
  (`parent.StartLogic`)
  (`self.Spawn Healing Range`) ; 첫 재생
  (`AudioComponent.SetSound` _healaudio "/Game/Assets/Sounds/Building/Sound_LV3_AttackTower_Heal.Sound_LV3_AttackTower_Heal")
  (`AudioComponent.Play` _healaudio 0.0)
  (`SceneComponent.K2_SetWorldLocation` _healaudio (`self.K2_GetActorLocation`) false false))

(event `Spawn Healing Range`
  (bind _returnvalue (`self.GetTransform` self))
  ;[1 1 1] 타워 힐 스킬
  (bind _returnvalue_2 (`|SpawnActorFromClass` "/Game/Building/AttackBuilding/BP/Skills/BP_HealSkill.BP_HealSkill_C" (`KismetMathLibrary.MakeTransform` (`KismetMathLibrary.MakeVector` (.x (.location _returnvalue)) (.y (.location _returnvalue)))) "AlwaysSpawn" "MultiplyWithRoot" null null))
  (set `/Game/Building/AttackBuilding/BP/Skills/BP_HealSkill.DefBuilding` self _returnvalue_2)
  (set `self.Heal Skill Actor` _returnvalue_2))

(fn `OnDestroy`
  (`self.K2_DestroyActor` (`self.Heal Skill Actor`))
  (`AudioComponent.Stop` (`self.HealAudio`))
  (`parent.OnDestroy`))

(fn `StopLogic`)

(fn `UserConstructionScript`
  (`parent.UserConstructionScript`))