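; BP_Arrow is an attack-building projectile that explodes on impact and can be switched into homing mode.
; The first Sphere hit fires the ExplosionForce radial impulse, spawns an explosion particle there and destroys the actor.
; HomingMissile validates the passed target and enables strong homing on the Projectile component, but sets its homing target component to None rather than to that target.
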(event `self.Sphere.OnComponentHit`
  (params (HitComponent :type "PrimitiveComponent Object Reference") (OtherActor :type "Actor Object Reference") (OtherComp :type "PrimitiveComponent Object Reference") (NormalImpulse :type "Vector Structure") (Hit :type "HitResult Structure (by ref)"))
  (bind _explosionforce (`self.ExplosionForce`))
  ;[1 1 1] 부딧히면 폭팔
  (`/Engine/EditorBlueprintResources/StandardMacros.DoOnce` false
    (:`Completed`
      (`RadialForceComponent.FireImpulse` _explosionforce)
      (`GameplayStatics.SpawnEmitterAtLocation` "/Game/StarterContent/Particles/P_Explosion.P_Explosion" (`SceneComponent.K2_GetComponentLocation` _explosionforce))
      (`self.K2_DestroyActor`))))

(event `HomingMissile`
  (params (TargetToHit :type "GraduationWork2024Character Object Reference"))
  (bind _projectile (`self.Projectile`))
  ;[1 1 1] 유도탄 설정
  (if (`KismetSystemLibrary.IsValid` TargetToHit)
    (set `ProjectileMovementComponent.HomingTargetComponent` null _projectile)
    (set `ProjectileMovementComponent.bIsHomingProjectile` true _projectile)
    (set `ProjectileMovementComponent.HomingAccelerationMagnitude` 25000.0 _projectile)))

(fn `UserConstructionScript`)