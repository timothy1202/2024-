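; Base build plot actor for placing, upgrading and repairing buildings by spending player resources.
; Box overlap registers the plot with BP_Player and previews the attached building, while interaction opens a build info widget.
; Tick times construction, swapping staged meshes by thirds before activating the building and raising its tier.
; Upgrades spawn and attach a replacement building, CheckAbleToUpgrade compares headquarters tier, and repair cost scales with damage.
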(event `self.ReceiveBeginPlay`
  (bind _constructmeshes (`self.ConstructMeshes`))
  (bind _box (`self.Box`))
  (`/Engine/EditorBlueprintResources/StandardMacros.IsValid` (`|GetArrayItem` (`self.GetAttachedActors` true))
    (:`Is Valid`
      (`self.InitProperty`)
      (`PrimitiveComponent.SetCollisionEnabled` _box "QueryOnly")
      (`SceneComponent.SetVisibility` _constructmeshes true true)
      (`KismetSystemLibrary.DelayUntilNextTick`)
      (`self.GetBuildInfoProperty` false)
      (`self.UpdateBuildInfoWidget`))
    (:`Is Not Valid`
      (`PrimitiveComponent.SetCollisionEnabled` _box "NoCollision")
      (`SceneComponent.SetVisibility` _constructmeshes false true))))

(event `ResetBuildSystem`
  (bind _build_ui_widget (`self.Build_UI_Widget`))
  (set `self.bBuilt` false)
  (`/Engine/EditorBlueprintResources/StandardMacros.DecrementInt` (`self.buildTier`)
    (:`  `
      (set `/Game/TopDown/Blueprints/BP_Player.ButtonState` "NewEnumerator1" (`self.Player`))
      (`SceneComponent.SetVisibility` (`self.ConstructMeshes`) true true)
      (`self.SetBuildRange` "Small")
      (`/Game/Building/Widget/BuildingInfoUI/WP_MainBuildingUI.CloseUI` _build_ui_widget)
      (`/Game/TopDown/Blueprints/BP_Player.RemoveWidget` (`self.Player`) _build_ui_widget)
      (`self.GetBuildInfoProperty` false)
      (`self.UpdateBuildInfoWidget`)
      (if (`PrimitiveComponent.IsOverlappingComponent` (`self.Box`) (`Character.CapsuleComponent` (`self.Player`)))
        (`self.SetBuildingMesh` true)))))

(event `RepairMyBuilding`
  (`/Game/Building/BP_BaseBuilding.InitializeHealth` (`self.AssignedBuilding`))
  (`self.PlayUpgradeEffect` "Start"))

(event `self.Box.OnComponentBeginOverlap`
  (params (OverlappedComponent :type "PrimitiveComponent Object Reference") (OtherActor :type "Actor Object Reference") (OtherComp :type "PrimitiveComponent Object Reference") (OtherBodyIndex :type Integer) (bFromSweep :type Boolean) (SweepResult :type "HitResult Structure (by ref)"))
  (bind _player (`self.Player`))
  (if (`ActorComponent.ComponentHasTag` OtherComp "Player")
    (`/Game/TopDown/Blueprints/BP_Player.Update Current Build Place` _player self)
    (set `/Game/TopDown/Blueprints/BP_Player.ButtonState` "NewEnumerator1" _player)
    (if (and (not (`self.bBuilt`)) (not (`self.bConstructing`)))
      (`self.SetBuildingMesh` true))))

(event `self.Box.OnComponentEndOverlap`
  (params (OverlappedComponent :type "PrimitiveComponent Object Reference") (OtherActor :type "Actor Object Reference") (OtherComp :type "PrimitiveComponent Object Reference") (OtherBodyIndex :type Integer))
  (if (`ActorComponent.ComponentHasTag` OtherComp "Player")
    (set `/Game/TopDown/Blueprints/BP_Player.currentBuildPlace` null (`self.Player`))
    (`self.ToggleBuildInfo` false)
    (`self.ExecuteInteract` false)
    (if (and (not (`self.bBuilt`)) (not (`self.bConstructing`)))
      (`self.SetBuildingMesh` false))))

(event `self.ReceiveTick`
  (params (DeltaSeconds :type "Float (single-precision)"))
  (`self.ConstructLogic` DeltaSeconds))

(fn `ChangeConstructMeshAsProgress`
  (params (ProgressNum :type Integer))
  (`/Game/Building/BP_BaseBuilding.SetConstructMesh` (`self.AssignedBuilding`) ProgressNum))

(fn `CheckAbleToUpgrade`
  (returns (bAble :type Boolean))
  (bind _headquaterref (`/Game/TopDown/Blueprints/BP_Player.HeadquaterREF` (`self.Player`)))
  (if (`GameplayStatics.ObjectIsA` (`self.AssignedBuilding`) "/Game/Building/Headquater/BP_HeadquaterBase.BP_HeadquaterBase_C")
    (return true)
    (else
      (`/Engine/EditorBlueprintResources/StandardMacros.IsValid` _headquaterref
        (:`Is Valid`
          (if (> (`.Building_Tier_70_61BDC23145EEB8333C1249B405AB7931` (break `/Game/Building/ST_Building/ST_Building` (`/Game/Building/BP_BaseBuilding.ST_Building` _headquaterref))) (`self.buildTier`))
            (return true)
            (else
              (bind _returnvalue (`|CreateWidget` "/Game/TopDown/Blueprints/UI/WP_WarningMsg.WP_WarningMsg_C" (`GameplayStatics.GetPlayerController` 0) "본부 레벨이 낮습니다. \n본부 건물을 업그레이드하세요!"))
              (`UserWidget.AddToViewport` _returnvalue 0)
              (return false))))
        (:`Is Not Valid`
          (bind _returnvalue_2 (`|CreateWidget` "/Game/TopDown/Blueprints/UI/WP_WarningMsg.WP_WarningMsg_C" (`GameplayStatics.GetPlayerController` 0) "본부 건물이 아직 지어지지 않았습니다!"))
          (`UserWidget.AddToViewport` _returnvalue_2 0)
          (return false))))))

(fn `CheckConstructProgress`
  (returns (progressNum :type Integer))
  (bind _curbuildingtime (`self.curBuildingTime`))
  (bind _maxbuildingtime (`self.maxBuildingTIme`))
  (bind _returnvalue (* _maxbuildingtime 0.33))
  (bind _returnvalue_2 (* _maxbuildingtime 0.66))
  (if (`KismetMathLibrary.InRange_FloatFloat` _curbuildingtime 0.0 _returnvalue true false)
    (return 0)
    (elif (`KismetMathLibrary.InRange_FloatFloat` _curbuildingtime _returnvalue _returnvalue_2 true false)
      (return 1)
      (elif (`KismetMathLibrary.InRange_FloatFloat` _curbuildingtime _returnvalue_2 (* _maxbuildingtime 1.0) true false)
        (return 2)
        (else
          (return 3))))))

(fn `ConstructBuildings`
  (`/Game/Building/BP_BaseBuilding.Initialize` (`self.AssignedBuilding`) true)
  (`self.PlayUpgradeEffect` "Finish")
  (`self.ToggleConstructEffect` false)
  (if (`self.Destroyed`)
    (`self.SetBuildRange` "Large")))

(fn `ConstructLogic`
  (params (time :type "Float (double-precision)"))
  (locals (deltaTime :type "Float (double-precision)") (index :type Integer :default 0))
  (bind _changeconstructstateonce (`self.ChangeConstructStateOnce`))
  (bind _output_get (set `local.deltaTime` time))
  (if (`self.bConstructing`)
    (set `self.curBuildingTime` (+ (`self.curBuildingTime`) _output_get))
    (bind _output_get_2 (set `local.index` (`self.CheckConstructProgress`)))
    (if (!= _output_get_2 3)
      (if (`|GetArrayItem` (`self.ChangeConstructStateOnce`) _output_get_2)
        (`KismetArrayLibrary.Array_Set` (`self.ChangeConstructStateOnce`) (`local.index`))
        (`self.ChangeConstructMeshAsProgress` (`local.index`)))
      (else
        (`self.OnFinishConstruct`)))
    (else
      (set `self.curBuildingTime` 0.0)
      (for (_ _array_index) _changeconstructstateonce
        (`KismetArrayLibrary.Array_Set` _changeconstructstateonce _array_index true)))))

(fn `ExecuteInteract`
  (params (Toggle :type Boolean)))

(fn `GetAssignedBuildingFatalRate`
  (returns (Rate :type "Float (double-precision)"))
  (locals (FatalRate :type "Float (double-precision)"))
  (switch `int` (`/Game/Building/BP_BaseBuilding.HealthIndex` (`self.AssignedBuilding`))
    (:`0`
      (set `local.FatalRate` 1.0))
    (:`1`
      (set `local.FatalRate` 0.75))
    (:`2`
      (set `local.FatalRate` 0.5))
    (:`3`
      (set `local.FatalRate` 0.25))
    (:`4`
      (set `local.FatalRate` 0.0)))
  (return (`local.FatalRate`)))

(fn `GetBuildInfoProperty`
  (params (bNextBuildInfo :type Boolean))
  (locals (Index :type Integer))
  (`KismetArrayLibrary.Array_Clear` (`self.NextBuildingInfo`))
  (if bNextBuildInfo
    (set `self.NextBuildingInfo` (`/Game/Building/BP_BaseBuilding.myBuildInfoArr` (`self.AssignedBuilding`)))
    (else
      (`KismetArrayLibrary.Array_Add` (`self.NextBuildingInfo`) (`.BuildInfo_106_3A7C77CB417F746A8E374CA9D329901F` (break `/Game/Building/ST_Building/ST_Building` (`/Game/Building/BP_BaseBuilding.ST_Building` (`self.AssignedBuilding`))))))))

(fn `GetCurrentBuildInfo`
  (returns (ReturnValue :type "/Game/Building/ST_Building/ST_BuildInfo Structure"))
  (return (`.BuildInfo_106_3A7C77CB417F746A8E374CA9D329901F` (break `/Game/Building/ST_Building/ST_Building` (`/Game/Building/BP_BaseBuilding.ST_Building` (`self.AssignedBuilding`))))))

(fn `GetInteractable`
  (returns (bInteractable :type Boolean))
  (return (`/Game/Building/BP_BaseBuilding.bInteractable` (`self.AssignedBuilding`))))

(fn `GetRepairCost`
  (returns (ReturnValue :type Integer))
  (bind _output_get (set `self.BuildingRepairCost` (`KismetMathLibrary.FTrunc` (* (`.Coin_9_91B901A9466F603082C150A4480EA876` (break `/Game/Building/ST_Building/ST_BuildInfo` (`self.GetCurrentBuildInfo`))) (`self.GetAssignedBuildingFatalRate`)))))
  (return _output_get))

(fn `InitializeBuildPlace`
  (params (AssignedBuilding :type "/Game/Building/BP_BaseBuilding Object Reference"))
  (bind _output_get (set `self.AssignedBuilding` AssignedBuilding))
  (set `self.maxBuildingTIme` (`/Game/Building/BP_BaseBuilding.Construction Time` _output_get)))

(fn `InitProperty`
  (bind _asbp_player (cast `/Game/TopDown/Blueprints/BP_Player` (`GameplayStatics.GetPlayerCharacter` 0)))
  (bind _output_get (set `self.Player` _asbp_player))
  (bind _returnvalue (`|CreateWidget` "/Game/Building/Widget/BuildingInfoUI/WP_MainBuildingUI.WP_MainBuildingUI_C" (`GameplayStatics.GetPlayerController` 0) _output_get))
  (set `self.Build_UI_Widget` _returnvalue)
  (set `self.OriginalExtend` (`BoxComponent.BoxExtent` (`self.Box`))))

(fn `InteractBuilding`
  (params (ButtonState :type "/Game/TopDown/Blueprints/Enums/EButtonState Enum" :default "NewEnumerator1"))
  (switch `/Game/TopDown/Blueprints/Enums/EButtonState` ButtonState
    (:`NewEnumerator1`
      (`self.ToggleBuildInfo` true))
    (:`NewEnumerator2`
      (`self.ExecuteInteract` true))
    (:`NewEnumerator3`
      (`self.RepairBuilding`))))

(fn `OnFinishConstruct`
  (`self.SetConstructState` false)
  (set `self.bBuilt` true)
  (`self.ConstructBuildings`)
  (set `self.ConstructingState` "NewEnumerator0")
  (`/Engine/EditorBlueprintResources/StandardMacros.IncrementInt` (`self.buildTier`)
    (:`  `
      (`self.GetBuildInfoProperty` true)
      (`self.UpdateBuildInfoWidget`)
      (`self.PlaySound` "/Game/Building/Sounds/Building_Clear.Building_Clear" (`self.K2_GetActorLocation`)))))

(fn `OnStartConstruct`
  (`self.ToggleConstructEffect` true)
  (`self.SetBuildingMesh` false)
  (`SceneComponent.SetVisibility` (`self.ConstructMeshes`) false true)
  (`self.PlayUpgradeEffect` "Start")
  (set `self.ConstructingState` "NewEnumerator1")
  (`self.PlaySound` "/Game/Building/Sounds/Sound_BuildingUpgrade.Sound_BuildingUpgrade" (`self.K2_GetActorLocation`)))

(fn `PlaySound`
  (params (Sound :type "SoundBase Object Reference") (Location :type "Vector Structure"))
  (bind _currentsoundsource (`self.CurrentSoundSource`))
  (`|ExecutionSequence`
    (:`then_0`
      (`/Engine/EditorBlueprintResources/StandardMacros.IsValid` _currentsoundsource
        (:`Is Valid`
          (if (`AudioComponent.IsPlaying` _currentsoundsource)
            (`AudioComponent.Stop` (`self.CurrentSoundSource`))))))
    (:`then_1`
      (bind _returnvalue (`GameplayStatics.SpawnSoundAtLocation` Sound Location (struct) 0.5 1.0 0.0 "/Game/NPC/EnemeyNPC/BP/Building_SoundAttenuation.Building_SoundAttenuation" null))
      (set `self.CurrentSoundSource` _returnvalue))))

(fn `PlayUpgradeEffect`
  (params (ProgressType :type String))
  (bind _returnvalue (`self.K2_GetActorLocation`))
  (bind _assignedbuilding (`self.AssignedBuilding`))
  (bind _upgradeeffectsmokescale (`/Game/Building/BP_BaseBuilding.upgradeEffectSmokeScale` _assignedbuilding))
  (switch `string` ProgressType
    (:`Start`
      (`/Game/Building/BP_BaseBuilding.PlayUpgradeEffect` _assignedbuilding (* _upgradeeffectsmokescale 0.5) _returnvalue))
    (:`Finish`
      (`/Game/Building/BP_BaseBuilding.PlayUpgradeEffect` _assignedbuilding _upgradeeffectsmokescale _returnvalue))))

(fn `RepairBuilding`
  (bind _buildingrepaircost (`self.BuildingRepairCost`))
  (if (> _buildingrepaircost 0)
    (`/Game/TopDown/Blueprints/BP_Player.ChangePlayerResource` (`self.Player`) "NewEnumerator6" (* _buildingrepaircost -1))
    (`self.RepairMyBuilding`)))

(fn `SetBuildingMesh`
  (params (bVisible :type Boolean))
  (bind _assignedbuilding (`self.AssignedBuilding`))
  (`self.AssignedBuilding`
    (:`then`
      (if bVisible
        (`/Game/Building/BP_BaseBuilding.Initialize` _assignedbuilding false)
        (else
          (`/Game/Building/BP_BaseBuilding.HideBuilding` _assignedbuilding))))
    (:`else`)))

(fn `SetBuildRange`
  (params (Range :type String))
  (bind (_originalextend_x _originalextend_y _originalextend_z) (`KismetMathLibrary.BreakVector` (`self.OriginalExtend`)))
  (switch `string` Range
    (:`Small`
      (`BoxComponent.SetBoxExtent` (`self.Box`) (`self.OriginalExtend`) true)
      (set `self.Destroyed` true))
    (:`Large`
      (`BoxComponent.SetBoxExtent` (`self.Box`) (`KismetMathLibrary.MakeVector` (* _originalextend_x 1.5) (* _originalextend_y 1.5) _originalextend_z) true)
      (set `self.Destroyed` false))))

(fn `SetConstructMeshVisibility`
  (params (bVisible :type Boolean))
  (`/Game/Building/BP_BaseBuilding.ToggleConstructMesh` (`self.AssignedBuilding`) bVisible))

(fn `SetConstructProressBarVisibility`
  (params (bVisibility :type Boolean))
  (`SceneComponent.SetVisibility` (`/Game/Building/BP_BaseBuilding.BuildProgressWidget` (`self.AssignedBuilding`)) bVisibility false))

(fn `SetConstructState`
  (params (bConstruct :type Boolean))
  (bind _output_get (set `self.bConstructing` bConstruct))
  (`self.SetConstructMeshVisibility` _output_get)
  (`self.SetConstructProressBarVisibility` _output_get)
  (if _output_get
    (if (`self.bPlayOnce`)
      (set `self.bPlayOnce` false)
      (`self.OnStartConstruct`))
    (else
      (set `self.bPlayOnce` true))))

(fn `SetNextBuilding`
  (params (buildInfo :type "BaseBuilding Class Reference"))
  (bind _returnvalue (`BaseBuilding.SpawnBuildinig` (`self.AssignedBuilding`) buildInfo))
  (`/Engine/EditorBlueprintResources/StandardMacros.IsValid` _returnvalue
    (:`Is Valid`
      (`/Game/Building/BP_BaseBuilding.OnRemove` (`self.AssignedBuilding`))
      (`self.K2_AttachToActor` _returnvalue self "None" "KeepWorld" "KeepWorld" "KeepWorld" true)
      (`BaseBuilding.OnSpawned` _returnvalue)
      (`self.SetConstructState` true))
    (:`Is Not Valid`
      (`KismetSystemLibrary.PrintString` "클래스가 잘 못 할당되어있습니다! \nDT_Building확인 바람." true true (struct :`R` 1.0 :`A` 1.0) 10.0))))

(fn `ShowMessage`
  (params (Text :type Text))
  (bind _returnvalue (`|SpawnActorFromClass` "/Game/TopDown/Blueprints/BP_Message.BP_Message_C" (`KismetMathLibrary.MakeTransform` (`KismetSystemLibrary.GetComponentBounds` (`/Game/Building/BP_BaseBuilding.HitCollision` (`self.AssignedBuilding`)))) "Undefined" "MultiplyWithRoot" null null))
  (`/Game/TopDown/Blueprints/BP_Message.PlayText` _returnvalue "NewEnumerator2" Text))

(fn `ToggleBuildInfo`
  (params (Toggle :type Boolean))
  (bind _build_ui_widget (`self.Build_UI_Widget`))
  (bind _build_ui_widget_2 (`self.Build_UI_Widget`))
  (bind _returnvalue (!= (`self.buildTier`) 3))
  (if Toggle
    (if _returnvalue
      (if (not (`/Game/Building/Widget/BuildingInfoUI/WP_MainBuildingUI.bShow` (`self.Build_UI_Widget`)))
        (`UserWidget.AddToViewport` _build_ui_widget_2 0)
        (`/Game/TopDown/Blueprints/BP_Player.AddWidget` (`self.Player`) _build_ui_widget_2)
        (`/Game/Building/Widget/BuildingInfoUI/WP_MainBuildingUI.ShowBuildInfoUI` _build_ui_widget_2))
      (else
        (`self.ShowMessage` "최대 업그레이드입니다!")))
    (elif _returnvalue
      (`/Game/Building/Widget/BuildingInfoUI/WP_MainBuildingUI.CloseUI` _build_ui_widget)
      (`/Game/TopDown/Blueprints/BP_Player.RemoveWidget` (`self.Player`) _build_ui_widget))))

(fn `ToggleConstructEffect`
  (params (bToggle :type Boolean))
  (`/Game/Building/BP_BaseBuilding.ToggleConstructingEffet` (`self.AssignedBuilding`) bToggle (`self.K2_GetActorLocation`)))

(fn `UpdateBuildInfoWidget`
  (locals (BuildInfoClass :type "/Game/Building/Widget/BuildingInfoUI/WP_BuildInfoBase Class Reference" :default "/Script/UMG.WidgetBlueprintGeneratedClass'/Game/Building/Widget/BuildingInfoUI/WP_BuildInfoBase.WP_BuildInfoBase_C'"))
  (if (> (`KismetArrayLibrary.Array_Length` (`self.NextBuildingInfo`)) 1)
    (set `local.BuildInfoClass` "/Game/Building/Widget/BuildingInfoUI/WP_AttackBuildInfo.WP_AttackBuildInfo_C")
    (else
      (set `local.BuildInfoClass` "/Game/Building/Widget/BuildingInfoUI/WP_NormalBuildInfo.WP_NormalBuildInfo_C")))
  (`/Game/Building/Widget/BuildingInfoUI/WP_MainBuildingUI.UpdateBuildingWidget` (`self.Build_UI_Widget`) (`local.BuildInfoClass`) (`/Game/Building/BP_BaseBuilding.BuildingType` (`self.AssignedBuilding`)) (`self.NextBuildingInfo`) self))

(fn `UpgradeBuilding`
  (params (buildInfo :type "/Game/Building/ST_Building/ST_BuildInfo Structure"))
  (`self.UseResources` buildInfo)
  (if (`self.bBuilt`)
    (`self.ToggleBuildInfo` false)
    (`self.SetNextBuilding` (`.BuildClass_19_0ADEAC034F479993BA5F27928C52A04B` (break `/Game/Building/ST_Building/ST_BuildInfo` buildInfo)))
    (else
      (`self.ToggleBuildInfo` false)
      (`self.SetConstructState` true))))

(fn `UserConstructionScript`)

(fn `UseResources`
  (params (Info :type "/Game/Building/ST_Building/ST_BuildInfo Structure"))
  (bind (_buildclass _buildname _builddetails _coin _skeletongem _lizardmangem _orcgem) (break `/Game/Building/ST_Building/ST_BuildInfo` Info))
  (bind _player (`self.Player`))
  (`|ExecutionSequence`
    (:`then_0`
      (`/Game/TopDown/Blueprints/BP_Player.ChangePlayerResource` _player "NewEnumerator6" (* _coin -1)))
    (:`then_1`
      (`/Game/TopDown/Blueprints/BP_Player.ChangePlayerResource` _player "NewEnumerator4" (* _skeletongem -1)))
    (:`then_2`
      (`/Game/TopDown/Blueprints/BP_Player.ChangePlayerResource` _player "NewEnumerator3" (* _lizardmangem -1)))
    (:`then_3`
      (`/Game/TopDown/Blueprints/BP_Player.ChangePlayerResource` _player "NewEnumerator5" (* _orcgem -1)))))