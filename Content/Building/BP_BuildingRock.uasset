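; BP_BuildingRock is a build-site actor that shows a build widget and reveals its assigned buildings while the player is inside its trigger box.
; BeginPlay marks those buildings as not yet built and offsets the hidden widget using the first building's footprint diagonal.
; Overlap begin and end toggle the widget and call Initialize or HideBuilding on each building.
; While visible, the widget's pivot follows camera-boom yaw each tick and the widget faces the viewpoint.
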(event `self.ReceiveBeginPlay`
  (bind (_boxextent_x _boxextent_y) (`KismetMathLibrary.BreakVector` (`BoxComponent.BoxExtent` (`/Game/Building/BP_BaseBuilding.HitCollision` (`|GetArrayItem` (`self.AssignedBuildings`))))))
  (for _array_element (`self.AssignedBuildings`)
    (`/Game/Building/BP_BaseBuilding.NotBuiltYet` _array_element)
    (bind _asbp_player (cast `/Game/TopDown/Blueprints/BP_Player` (`GameplayStatics.GetPlayerCharacter` 0)))
    (set `self.Player` _asbp_player)
    (`SceneComponent.K2_SetRelativeLocation` (`self.BuildWidgetComponent`) (`KismetMathLibrary.MakeVector` 0.0 (+ (`KismetMathLibrary.Sqrt` (+ (`KismetMathLibrary.Square` _boxextent_x) (`KismetMathLibrary.Square` _boxextent_y))) (`self.offsetValue`)) 300.0) false false)
    (`SceneComponent.SetVisibility` (`self.BuildWidgetComponent`) false false)))

(event `self.Box.OnComponentBeginOverlap`
  (params (OverlappedComponent :type "PrimitiveComponent Object Reference") (OtherActor :type "Actor Object Reference") (OtherComp :type "PrimitiveComponent Object Reference") (OtherBodyIndex :type Integer) (bFromSweep :type Boolean) (SweepResult :type "HitResult Structure (by ref)"))
  (cast `/Game/TopDown/Blueprints/BP_Player` OtherActor)
  (bind _output_get (set `self.IsWidgetOn` true))
  (`SceneComponent.SetVisibility` (`self.BuildWidgetComponent`) _output_get false)
  (for _array_element (`self.AssignedBuildings`)
    (`/Game/Building/BP_BaseBuilding.Initialize` _array_element false)))

(event `self.Box.OnComponentEndOverlap`
  (params (OverlappedComponent :type "PrimitiveComponent Object Reference") (OtherActor :type "Actor Object Reference") (OtherComp :type "PrimitiveComponent Object Reference") (OtherBodyIndex :type Integer))
  (cast `/Game/TopDown/Blueprints/BP_Player` OtherActor)
  (bind _output_get (set `self.IsWidgetOn` false))
  (`SceneComponent.SetVisibility` (`self.BuildWidgetComponent`) _output_get false)
  (for _array_element (`self.AssignedBuildings`)
    (`/Game/Building/BP_BaseBuilding.HideBuilding` _array_element)))

(event `self.ReceiveTick`
  (params (DeltaSeconds :type "Float (single-precision)"))
  (`self.BuildingWidgetLogic`))

(fn `BuildingWidgetLogic`
  (bind (_returnvalue_roll _returnvalue_pitch _returnvalue_yaw) (`KismetMathLibrary.BreakRotator` (`SceneComponent.K2_GetComponentRotation` (`GraduationWork2024Character.CameraBoom` (`self.Player`)))))
  (bind (_returnvalue_roll_2 _returnvalue_pitch_2 _returnvalue_yaw_2) (`KismetMathLibrary.BreakRotator` (`KismetMathLibrary.FindLookAtRotation` (`SceneComponent.K2_GetComponentLocation` (`self.BuildWidgetComponent`)) (`Controller.GetPlayerViewPoint` (`GameplayStatics.GetPlayerController` 0)))))
  (if (`self.IsWidgetOn`)
    (`SceneComponent.K2_SetWorldRotation` (`self.WidgetRot`) (`KismetMathLibrary.MakeRotator` 0.0 0.0 _returnvalue_yaw) false false)
    (`SceneComponent.K2_SetWorldRotation` (`self.BuildWidgetComponent`) (`KismetMathLibrary.MakeRotator` 0.0 _returnvalue_pitch_2 _returnvalue_yaw_2) false false)))

(fn `UserConstructionScript`)