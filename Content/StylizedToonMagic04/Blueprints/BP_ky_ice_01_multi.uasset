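; Effect spawner actor that plays a staggered multi-hit burst of the NS_ky_ice_01 Niagara ice effect.
; On BeginPlay it spawns one system at Point1, then a short counter-driven series at random horizontal offsets around the actor, separated by brief random delays.
; After a final pause it either resets the counter and repeats when IsRepeat is set, or destroys itself.
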(event `self.ReceiveBeginPlay`
  ;[1 1 1] spawn fx
  (`NiagaraFunctionLibrary.SpawnSystemAtLocation` "/Game/StylizedToonMagic04/Particles/NS_ky_ice_01.NS_ky_ice_01" (`SceneComponent.K2_GetComponentLocation` (`self.point1`)) :!label _label)
  (`KismetSystemLibrary.Delay` (`KismetMathLibrary.RandomFloatInRange` 0.05 0.2))
  (`NiagaraFunctionLibrary.SpawnSystemAtLocation` "/Game/StylizedToonMagic04/Particles/NS_ky_ice_01.NS_ky_ice_01" (+ (`KismetMathLibrary.MakeVector` (`KismetMathLibrary.Conv_IntToDouble` (`KismetMathLibrary.RandomIntegerInRange` -150 150)) (`KismetMathLibrary.Conv_IntToDouble` (`KismetMathLibrary.RandomIntegerInRange` -150 150))) (`self.K2_GetActorLocation`)) :!label _label_2)
  (`KismetSystemLibrary.Delay` (`KismetMathLibrary.RandomFloatInRange` 0.05 0.2))
  (if (> (`self.Counter`) 1)
    ;[1 1 1] end
    (`KismetSystemLibrary.Delay` 2.0)
    (if (`self.isRepeat`)
      (set `self.Counter` 0)
      (goto _label)
      (else
        (`self.K2_DestroyActor`)))
    (else
      (`/Engine/EditorBlueprintResources/StandardMacros.IncrementInt` (`self.Counter`)
        (:`  `
          (goto _label_2))))))

(fn `UserConstructionScript`)