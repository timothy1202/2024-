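; Effect actor that plays a burst of stylized thunder strikes using the NS_ky_thunder_02 Niagara system.
; On BeginPlay it spawns one strike at Point1, then a counter-driven Delay loop spawns several more at random XY offsets around the actor with randomized short gaps.
; After a final pause it either resets and repeats the burst when IsRepeat is set, or destroys itself.
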(event `self.ReceiveBeginPlay`
  ;[1 1 1] spawn fx
  (`NiagaraFunctionLibrary.SpawnSystemAtLocation` "/Game/StylizedToonMagic04/Particles/NS_ky_thunder_02.NS_ky_thunder_02" (`SceneComponent.K2_GetComponentLocation` (`self.point1`)) :!label _label)
  (`KismetSystemLibrary.Delay` (`KismetMathLibrary.RandomFloatInRange` 0.1 0.3))
  (`NiagaraFunctionLibrary.SpawnSystemAtLocation` "/Game/StylizedToonMagic04/Particles/NS_ky_thunder_02.NS_ky_thunder_02" (+ (`KismetMathLibrary.MakeVector` (`KismetMathLibrary.Conv_IntToDouble` (`KismetMathLibrary.RandomIntegerInRange` -200 200)) (`KismetMathLibrary.Conv_IntToDouble` (`KismetMathLibrary.RandomIntegerInRange` -200 200))) (`self.K2_GetActorLocation`)) :!label _label_2)
  (`KismetSystemLibrary.Delay` (`KismetMathLibrary.RandomFloatInRange` 0.1 0.3))
  (if (> (`self.Counter`) 2)
    ;[1 1 1] end
    (`KismetSystemLibrary.Delay` 1.5)
    (if (`self.isRepeat`)
      (set `self.Counter` 0)
      (goto _label)
      (else
        (`self.K2_DestroyActor`)))
    (else
      (`/Engine/EditorBlueprintResources/StandardMacros.IncrementInt` (`self.Counter`)
        (:`  `
          (goto _label_2))))))

(fn `UserConstructionScript`)